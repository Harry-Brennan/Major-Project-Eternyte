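; One rotating dial of a combination lock, showing six icon keys (pickaxe, rope, skull, stopwatch, dynamite, gas) on widget components.
; TurnLockPart advances to the next key with wraparound, tweens the mesh to that key's angle, then asks its AssociatedFullLock to check the combination.
; Construction script and BeginPlay set up icons, prompt text and starting rotation.
; ShowPrompt fades in a turn prompt that a looping timer keeps facing the player until HidePrompt.
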(event `self.ReceiveBeginPlay`
  (bind _aswbp_wiggly_menu_text (cast `/Game/UI/Menus/WBP_Wiggly_Menu_Text` (`WidgetComponent.GetWidget` (`self.Interact Prompt`))))
  (bind _output_get (set `self.Interact Text` _aswbp_wiggly_menu_text))
  (set `/Game/UI/Menus/WBP_Wiggly_Menu_Text.Text` "LMB TURN" _output_get)
  (set `/Game/UI/Menus/WBP_Wiggly_Menu_Text.Size` 480.0 _output_get)
  (set `/Game/UI/Menus/WBP_Wiggly_Menu_Text.Irregular Shake Intensity?` false _output_get)
  (set `/Game/UI/Menus/WBP_Wiggly_Menu_Text.Shake Intensity` 0.05 _output_get)
  (set `/Game/UI/Menus/WBP_Wiggly_Menu_Text.Text Colour` (struct :`R` 1.0 :`G` 1.0 :`B` 1.0 :`A` 1.0) _output_get)
  (set `/Game/UI/Menus/WBP_Wiggly_Menu_Text.Shadow Colour` (struct :`R` 0.119792 :`A` 1.0) _output_get)
  (`Widget.SetRenderOpacity` (`/Game/UI/Menus/WBP_Wiggly_Menu_Text.WiggleTextWrapBox` (`self.Interact Text`)) 0.0)
  (`self.Reset Lock Part`)
  (`|ExecutionSequence`
    (:`then_0`
      (bind _aswbp_lock_part_icon (cast `/Game/Environment_BPs/Lock/WBP_Lock_Part_Icon` (`WidgetComponent.GetWidget` (`self.Dynamite Icon`))))
      (set `/Game/Environment_BPs/Lock/WBP_Lock_Part_Icon.Associated Key` "NewEnumerator4" _aswbp_lock_part_icon)
      (`/Game/Environment_BPs/Lock/WBP_Lock_Part_Icon.Update Icon` _aswbp_lock_part_icon))
    (:`then_1`
      (bind _aswbp_lock_part_icon_2 (cast `/Game/Environment_BPs/Lock/WBP_Lock_Part_Icon` (`WidgetComponent.GetWidget` (`self.Pickaxe Icon`))))
      (set `/Game/Environment_BPs/Lock/WBP_Lock_Part_Icon.Associated Key` "NewEnumerator1" _aswbp_lock_part_icon_2)
      (`/Game/Environment_BPs/Lock/WBP_Lock_Part_Icon.Update Icon` _aswbp_lock_part_icon_2))
    (:`then_2`
      (bind _aswbp_lock_part_icon_3 (cast `/Game/Environment_BPs/Lock/WBP_Lock_Part_Icon` (`WidgetComponent.GetWidget` (`self.Gas Icon`))))
      (set `/Game/Environment_BPs/Lock/WBP_Lock_Part_Icon.Associated Key` "NewEnumerator5" _aswbp_lock_part_icon_3)
      (`/Game/Environment_BPs/Lock/WBP_Lock_Part_Icon.Update Icon` _aswbp_lock_part_icon_3))
    (:`then_3`
      (bind _aswbp_lock_part_icon_4 (cast `/Game/Environment_BPs/Lock/WBP_Lock_Part_Icon` (`WidgetComponent.GetWidget` (`self.Stopwatch Icon`))))
      (set `/Game/Environment_BPs/Lock/WBP_Lock_Part_Icon.Associated Key` "NewEnumerator3" _aswbp_lock_part_icon_4)
      (`/Game/Environment_BPs/Lock/WBP_Lock_Part_Icon.Update Icon` _aswbp_lock_part_icon_4))
    (:`then_4`
      (bind _aswbp_lock_part_icon_5 (cast `/Game/Environment_BPs/Lock/WBP_Lock_Part_Icon` (`WidgetComponent.GetWidget` (`self.Skull Icon`))))
      (set `/Game/Environment_BPs/Lock/WBP_Lock_Part_Icon.Associated Key` "NewEnumerator0" _aswbp_lock_part_icon_5)
      (`/Game/Environment_BPs/Lock/WBP_Lock_Part_Icon.Update Icon` _aswbp_lock_part_icon_5))
    (:`then_5`
      (bind _aswbp_lock_part_icon_6 (cast `/Game/Environment_BPs/Lock/WBP_Lock_Part_Icon` (`WidgetComponent.GetWidget` (`self.Rope Icon`))))
      (set `/Game/Environment_BPs/Lock/WBP_Lock_Part_Icon.Associated Key` "NewEnumerator2" _aswbp_lock_part_icon_6)
      (`/Game/Environment_BPs/Lock/WBP_Lock_Part_Icon.Update Icon` _aswbp_lock_part_icon_6))))

(event `Turn Lock Part`
  (bind _returnvalue (+ (`self.Current Key`) 1))
  (set `self.Key Before Changing` (`self.Current Key`))
  (set `self.Current Key` (select `bool` (> _returnvalue (`KismetMathLibrary.Conv_IntToByte` (- (enumcount `/Game/Environment_BPs/Lock/Enum_Lock_Keys`) 1))) :`false` (cast `/Game/Environment_BPs/Lock/Enum_Lock_Keys` _returnvalue) :`true` "NewEnumerator1"))
  (bind (_direction _alpha) (`Timeline|Rotate Lock Key Timeline` :!via `PlayFromStart`)
    (:`Update`
      (`SceneComponent.K2_SetRelativeRotation` (`self.Lock Part Mesh`) (`KismetMathLibrary.RLerp` (select `/Game/Environment_BPs/Lock/Enum_Lock_Keys` (`self.Key Before Changing`) :`NewEnumerator1` (struct :`Yaw` 30.0) :`NewEnumerator2` (struct :`Yaw` 90.0) :`NewEnumerator0` (struct :`Yaw` 150.0) :`NewEnumerator3` (struct :`Yaw` 210.0) :`NewEnumerator4` (struct :`Yaw` 270.0) :`NewEnumerator5` (struct :`Yaw` 330.0) :!type "Rotator Structure") (select `/Game/Environment_BPs/Lock/Enum_Lock_Keys` (`self.Current Key`) :`NewEnumerator1` (struct :`Yaw` 30.0) :`NewEnumerator2` (struct :`Yaw` 90.0) :`NewEnumerator0` (struct :`Yaw` 150.0) :`NewEnumerator3` (struct :`Yaw` 210.0) :`NewEnumerator4` (struct :`Yaw` 270.0) :`NewEnumerator5` (struct :`Yaw` 330.0) :!type "Rotator Structure") _alpha true) false false))
    (:`Finished`
      (`/Game/Environment_BPs/Lock/BP_Full_Lock.Check Lock Combination` (`self.Associated Full Lock`)))))

(event `Reset Lock Part`
  (set `self.Current Key` (`self.Starting Key`))
  (`SceneComponent.K2_SetRelativeRotation` (`self.Lock Part Mesh`) (select `/Game/Environment_BPs/Lock/Enum_Lock_Keys` (`self.Starting Key`) :`NewEnumerator1` (struct :`Yaw` 30.0) :`NewEnumerator2` (struct :`Yaw` 90.0) :`NewEnumerator0` (struct :`Yaw` 150.0) :`NewEnumerator3` (struct :`Yaw` 210.0) :`NewEnumerator4` (struct :`Yaw` 270.0) :`NewEnumerator5` (struct :`Yaw` 330.0) :!type "Rotator Structure") false false))

(event `Rotate Prompt`
  (`SceneComponent.K2_SetWorldRotation` (`self.Interact Prompt`) (`KismetMathLibrary.FindLookAtRotation` (`SceneComponent.K2_GetComponentLocation` (`self.Interact Prompt`)) (`self.K2_GetActorLocation` (`GameplayStatics.GetPlayerCharacter` 0))) false false))

(event `Show Prompt`
  (`/Game/UI/Menus/WBP_Wiggly_Menu_Text.Fade Animation` (`self.Interact Text`) true)
  (bind _returnvalue (`KismetSystemLibrary.K2_SetTimerDelegate` (delegate `Rotate Prompt`) 0.05 true)))

(event `Hide Prompt`
  (`/Game/UI/Menus/WBP_Wiggly_Menu_Text.Fade Animation` (`self.Interact Text`) false)
  (`KismetSystemLibrary.K2_ClearAndInvalidateTimerHandle` (stale `Show Prompt` _returnvalue)))

(fn `UserConstructionScript`
  (bind _aswbp_wiggly_menu_text (cast `/Game/UI/Menus/WBP_Wiggly_Menu_Text` (`WidgetComponent.GetWidget` (`self.Interact Prompt`))))
  (bind _output_get (set `self.Interact Text` _aswbp_wiggly_menu_text))
  (set `/Game/UI/Menus/WBP_Wiggly_Menu_Text.Text` "LMB TURN" _output_get)
  (set `/Game/UI/Menus/WBP_Wiggly_Menu_Text.Size` 480.0 _output_get)
  (set `/Game/UI/Menus/WBP_Wiggly_Menu_Text.Irregular Shake Intensity?` false _output_get)
  (set `/Game/UI/Menus/WBP_Wiggly_Menu_Text.Shake Intensity` 0.05 _output_get)
  (set `/Game/UI/Menus/WBP_Wiggly_Menu_Text.Text Colour` (struct :`R` 1.0 :`G` 1.0 :`B` 1.0 :`A` 1.0) _output_get)
  (set `/Game/UI/Menus/WBP_Wiggly_Menu_Text.Shadow Colour` (struct :`R` 0.119792 :`A` 1.0) _output_get)
  (`SceneComponent.K2_SetRelativeRotation` (`self.Lock Part Mesh`) (select `/Game/Environment_BPs/Lock/Enum_Lock_Keys` (`self.Starting Key`) :`NewEnumerator1` (struct :`Yaw` 30.0) :`NewEnumerator2` (struct :`Yaw` 90.0) :`NewEnumerator0` (struct :`Yaw` 150.0) :`NewEnumerator3` (struct :`Yaw` 210.0) :`NewEnumerator4` (struct :`Yaw` 270.0) :`NewEnumerator5` (struct :`Yaw` 330.0) :!type "Rotator Structure") false false)
  (`|ExecutionSequence`
    (:`then_0`
      (bind _aswbp_lock_part_icon (cast `/Game/Environment_BPs/Lock/WBP_Lock_Part_Icon` (`WidgetComponent.GetWidget` (`self.Dynamite Icon`))))
      (set `/Game/Environment_BPs/Lock/WBP_Lock_Part_Icon.Associated Key` "NewEnumerator4" _aswbp_lock_part_icon)
      (`/Game/Environment_BPs/Lock/WBP_Lock_Part_Icon.Update Icon` _aswbp_lock_part_icon))
    (:`then_1`
      (bind _aswbp_lock_part_icon_2 (cast `/Game/Environment_BPs/Lock/WBP_Lock_Part_Icon` (`WidgetComponent.GetWidget` (`self.Pickaxe Icon`))))
      (set `/Game/Environment_BPs/Lock/WBP_Lock_Part_Icon.Associated Key` "NewEnumerator1" _aswbp_lock_part_icon_2)
      (`/Game/Environment_BPs/Lock/WBP_Lock_Part_Icon.Update Icon` _aswbp_lock_part_icon_2))
    (:`then_2`
      (bind _aswbp_lock_part_icon_3 (cast `/Game/Environment_BPs/Lock/WBP_Lock_Part_Icon` (`WidgetComponent.GetWidget` (`self.Gas Icon`))))
      (set `/Game/Environment_BPs/Lock/WBP_Lock_Part_Icon.Associated Key` "NewEnumerator5" _aswbp_lock_part_icon_3)
      (`/Game/Environment_BPs/Lock/WBP_Lock_Part_Icon.Update Icon` _aswbp_lock_part_icon_3))
    (:`then_3`
      (bind _aswbp_lock_part_icon_4 (cast `/Game/Environment_BPs/Lock/WBP_Lock_Part_Icon` (`WidgetComponent.GetWidget` (`self.Stopwatch Icon`))))
      (set `/Game/Environment_BPs/Lock/WBP_Lock_Part_Icon.Associated Key` "NewEnumerator3" _aswbp_lock_part_icon_4)
      (`/Game/Environment_BPs/Lock/WBP_Lock_Part_Icon.Update Icon` _aswbp_lock_part_icon_4))
    (:`then_4`
      (bind _aswbp_lock_part_icon_5 (cast `/Game/Environment_BPs/Lock/WBP_Lock_Part_Icon` (`WidgetComponent.GetWidget` (`self.Skull Icon`))))
      (set `/Game/Environment_BPs/Lock/WBP_Lock_Part_Icon.Associated Key` "NewEnumerator0" _aswbp_lock_part_icon_5)
      (`/Game/Environment_BPs/Lock/WBP_Lock_Part_Icon.Update Icon` _aswbp_lock_part_icon_5))
    (:`then_5`
      (bind _aswbp_lock_part_icon_6 (cast `/Game/Environment_BPs/Lock/WBP_Lock_Part_Icon` (`WidgetComponent.GetWidget` (`self.Rope Icon`))))
      (set `/Game/Environment_BPs/Lock/WBP_Lock_Part_Icon.Associated Key` "NewEnumerator2" _aswbp_lock_part_icon_6)
      (`/Game/Environment_BPs/Lock/WBP_Lock_Part_Icon.Update Icon` _aswbp_lock_part_icon_6))))