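; BP_Floating_Rock is an environment prop that plays an impact sound when something overlaps it.
; The construction script applies the configurable Mesh and Material to FloatingRockMesh, so instances can vary in look.
; A HitDetection overlap plays the Floating_Rock_Impact audio event at the actor's location, with a game-time cooldown to prevent rapid retriggering.
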(event `self.Hit Detection.OnComponentBeginOverlap`
  (params (OverlappedComponent :type "PrimitiveComponent Object Reference") (OtherActor :type "Actor Object Reference") (OtherComp :type "PrimitiveComponent Object Reference") (OtherBodyIndex :type Integer) (bFromSweep :type Boolean) (SweepResult :type "HitResult Structure (by ref)"))
  (if (>= (`KismetSystemLibrary.GetGameTimeInSeconds`) (+ (`self.Last Sound Production`) 0.5))
    (`FMODBlueprintStatics.PlayEventAtLocation` "/Game/FMOD/Events/Ambience/Floating_Rock_Impact.Floating_Rock_Impact" (`KismetMathLibrary.MakeTransform` (`self.K2_GetActorLocation`)))
    (set `self.Last Sound Production` (`KismetSystemLibrary.GetGameTimeInSeconds`))))

(fn `UserConstructionScript`
  (bind _floating_rock_mesh (`self.Floating Rock Mesh`))
  (`StaticMeshComponent.SetStaticMesh` _floating_rock_mesh (`self.Mesh`))
  (`PrimitiveComponent.SetMaterial` _floating_rock_mesh 0 (`self.Material`)))