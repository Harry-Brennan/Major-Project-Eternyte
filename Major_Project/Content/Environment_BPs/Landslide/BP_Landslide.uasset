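; Landslide obstacle that slides into place after a warning delay, damages the player while moving, then becomes a solid blockage destructible by dynamite.
; A timeline lerps the hidden mesh from neutral to active position with sound and Niagara effects, enabling collision at the end.
; An overlap, polled by timer until the required left-hand item is held, shows a player-facing prompt.
; Placed dynamite snaps to the player's side, then calls DynamiteExplosion after a fuse delay.
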(event `self.ReceiveBeginPlay`
  (`parent.ReceiveBeginPlay`)
  (`self.Reset Landslide`))

(event `Activate Landslide`
  (params (`Time until Landslide` :type "Float (double-precision)" :default 0.25))
  ;[1 1 1] Play landslide warning sounds
  (`FMODBlueprintStatics.PlayEventAtLocation` "/Game/FMOD/Events/Landslide/Landslide_Preparation.Landslide_Preparation" (`KismetMathLibrary.MakeTransform` (`SceneComponent.K2_GetComponentLocation` (`self.Landslide Active Position`))))
  (`KismetSystemLibrary.Delay` `Time until Landslide`)
  ;[1 1 1] Landslide sound
  (`FMODBlueprintStatics.PlayEventAtLocation` "/Game/FMOD/Events/Landslide/Landslide_Active.Landslide_Active" (`KismetMathLibrary.MakeTransform` (`SceneComponent.K2_GetComponentLocation` (`self.Landslide Active Position`))))
  (`self.Landslide Niagaras`)
  (`SceneComponent.SetHiddenInGame` (`self.Dynamite Destructible`) false false)
  (set `self.Landslide Moving` true)
  (bind (_direction _alpha) (`Timeline|Landslide Movement Timeline` :!via `PlayFromStart`)
    (:`Update`
      (`SceneComponent.K2_SetWorldLocation` (`self.Dynamite Destructible`) (`KismetMathLibrary.VLerp` (`SceneComponent.K2_GetComponentLocation` (`self.Landslide Neutral Position`)) (`SceneComponent.K2_GetComponentLocation` (`self.Landslide Active Position`)) _alpha) false false))
    (:`Finished`
      (`PrimitiveComponent.SetCollisionEnabled` (`self.Dynamite Destructible`) "QueryAndPhysics")
      (set `self.Active` true)
      (set `self.Landslide Moving` false)
      (set `self.Landslide Active` true))))

(event `Reset Landslide`
  (`SceneComponent.SetHiddenInGame` (`self.Dynamite Destructible`) true false)
  (`PrimitiveComponent.SetCollisionEnabled` (`self.Dynamite Destructible`) "NoCollision")
  (set `self.Active` false)
  (set `self.Landslide Moving` false)
  (set `self.Landslide Active` false)
  (`SceneComponent.SetHiddenInGame` (`self.Dynamite Placed Mesh`) true false))

(event `self.Push Player Collision.OnComponentBeginOverlap`
  (params (OverlappedComponent :type "PrimitiveComponent Object Reference") (OtherActor :type "Actor Object Reference") (OtherComp :type "PrimitiveComponent Object Reference") (OtherBodyIndex :type Integer) (bFromSweep :type Boolean) (SweepResult :type "HitResult Structure (by ref)"))
  (bind _returnvalue (`GameplayStatics.GetPlayerCharacter` 0))
  (if (`self.Landslide Moving`)
    (`/Game/Player/BPC_Player_Health.Player Take Damage` (`self.GetComponentByClass` _returnvalue "/Game/Player/BPC_Player_Health.BPC_Player_Health_C") 2.0 (`self.K2_GetActorLocation` _returnvalue) (0.0 0.0 0.0))))

(event `self.Activate Placed Dynamite`
  (`SceneComponent.K2_SetWorldTransform` (`self.Dynamite Placed Mesh`) (`KismetMathLibrary.SelectTransform` (`SceneComponent.K2_GetComponentToWorld` (`self.Forward Dynamite Placement`)) (`SceneComponent.K2_GetComponentToWorld` (`self.Backward Dynamite Placement`)) (`PrimitiveComponent.IsOverlappingActor` (`self.Forward Place Collision`) (`GameplayStatics.GetPlayerCharacter` 0))) false false)
  (`SceneComponent.SetHiddenInGame` (`self.Dynamite Placed Mesh`) false false)
  (`FMODBlueprintStatics.PlayEventAtLocation` "/Game/FMOD/Events/Dynamite/Dynamite_Fuse_then_Explode.Dynamite_Fuse_then_Explode" (`KismetMathLibrary.MakeTransform` (`SceneComponent.K2_GetComponentLocation` (`self.Dynamite Placed Mesh`))))
  (`LegacyCameraShake.StartLegacyCameraShake` (`GameplayStatics.GetPlayerCameraManager` 0) "/Game/Items/BP_Inventory_Camera_Shake.BP_Inventory_Camera_Shake_C")
  (`NiagaraFunctionLibrary.SpawnSystemAtLocation` "/Game/VFX/MsvFx_Niagara_Explosion_Pack_01/Prefabs/Niagara_Splash_Flame_01.Niagara_Splash_Flame_01" (`SceneComponent.K2_GetComponentLocation` (`self.Dynamite Placed Mesh`)) (struct) (1.0 1.0 1.0) true true "AutoRelease")
  (`KismetSystemLibrary.Delay` 1.75)
  (`self.Dynamite Explosion`))

(event `self.Player Detection Loop`
  (if (and (`|EnumEquality` (`/Game/Items/BPC_Inventory.Left Hand Item` (`self.GetComponentByClass` (`GameplayStatics.GetPlayerCharacter` 0) "/Game/Items/BPC_Inventory.BPC_Inventory_C")) "NewEnumerator3") (`KismetArrayLibrary.Array_IsNotEmpty` (`self.GetOverlappingActors` "/Game/Player/BP_Player.BP_Player_C")))
    (`SceneComponent.K2_SetWorldLocation` (`self.Dynamite Prompt`) (`KismetMathLibrary.SelectVector` (+ (`SceneComponent.K2_GetComponentLocation` (`self.Forward Dynamite Placement`)) (0.0 0.0 25.0)) (+ (`SceneComponent.K2_GetComponentLocation` (`self.Backward Dynamite Placement`)) (0.0 0.0 25.0)) (`PrimitiveComponent.IsOverlappingActor` (`self.Forward Place Collision`) (`GameplayStatics.GetPlayerCharacter` 0))) false false :!label _label)
    (`/Game/UI/Menus/WBP_Wiggly_Menu_Text.Fade Animation` (`self.Dynamite Prompt Widget`) true)
    (bind _returnvalue (`KismetSystemLibrary.K2_SetTimerDelegate` (delegate `self.Prompt Auto Rotation`) 0.01 true))
    (set `self.Prompt Auto Rotate Timer` _returnvalue)
    (set `self.Prompt Active` true)
    (`KismetSystemLibrary.K2_ClearAndInvalidateTimerHandle` (`self.Player Detection Loop Timer`))))

(event `self.Use Range.OnComponentBeginOverlap`
  (params (OverlappedComponent :type "PrimitiveComponent Object Reference") (OtherActor :type "Actor Object Reference") (OtherComp :type "PrimitiveComponent Object Reference") (OtherBodyIndex :type Integer) (bFromSweep :type Boolean) (SweepResult :type "HitResult Structure (by ref)"))
  (if (`PrimitiveComponent.K2_IsCollisionEnabled` (`self.Dynamite Destructible`))
    (if (`|EnumEquality` (`/Game/Items/BPC_Inventory.Left Hand Item` (`self.GetComponentByClass` (`GameplayStatics.GetPlayerCharacter` 0) "/Game/Items/BPC_Inventory.BPC_Inventory_C")) "NewEnumerator3")
      (goto _label)
      (else
        (bind _returnvalue (`KismetSystemLibrary.K2_SetTimerDelegate` (delegate `self.Player Detection Loop`) 0.25 true))
        (set `self.Player Detection Loop Timer` _returnvalue)))))

(event `self.Use Range.OnComponentEndOverlap`
  (params (OverlappedComponent :type "PrimitiveComponent Object Reference") (OtherActor :type "Actor Object Reference") (OtherComp :type "PrimitiveComponent Object Reference") (OtherBodyIndex :type Integer))
  (if (`PrimitiveComponent.K2_IsCollisionEnabled` (`self.Dynamite Destructible`)) :!label _label_2
    (if (`self.Prompt Active`)
      (`/Game/UI/Menus/WBP_Wiggly_Menu_Text.Fade Animation` (`self.Dynamite Prompt Widget`) false)
      (`KismetSystemLibrary.K2_ClearAndInvalidateTimerHandle` (`self.Prompt Auto Rotate Timer`))
      (set `self.Prompt Active` false))))

(event `self.Prompt Auto Rotation`
  (`SceneComponent.K2_SetWorldRotation` (`self.Dynamite Prompt`) (`KismetMathLibrary.FindLookAtRotation` (`SceneComponent.K2_GetComponentLocation` (`self.Dynamite Prompt`)) (`self.K2_GetActorLocation` (stale `self.Use Range.OnComponentBeginOverlap` OtherActor))) false false)
  (`SceneComponent.K2_SetWorldLocation` (`self.Dynamite Prompt`) (`KismetMathLibrary.SelectVector` (+ (`SceneComponent.K2_GetComponentLocation` (`self.Forward Dynamite Placement`)) (0.0 0.0 25.0)) (+ (`SceneComponent.K2_GetComponentLocation` (`self.Backward Dynamite Placement`)) (0.0 0.0 25.0)) (`PrimitiveComponent.IsOverlappingActor` (`self.Forward Place Collision`) (`GameplayStatics.GetPlayerCharacter` 0))) false false))

(event `self.Force Hide Prompt`
  (goto _label_2))

(fn `Landslide Niagaras`
  (bind _returnvalue (`SceneComponent.K2_GetComponentLocation` (`self.Landslide Active Position`)))
  (`NiagaraFunctionLibrary.SpawnSystemAtLocation` "/Game/VFX/MsvFx_Niagara_Explosion_Pack_01/Prefabs/Niagara_Dust_Explosion_01.Niagara_Dust_Explosion_01" _returnvalue (struct) (3.0 3.0 3.0) true true "AutoRelease")
  (`NiagaraFunctionLibrary.SpawnSystemAtLocation` "/Game/VFX/MsvFx_Niagara_Explosion_Pack_01/Prefabs/Niagara_Explosion_03.Niagara_Explosion_03" _returnvalue (struct) (1.0 1.0 1.0) true true "AutoRelease"))

(fn `UserConstructionScript`)