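; BP_Decaying_Tree is an environment tree that can switch between a living and a dead state.
; DecayTree spawns a Niagara transformation effect at the DecayNiagaraLocation component, then swaps TreeMesh to a dead-tree static mesh with a larger relative scale.
; ResetTree restores the original mesh at unit scale without playing an effect.
; Both events are instant swaps, and nothing in the file calls them.
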(event `Decay Tree`
  (`NiagaraFunctionLibrary.SpawnSystemAtLocation` "/Game/VFX/Environment/NS_Decaying_Tree_Transformation.NS_Decaying_Tree_Transformation" (`SceneComponent.K2_GetComponentLocation` (`self.Decay Niagara Location`)) (struct) (2.0 2.0 2.0))
  (`StaticMeshComponent.SetStaticMesh` (`self.Tree Mesh`) "/Game/Level_Assets/Temple/Foliage/TreeDead_01/sm_TreeDead_01_01.sm_TreeDead_01_01")
  (`SceneComponent.SetRelativeScale3D` (`self.Tree Mesh`) (2.173913 2.173913 2.173913)))

(event `Reset Tree`
  (`StaticMeshComponent.SetStaticMesh` (`self.Tree Mesh`) "/Game/Level_Assets/Temple/Foliage/Tree_02/sm_Tree_02_01.sm_Tree_02_01")
  (`SceneComponent.SetRelativeScale3D` (`self.Tree Mesh`) (1.0 1.0 1.0)))

(fn `UserConstructionScript`)