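; Manager for the Fog Twin environment that shifts fog from an upper emitter to lower ones as the game loop progresses.
; Each tick it reads the current loop time from the game mode and maps it, clamped over ten minutes, to Niagara "Fog Spawn Rate" values.
; Lower fogs ramp up from zero, with the last array entry growing far denser, while the upper fog fades out.
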(event `self.ReceiveTick`
  (params (DeltaSeconds :type "Float (single-precision)"))
  (bind _lower_fogs (`self.Lower Fogs`))
  (bind _current_loop_time (message `/Game/Core/Modes/BPI_Gamemode.Get Current Loop Time` (`GameplayStatics.GetGameMode`)))
  (for (_array_element _array_index) _lower_fogs
    (`NiagaraComponent.SetVariableFloat` (`NiagaraActor.NiagaraComponent` _array_element) "Fog Spawn Rate" (`KismetMathLibrary.SelectFloat` (`KismetMathLibrary.MapRangeClamped` _current_loop_time 0.0 600.0 0.0 8000.0) (`KismetMathLibrary.MapRangeClamped` _current_loop_time 0.0 600.0 0.0 200.0) (== _array_index (`KismetArrayLibrary.Array_LastIndex` _lower_fogs)))))
  (`NiagaraComponent.SetVariableFloat` (`NiagaraActor.NiagaraComponent` (`self.Upper Fog`)) "Fog Spawn Rate" (`KismetMathLibrary.MapRangeClamped` _current_loop_time 0.0 600.0 3000.0)))

(fn `UserConstructionScript`)