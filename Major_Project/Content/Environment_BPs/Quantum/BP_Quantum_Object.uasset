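; Quantum object that relocates to the next of its preset transforms once the player has looked away from it for a minimum time.
; A looping detection check combines camera FOV angle and a line trace; looking back cancels the pending move.
; The move skips an occupied spot, swaps mesh, flickers in with sound and dust, then briefly enables a damaging KillBox before detection restarts.
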(event `self.ReceiveBeginPlay`
  (bind _asbp_player (cast `/Game/Player/BP_Player` (`GameplayStatics.GetPlayerCharacter` 0)))
  (set `self.Player Ref` _asbp_player)
  (set `self.Starting Transform` (`self.GetTransform`)))

(event `Reset Quantum Object`
  (`self.K2_SetActorTransform` (`self.Starting Transform`)))

(event `Quantum Look Detection Loop`
  (bind _player_ref (`self.Player Ref`))
  (bind _player_camera (`/Game/Player/BP_Player.Player Camera` (`self.Player Ref`)))
  (if (`KismetMathLibrary.InRange_FloatFloat` (`KismetMathLibrary.DegAcos` (`KismetMathLibrary.Dot_VectorVector` (`KismetMathLibrary.GetDirectionUnitVector` (`SceneComponent.K2_GetComponentLocation` _player_camera) (`self.K2_GetActorLocation`)) (`SceneComponent.GetForwardVector` _player_camera))) 0.0 (* (`PlayerCameraManager.GetFOVAngle` (`GameplayStatics.GetPlayerCameraManager` 0)) (`self.FOV Look Multiplier`)))
    (bind (_outhit _returnvalue) (`KismetSystemLibrary.LineTraceSingle` (`SceneComponent.K2_GetComponentLocation` (`self.Trace Start`)) (+ (`SceneComponent.K2_GetComponentLocation` (`/Game/Player/BP_Player.Player Camera` _player_ref)) (* (`KismetMathLibrary.GetForwardVector` (`KismetMathLibrary.FindLookAtRotation` (`SceneComponent.K2_GetComponentLocation` (`self.Trace Start`)) (`self.K2_GetActorLocation` _player_ref))) 25.0)) "TraceTypeQuery1" false (`|MakeArray` (`self.Player Ref`) :!type "Actor Object Reference") "ForOneFrame"))
    (if _returnvalue
      (if (`self.Being Looked At`) :!label _label
        (set `self.Being Looked At` false)
        (bind _returnvalue_2 (`KismetSystemLibrary.K2_SetTimerDelegate` (delegate `Deactivate Look Detection`) (`self.Look Away Min Time`)))
        (set `self.Deactivate Look Detection Timer` _returnvalue_2)
        (bind _returnvalue_3 (`KismetSystemLibrary.K2_SetTimerDelegate` (delegate `Move Quantum`) (`self.Look Away Min Time`)))
        (set `self.Move Quantum Timer` _returnvalue_3))
      (elif (not (`self.Being Looked At`))
        (set `self.Being Looked At` true)
        (`KismetSystemLibrary.K2_ClearAndInvalidateTimerHandle` (`self.Deactivate Look Detection Timer`))
        (`KismetSystemLibrary.K2_ClearAndInvalidateTimerHandle` (`self.Move Quantum Timer`))))
    (else
      (goto _label))))

(event `Move Quantum`
  (bind _found_current_transform_index (`self.Found Current Transform Index`))
  (bind _returnvalue (`KismetArrayLibrary.Array_LastIndex` (`self.Total Possible Transforms`)))
  (bind _returnvalue_2 (`SceneComponent.K2_GetComponentLocation` (`self.Quantum Mesh`)))
  (bind _returnvalue_3 (`SceneComponent.K2_GetComponentLocation` (`self.Quantum Mesh`)))
  (bind _returnvalue_4 (+ (`self.Found Current Transform Index`) 2))
  (bind _returnvalue_5 (`KismetMathLibrary.SelectInt` 0 (+ _found_current_transform_index 1) (== _found_current_transform_index (`KismetArrayLibrary.Array_LastIndex` (`self.Total Possible Transforms`)))))
  (bind _output (`|GetArrayItem` (`self.Total Possible Transforms`) _returnvalue_5))
  (bind _location (.location _output))
  (for (_array_element _array_index) (`self.Total Possible Transforms`)
    (if (`KismetMathLibrary.NearlyEqual_TransformTransform` _array_element (`self.GetTransform`) 1.0 1.0 1.0)
      (set `self.Found Current Transform Index` _array_index)
      (break)))
  (`FMODBlueprintStatics.PlayEventAtLocation` "/Game/FMOD/Events/Quantum_Object/Quantum_Disappear.Quantum_Disappear" (`KismetMathLibrary.MakeTransform` _returnvalue_3))
  (`NiagaraFunctionLibrary.SpawnSystemAtLocation` "/Game/VFX/MsvFx_Niagara_Explosion_Pack_01/Prefabs/Niagara_Dust_Explosion_01.Niagara_Dust_Explosion_01" _returnvalue_3 (struct) (1.0 1.0 1.0) true true "AutoRelease")
  (`self.SetActorHiddenInGame` true)
  (`self.SetActorEnableCollision` false)
  (`KismetSystemLibrary.Delay` 1.0)
  (bind (_outhit _returnvalue_6) (`KismetSystemLibrary.SphereTraceSingleForObjects` _location _location 15.0 (`|MakeArray` "ObjectTypeQuery10" :!type "EObjectTypeQuery Enum") false (`|MakeArray` self :!type "Actor Object Reference")))
  (if _returnvalue_6
    (set `self.New Transform` (`|GetArrayItem` (`self.Total Possible Transforms`) (`KismetMathLibrary.SelectInt` 1 (`KismetMathLibrary.SelectInt` 0 _returnvalue_4 (> _returnvalue_4 _returnvalue)) (== (`self.Found Current Transform Index`) _returnvalue))))
    (else
      (set `self.New Transform` _output)))
  (`StaticMeshComponent.SetStaticMesh` (`self.Quantum Mesh`) (`|GetArrayItem` (`self.Transform Index -> Static Mesh`) _returnvalue_5))
  (`self.SetActorHiddenInGame` false)
  (`self.K2_SetActorTransform` (`self.New Transform`))
  (`KismetSystemLibrary.Delay` 0.1)
  (`self.SetActorHiddenInGame` true)
  (`KismetSystemLibrary.Delay` 0.1)
  (`self.SetActorHiddenInGame` false)
  (`KismetSystemLibrary.Delay` 0.1)
  (`self.SetActorHiddenInGame` true)
  (`KismetSystemLibrary.Delay` 0.1)
  (`FMODBlueprintStatics.PlayEventAtLocation` "/Game/FMOD/Events/Quantum_Object/Quantum_Reappear.Quantum_Reappear" (`KismetMathLibrary.MakeTransform` _returnvalue_2))
  (`NiagaraFunctionLibrary.SpawnSystemAtLocation` "/Game/VFX/MsvFx_Niagara_Explosion_Pack_01/Prefabs/Niagara_Dust_Explosion_01.Niagara_Dust_Explosion_01" _returnvalue_2 (struct) (1.0 1.0 1.0) true true "AutoRelease")
  (`self.SetActorHiddenInGame` false)
  (`self.SetActorEnableCollision` true)
  (`KismetSystemLibrary.Delay` 1.0)
  (set `PrimitiveComponent.bGenerateOverlapEvents` true (`self.Kill Box`))
  (`|ExecutionSequence`
    (:`then_0`
      (bind _returnvalue_7 (`KismetSystemLibrary.K2_SetTimer` null "Quantum Look Detection Loop" 0.05 true false 5.0))
      (set `self.Quantum Look Detection Timer` _returnvalue_7))
    (:`then_1`
      (`KismetSystemLibrary.Delay` 3.0)
      (set `PrimitiveComponent.bGenerateOverlapEvents` false (`self.Kill Box`)))))

(event `Deactivate Look Detection`
  (`KismetSystemLibrary.K2_ClearAndInvalidateTimerHandle` (`self.Quantum Look Detection Timer`)))

(event `self.Kill Box.OnComponentBeginOverlap`
  (params (OverlappedComponent :type "PrimitiveComponent Object Reference") (OtherActor :type "Actor Object Reference") (OtherComp :type "PrimitiveComponent Object Reference") (OtherBodyIndex :type Integer) (bFromSweep :type Boolean) (SweepResult :type "HitResult Structure (by ref)"))
  (`/Game/Player/BPC_Player_Health.Player Take Damage` (`self.GetComponentByClass` (`GameplayStatics.GetPlayerCharacter` 0) "/Game/Player/BPC_Player_Health.BPC_Player_Health_C") 5.0 (`self.K2_GetActorLocation`) (0.0 0.0 0.0)))

(fn `UserConstructionScript`)