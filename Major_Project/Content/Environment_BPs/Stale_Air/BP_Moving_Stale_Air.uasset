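; Moving stale air hazard actor whose collision volume travels from a neutral point to an active point.
; On BeginPlay it parks the volume at the neutral position with collision disabled.
; Activation enables collision and plays a timeline, rate-scaled by TotalMovementTime, that lerps the volume between the two marker components' world locations.
; Deactivation disables collision and snaps it back to neutral.
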(event `self.ReceiveBeginPlay`
  (`parent.ReceiveBeginPlay`)
  (`self.Deactivate Stale Air Movement`))

(event `Activate Stale Air Movement`
  (`PrimitiveComponent.SetCollisionEnabled` (`self.Stale Air Collision`) "QueryAndPhysics")
  (`TimelineComponent.SetPlayRate` (`self.Stale Air Movement Timeline`) (/ 1.0 (`self.Total Movement Time`)))
  (bind (_direction _alpha) (`Timeline|Stale Air Movement Timeline` :!via `PlayFromStart`)
    (:`Update`
      (`SceneComponent.K2_SetWorldLocation` (`self.Stale Air Collision`) (`KismetMathLibrary.VLerp` (`SceneComponent.K2_GetComponentLocation` (`self.Stale Air Neutral Position`)) (`SceneComponent.K2_GetComponentLocation` (`self.Stale Air Active Position`)) _alpha) false false))))

(event `Deactivate Stale Air Movement`
  (`PrimitiveComponent.SetCollisionEnabled` (`self.Stale Air Collision`) "NoCollision")
  (`SceneComponent.K2_SetWorldLocation` (`self.Stale Air Collision`) (`SceneComponent.K2_GetComponentLocation` (`self.Stale Air Neutral Position`)) false false))

(fn `UserConstructionScript`
  (`parent.UserConstructionScript`))