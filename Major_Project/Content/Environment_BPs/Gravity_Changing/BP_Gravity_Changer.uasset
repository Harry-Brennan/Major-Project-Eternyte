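; BP_Gravity_Changer is a volume that scales gravity for characters and objects inside it by GravityPercentage.
; Overlapping characters get their CharacterMovement GravityScale changed, then reset to 1 on exit.
; Other actors have mesh gravity disabled and join a list that a looping timer pushes down with mass-scaled force, using the percentage clamped to 0–1.
; Activate and Deactivate events set an Active flag, which these graphs never read.
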(event `self.ReceiveBeginPlay`
  (for _array_element (`self.GetOverlappingActors` null)
    (cast `/Game/Player/BP_Player` _array_element
      (:`CastFailed`
        (`KismetArrayLibrary.Array_Add` (`self.Affected Non-Players`) _array_element)
        (`PrimitiveComponent.SetEnableGravity` (`self.GetComponentByClass` _array_element "/Script/Engine.StaticMeshComponent") false))))
  (if (not (`KismetArrayLibrary.Array_IsEmpty` (`self.Affected Non-Players`)))
    (bind _returnvalue (`KismetSystemLibrary.K2_SetTimerDelegate` (delegate `Gravity Object Loop`) 0.01 true :!label _label))))

(event `Activate Gravity Changer`
  (set `self.Active` true))

(event `Deactivate Gravity Changer`
  (set `self.Active` false))

(event `Gravity Object Loop`
  (for _array_element (`self.Affected Non-Players`)
    (bind _returnvalue (`self.GetComponentByClass` _array_element "/Script/Engine.StaticMeshComponent"))
    (`PrimitiveComponent.AddForce` _returnvalue (`KismetMathLibrary.MakeVector` 0.0 0.0 (* (`PrimitiveComponent.GetMass` _returnvalue) (* -980.0 (`KismetMathLibrary.FClamp` (`self.Gravity Percentage`))))) "None" false)))

(event `self.Gravity Changer Collision.OnComponentBeginOverlap`
  (params (OverlappedComponent :type "PrimitiveComponent Object Reference") (OtherActor :type "Actor Object Reference") (OtherComp :type "PrimitiveComponent Object Reference") (OtherBodyIndex :type Integer) (bFromSweep :type Boolean) (SweepResult :type "HitResult Structure (by ref)"))
  (bind _returnvalue (`self.GetComponentByClass` OtherActor "/Script/Engine.CharacterMovementComponent"))
  (`/Engine/EditorBlueprintResources/StandardMacros.IsValid` _returnvalue
    (:`Is Valid`
      (set `CharacterMovementComponent.GravityScale` (`self.Gravity Percentage`) _returnvalue))
    (:`Is Not Valid`
      (`KismetArrayLibrary.Array_Add` (`self.Affected Non-Players`) OtherActor)
      (`PrimitiveComponent.SetEnableGravity` (`self.GetComponentByClass` OtherActor "/Script/Engine.StaticMeshComponent") false)
      (goto _label))))

(event `self.Gravity Changer Collision.OnComponentEndOverlap`
  (params (OverlappedComponent :type "PrimitiveComponent Object Reference") (OtherActor :type "Actor Object Reference") (OtherComp :type "PrimitiveComponent Object Reference") (OtherBodyIndex :type Integer))
  (bind _returnvalue (`self.GetComponentByClass` OtherActor "/Script/Engine.CharacterMovementComponent"))
  (`/Engine/EditorBlueprintResources/StandardMacros.IsValid` _returnvalue
    (:`Is Valid`
      (set `CharacterMovementComponent.GravityScale` 1.0 _returnvalue))
    (:`Is Not Valid`
      (`KismetArrayLibrary.Array_RemoveItem` (`self.Affected Non-Players`) OtherActor)
      (`PrimitiveComponent.SetEnableGravity` (`self.GetComponentByClass` OtherActor "/Script/Engine.StaticMeshComponent") true)
      (if (`KismetArrayLibrary.Array_IsEmpty` (`self.Affected Non-Players`))
        (`KismetSystemLibrary.K2_ClearAndInvalidateTimerHandle` (stale `self.ReceiveBeginPlay` _returnvalue))))))

(fn `UserConstructionScript`)