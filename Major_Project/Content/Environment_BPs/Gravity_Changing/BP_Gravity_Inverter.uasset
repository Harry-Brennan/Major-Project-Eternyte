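; BP_Gravity_Inverter is a switchable zone that turns antigravity on for the player while inside it.
; While active, begin and end overlap on its GravityInvertCollision call ActivateAntigravity and DeactivateAntigravity on BP_Player.
; ActivateGravityInverter and DeactivateGravityInverter toggle the Active flag and immediately apply or remove antigravity if the player is already overlapping the actor.
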(event `self.Gravity Invert Collision.OnComponentBeginOverlap`
  (params (OverlappedComponent :type "PrimitiveComponent Object Reference") (OtherActor :type "Actor Object Reference") (OtherComp :type "PrimitiveComponent Object Reference") (OtherBodyIndex :type Integer) (bFromSweep :type Boolean) (SweepResult :type "HitResult Structure (by ref)"))
  (if (`self.Active`)
    (bind _asbp_player (cast `/Game/Player/BP_Player` OtherActor))
    (`/Game/Player/BP_Player.Activate Anti-gravity` _asbp_player)))

(event `self.Gravity Invert Collision.OnComponentEndOverlap`
  (params (OverlappedComponent :type "PrimitiveComponent Object Reference") (OtherActor :type "Actor Object Reference") (OtherComp :type "PrimitiveComponent Object Reference") (OtherBodyIndex :type Integer))
  (if (`self.Active`)
    (bind _asbp_player (cast `/Game/Player/BP_Player` OtherActor))
    (`/Game/Player/BP_Player.Deactivate Anti-gravity` _asbp_player)))

(event `Activate Gravity Inverter`
  (bind _returnvalue (`GameplayStatics.GetPlayerCharacter` 0))
  (set `self.Active` true)
  (if (`self.IsOverlappingActor` _returnvalue)
    (bind _asbp_player (cast `/Game/Player/BP_Player` _returnvalue))
    (`/Game/Player/BP_Player.Activate Anti-gravity` _asbp_player)))

(event `Deactivate Gravity Inverter`
  (bind _returnvalue (`GameplayStatics.GetPlayerCharacter` 0))
  (if (`self.Active`)
    (if (`self.IsOverlappingActor` _returnvalue)
      (bind _asbp_player (cast `/Game/Player/BP_Player` _returnvalue))
      (`/Game/Player/BP_Player.Deactivate Anti-gravity` _asbp_player))
    (set `self.Active` false)))

(fn `UserConstructionScript`)