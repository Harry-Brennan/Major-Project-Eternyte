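; BP_Minecart is a rideable minecart that carries the player along a spline track and drops them at an exit point.
; The construction script builds rail spline meshes between spline points and places the cart at the start.
; An overlap zone shows a player-facing "LMB RIDE" prompt; StartMinecart locks movement and drives cart and player along the spline by timeline, timed by MinecartTotalTime.
; Camera fades mask boarding and exit teleports, and ResetMinecart re-arms the ride.
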(event `self.ReceiveBeginPlay`
  (bind _aswbp_wiggly_menu_text (cast `/Game/UI/Menus/WBP_Wiggly_Menu_Text` (`WidgetComponent.GetWidget` (`self.Interact Widget`))))
  (bind _output_get (set `self.Interact Text` _aswbp_wiggly_menu_text))
  (set `/Game/UI/Menus/WBP_Wiggly_Menu_Text.Text` "LMB RIDE" _output_get)
  (set `/Game/UI/Menus/WBP_Wiggly_Menu_Text.Size` 480.0 _output_get)
  (set `/Game/UI/Menus/WBP_Wiggly_Menu_Text.Irregular Shake Intensity?` false _output_get)
  (set `/Game/UI/Menus/WBP_Wiggly_Menu_Text.Shake Intensity` 0.05 _output_get)
  (set `/Game/UI/Menus/WBP_Wiggly_Menu_Text.Text Colour` (struct :`R` 1.0 :`G` 1.0 :`B` 1.0 :`A` 1.0) _output_get)
  (set `/Game/UI/Menus/WBP_Wiggly_Menu_Text.Shadow Colour` (struct :`R` 0.119792 :`A` 1.0) _output_get)
  (`Widget.SetRenderOpacity` (`/Game/UI/Menus/WBP_Wiggly_Menu_Text.WiggleTextWrapBox` (`self.Interact Text`)) 0.0))

(event `Reset Minecart`
  (bind _minecart_track (`self.Minecart Track`))
  (`SceneComponent.K2_SetWorldLocationAndRotation` (`self.Minecart SM`) (`SplineComponent.GetLocationAtDistanceAlongSpline` _minecart_track 0.0 "World") (`SplineComponent.GetRotationAtDistanceAlongSpline` _minecart_track 0.0 "World") false false)
  (set `self.Active` false)
  (set `PrimitiveComponent.bGenerateOverlapEvents` true (`self.Interact / Ride Collision`)))

(event `Start Minecart`
  (bind _returnvalue (`GameplayStatics.GetPlayerController` 0))
  (bind _returnvalue_2 (`GameplayStatics.GetPlayerCharacter` 0))
  (bind _minecart_track (`self.Minecart Track`))
  (if (not (`self.Active`))
    (set `PrimitiveComponent.bGenerateOverlapEvents` false (`self.Interact / Ride Collision`))
    (`FMODBlueprintStatics.PlayEventAtLocation` "/Game/FMOD/Events/Minecart/Minecart_Start_End.Minecart_Start_End" (`KismetMathLibrary.MakeTransform` (`SceneComponent.K2_GetComponentLocation` (`self.Minecart SM`))))
    (`KismetSystemLibrary.K2_ClearAndInvalidateTimerHandle` (`self.Rotate Prompt to Player Timer`))
    (`/Game/UI/Menus/WBP_Wiggly_Menu_Text.Fade Animation` (`self.Interact Text`) false)
    (`PlayerCameraManager.StartCameraFade` :`self` (`GameplayStatics.GetPlayerCameraManager` 0) :`ToAlpha` 1.0 :`Duration` 0.2 :`bHoldWhenFinished` true)
    (`KismetSystemLibrary.Delay` 0.2)
    (`Controller.SetIgnoreMoveInput` _returnvalue true)
    (`Controller.SetControlRotation` _returnvalue (`SplineComponent.GetRotationAtDistanceAlongSpline` (`self.Minecart Track`) 0.0 "World"))
    (`self.SetActorEnableCollision` _returnvalue_2 false)
    (`self.K2_SetActorLocation` _returnvalue_2 (`SceneComponent.K2_GetComponentLocation` (`self.Player Position Within Minecart`)) false true)
    (set `self.Active` true)
    (`TimelineComponent.SetPlayRate` (`self.Move Minecart Along Track Timeline`) (/ 1.0 (`self.Minecart Total Time`)))
    (`KismetSystemLibrary.Delay` 0.15)
    (`PlayerCameraManager.StartCameraFade` :`self` (`GameplayStatics.GetPlayerCameraManager` 0) :`FromAlpha` 1.0 :`Duration` 0.15)
    (`KismetSystemLibrary.Delay` 0.2)
    (`ActorComponent.Activate` (`self.Minecart Active Audio`) false)
    (bind (_direction _alpha) (`Timeline|Move Minecart Along Track Timeline` :!via `PlayFromStart`)
      (:`Update`
        (bind _returnvalue_3 (* (`SplineComponent.GetSplineLength` _minecart_track) _alpha))
        (`SceneComponent.K2_SetWorldLocationAndRotation` (`self.Minecart SM`) (`SplineComponent.GetLocationAtDistanceAlongSpline` _minecart_track _returnvalue_3 "World") (`SplineComponent.GetRotationAtDistanceAlongSpline` _minecart_track _returnvalue_3 "World") false false)
        (`self.K2_SetActorLocation` (`GameplayStatics.GetPlayerCharacter` 0) (`SceneComponent.K2_GetComponentLocation` (`self.Player Position Within Minecart`)) false true))
      (:`Finished`
        (`self.Stop Minecart`)
        (`ActorComponent.Deactivate` (`self.Minecart Active Audio`))))))

(event `Stop Minecart`
  (bind _returnvalue (`GameplayStatics.GetPlayerController` 0))
  (bind _leave_minecart_position (`self.Leave Minecart Position`))
  (`PlayerCameraManager.StartCameraFade` :`self` (`GameplayStatics.GetPlayerCameraManager` 0) :`ToAlpha` 1.0 :`Duration` 0.2 :`bHoldWhenFinished` true)
  (`FMODBlueprintStatics.PlayEventAtLocation` "/Game/FMOD/Events/Minecart/Minecart_Start_End.Minecart_Start_End" (`KismetMathLibrary.MakeTransform` (`SceneComponent.K2_GetComponentLocation` (`self.Minecart SM`))))
  (`KismetSystemLibrary.Delay` 0.25)
  (`self.K2_SetActorLocation` (`GameplayStatics.GetPlayerCharacter` 0) (`SceneComponent.K2_GetComponentLocation` _leave_minecart_position) false true)
  (`self.SetActorEnableCollision` (`GameplayStatics.GetPlayerCharacter` 0) true)
  (`Controller.SetIgnoreMoveInput` _returnvalue false)
  (`Controller.SetControlRotation` _returnvalue (`SceneComponent.K2_GetComponentRotation` _leave_minecart_position))
  (`KismetSystemLibrary.Delay` 0.15)
  (`PlayerCameraManager.StartCameraFade` :`self` (`GameplayStatics.GetPlayerCameraManager` 0) :`FromAlpha` 1.0 :`Duration` 0.15))

(event `self.Interact / Ride Collision.OnComponentEndOverlap`
  (params (OverlappedComponent :type "PrimitiveComponent Object Reference") (OtherActor :type "Actor Object Reference") (OtherComp :type "PrimitiveComponent Object Reference") (OtherBodyIndex :type Integer))
  (`/Game/UI/Menus/WBP_Wiggly_Menu_Text.Fade Animation` (`self.Interact Text`) false)
  (`KismetSystemLibrary.K2_ClearAndInvalidateTimerHandle` (`self.Rotate Prompt to Player Timer`)))

(event `self.Interact / Ride Collision.OnComponentBeginOverlap`
  (params (OverlappedComponent :type "PrimitiveComponent Object Reference") (OtherActor :type "Actor Object Reference") (OtherComp :type "PrimitiveComponent Object Reference") (OtherBodyIndex :type Integer) (bFromSweep :type Boolean) (SweepResult :type "HitResult Structure (by ref)"))
  (if (not (`self.Active`))
    (`SceneComponent.K2_SetWorldRotation` (`self.Interact Widget`) (`KismetMathLibrary.FindLookAtRotation` (`SceneComponent.K2_GetComponentLocation` (`self.Interact Widget`)) (`self.K2_GetActorLocation` (`GameplayStatics.GetPlayerCharacter` 0))) false false)
    (`/Game/UI/Menus/WBP_Wiggly_Menu_Text.Fade Animation` (`self.Interact Text`) true)
    (bind _returnvalue (`KismetSystemLibrary.K2_SetTimerDelegate` (delegate `Rotate Prompt to Player`) 0.01 true))
    (set `self.Rotate Prompt to Player Timer` _returnvalue)))

(event `Rotate Prompt to Player`
  (`SceneComponent.K2_SetWorldRotation` (`self.Interact Widget`) (`KismetMathLibrary.FindLookAtRotation` (`SceneComponent.K2_GetComponentLocation` (`self.Interact Widget`)) (`self.K2_GetActorLocation` (`GameplayStatics.GetPlayerCharacter` 0))) false false))

(fn `UserConstructionScript`
  (bind _minecart_track (`self.Minecart Track`))
  (bind _minecart_track_2 (`self.Minecart Track`))
  (bind (_returnvalue_roll _returnvalue_pitch _returnvalue_yaw) (`KismetMathLibrary.BreakRotator` (`SplineComponent.GetRotationAtDistanceAlongSpline` _minecart_track_2 0.0 "World")))
  (for _index (range (+ (- (`SplineComponent.GetNumberOfSplinePoints` (`self.Minecart Track`)) 2) 1))
    (bind _returnvalue (`AddComponent|NODE_AddSplineMeshComponent-0` :`bManualAttachment` true))
    (`StaticMeshComponent.SetStaticMesh` _returnvalue "/Game/Level_Assets/Scene_OldMine/Assets/Megascans/3D_Assets/Ind_Min_Rail_Metal_Pack_01/SM_Ind_Min_Rail_Metal_Pack_01_C.SM_Ind_Min_Rail_Metal_Pack_01_C")
    (bind (_location _tangent) (`SplineComponent.GetLocationAndTangentAtSplinePoint` _minecart_track _index "World"))
    (bind (_location_2 _tangent_2) (`SplineComponent.GetLocationAndTangentAtSplinePoint` _minecart_track (+ _index 1) "World"))
    (`SplineMeshComponent.SetStartAndEnd` _returnvalue _location _tangent _location_2 _tangent_2 true)
    (bind _aswbp_wiggly_menu_text (cast `/Game/UI/Menus/WBP_Wiggly_Menu_Text` (`WidgetComponent.GetWidget` (`self.Interact Widget`)) :!label _label))
    (bind _output_get (set `self.Interact Text` _aswbp_wiggly_menu_text))
    (set `/Game/UI/Menus/WBP_Wiggly_Menu_Text.Text` "LMB RIDE" _output_get)
    (set `/Game/UI/Menus/WBP_Wiggly_Menu_Text.Size` 480.0 _output_get)
    (set `/Game/UI/Menus/WBP_Wiggly_Menu_Text.Irregular Shake Intensity?` false _output_get)
    (set `/Game/UI/Menus/WBP_Wiggly_Menu_Text.Shake Intensity` 0.05 _output_get)
    (set `/Game/UI/Menus/WBP_Wiggly_Menu_Text.Text Colour` (struct :`R` 1.0 :`G` 1.0 :`B` 1.0 :`A` 1.0) _output_get)
    (set `/Game/UI/Menus/WBP_Wiggly_Menu_Text.Shadow Colour` (struct :`R` 0.119792 :`A` 1.0) _output_get)
    (`SceneComponent.K2_SetWorldLocationAndRotation` (`self.Minecart SM`) (`SplineComponent.GetLocationAtDistanceAlongSpline` _minecart_track_2 0.0 "World") (`KismetMathLibrary.MakeRotator` _returnvalue_roll _returnvalue_pitch (+ 90.0 _returnvalue_yaw)) false false))
  (goto _label))