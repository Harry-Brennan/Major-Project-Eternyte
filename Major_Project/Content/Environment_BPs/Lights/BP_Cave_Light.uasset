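; Configurable cave light actor that shows a mesh with either a point or spot light, driven by a LightInfo struct.
; Organic lights use timers to start random flicker bursts that briefly dim the intensity.
; A chase sequence strobes the light red on a looping timer that speeds up with chase intensity.
; An optional lifetime timeline scales brightness over a set duration, and starting a chase cancels it.
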(event `/Game/Environment_BPs/Lights/BPI_Cave_Light.Update Light Info`
  (params (`Cave Light Info` :type "/Game/Environment_BPs/Lights/Struct_Cave_Light_Info Structure"))
  (bind (_lighttype _lightintensity _attenuationradius _lightcolour _usetemperature _temperature) (break `/Game/Environment_BPs/Lights/Struct_Cave_Light_Info` (`self.Light Info`)))
  (set `self.Light Info` `Cave Light Info`)
  (`LightComponent.SetIntensity` (select `/Game/Environment_BPs/Lights/Enum_Cave_Light_Types` _lighttype :`NewEnumerator0` (`self.Cave Light Point`) :`NewEnumerator2` (`self.Cave Light Spot`) :!type "LightComponent Object Reference") _lightintensity)
  (`LocalLightComponent.SetAttenuationRadius` (select `/Game/Environment_BPs/Lights/Enum_Cave_Light_Types` _lighttype :`NewEnumerator0` (`self.Cave Light Point`) :`NewEnumerator2` (`self.Cave Light Spot`) :!type "LocalLightComponent Object Reference") _attenuationradius)
  (`LightComponent.SetLightColor` (select `/Game/Environment_BPs/Lights/Enum_Cave_Light_Types` _lighttype :`NewEnumerator0` (`self.Cave Light Point`) :`NewEnumerator2` (`self.Cave Light Spot`) :!type "LocalLightComponent Object Reference") _lightcolour true)
  (`LightComponent.SetUseTemperature` (select `/Game/Environment_BPs/Lights/Enum_Cave_Light_Types` _lighttype :`NewEnumerator0` (`self.Cave Light Point`) :`NewEnumerator2` (`self.Cave Light Spot`) :!type "LocalLightComponent Object Reference") _usetemperature)
  (`LightComponent.SetTemperature` (select `/Game/Environment_BPs/Lights/Enum_Cave_Light_Types` _lighttype :`NewEnumerator0` (`self.Cave Light Point`) :`NewEnumerator2` (`self.Cave Light Spot`) :!type "LocalLightComponent Object Reference") _temperature))

(event `/Game/Environment_BPs/Lights/BPI_Cave_Light.Start Chase Sequence`
  (bind _returnvalue (`KismetSystemLibrary.K2_SetTimerDelegate` (delegate `Chase Sequence Ticker`) (`self.Starting Chase Loop Time`) true))
  (set `self.Chase Sequence Timer` _returnvalue)
  (`/Game/Environment_BPs/Lights/BPI_Cave_Light.Deactivate Life Duration`))

(event `Chase Sequence Ticker`
  (bind _returnvalue (select `/Game/Environment_BPs/Lights/Enum_Cave_Light_Types` (`.LightType_18_0A74EB4641551F41F0FC41B50E7D4E5C` (break `/Game/Environment_BPs/Lights/Struct_Cave_Light_Info` (`self.Light Info`))) :`NewEnumerator0` (`self.Cave Light Point`) :`NewEnumerator2` (`self.Cave Light Spot`) :!type "LocalLightComponent Object Reference"))
  (bind _isa (`/Engine/EditorBlueprintResources/StandardMacros.FlipFlop`)
    (:`A`
      _)
    (:`B`
      _))
  (`LightComponent.SetIntensity` (select `/Game/Environment_BPs/Lights/Enum_Cave_Light_Types` (`.LightType_18_0A74EB4641551F41F0FC41B50E7D4E5C` (break `/Game/Environment_BPs/Lights/Struct_Cave_Light_Info` (`self.Light Info`))) :`NewEnumerator0` (`self.Cave Light Point`) :`NewEnumerator2` (`self.Cave Light Spot`) :!type "LightComponent Object Reference") (`KismetMathLibrary.SelectFloat` 999.0 0.0 _isa))
  (`LocalLightComponent.SetAttenuationRadius` _returnvalue 9999.0)
  (`LightComponent.SetLightColor` _returnvalue (`KismetMathLibrary.MakeColor` 1.0) true))

(event `/Game/Environment_BPs/Lights/BPI_Cave_Light.Update Chase Intensity`
  (params (`New Chase Intensity` :type "Float (double-precision)"))
  (set `self.Chase Intensity` `New Chase Intensity`)
  (bind _returnvalue (`KismetSystemLibrary.K2_SetTimerDelegate` (delegate `Chase Sequence Ticker`) (* (`self.Starting Chase Loop Time`) (`KismetMathLibrary.FClamp` (- 1.0 `New Chase Intensity`) 0.1)) true))
  (set `self.Chase Sequence Timer` _returnvalue)
  (`ActorComponent.SetActive` (select `/Game/Environment_BPs/Lights/Enum_Cave_Light_Types` (`.LightType_18_0A74EB4641551F41F0FC41B50E7D4E5C` (break `/Game/Environment_BPs/Lights/Struct_Cave_Light_Info` (`self.Light Info`))) :`NewEnumerator0` (`self.Cave Light Point`) :`NewEnumerator2` (`self.Cave Light Spot`) :!type "ActorComponent Object Reference") true false))

(event `/Game/Environment_BPs/Lights/BPI_Cave_Light.Stop Chase Sequence`
  (bind ((`LightType_18_0A74EB4641551F41F0FC41B50E7D4E5C` _lighttype) (`LightIntensity_9_ECD54D6042218D6F0D69FEAA9BDDBD7C` _lightintensity) (`LightColour_11_9853A6894656DE5AEAE7BC82B9CF57BF` _lightcolour)) (break `/Game/Environment_BPs/Lights/Struct_Cave_Light_Info` (`self.Light Info`)))
  (bind _returnvalue (select `/Game/Environment_BPs/Lights/Enum_Cave_Light_Types` _lighttype :`NewEnumerator0` (`self.Cave Light Point`) :`NewEnumerator2` (`self.Cave Light Spot`) :!type "LightComponent Object Reference"))
  (`KismetSystemLibrary.K2_ClearAndInvalidateTimerHandle` (`self.Chase Sequence Timer`))
  (`LightComponent.SetIntensity` _returnvalue (* _lightintensity (`self.Life Remaining %`)))
  (`LightComponent.SetLightColor` _returnvalue _lightcolour true))

(event `/Game/Environment_BPs/Lights/BPI_Cave_Light.Activate Life Duration`
  (bind ((`LightType_18_0A74EB4641551F41F0FC41B50E7D4E5C` _lighttype) (`LightIntensity_9_ECD54D6042218D6F0D69FEAA9BDDBD7C` _lightintensity)) (break `/Game/Environment_BPs/Lights/Struct_Cave_Light_Info` (`self.Light Info`)))
  (if (`self.Has Life Duration`)
    (`TimelineComponent.SetPlayRate` (`self.LifeDuration Timeline`) (/ 1.0 (`self.Life Duration`)))
    (bind (_direction _life_remaining__) (`Timeline|LifeDuration Timeline` :!via `PlayFromStart` :!label _label)
      (:`Update`
        (set `self.Life Remaining %` _life_remaining__)
        (`LightComponent.SetIntensity` (select `/Game/Environment_BPs/Lights/Enum_Cave_Light_Types` _lighttype :`NewEnumerator0` (`self.Cave Light Point`) :`NewEnumerator2` (`self.Cave Light Spot`) :!type "LightComponent Object Reference") (`KismetMathLibrary.Lerp` 0.0 _lightintensity _life_remaining__))))))

(event `/Game/Environment_BPs/Lights/BPI_Cave_Light.Deactivate Life Duration`
  (bind ((`LightType_18_0A74EB4641551F41F0FC41B50E7D4E5C` _lighttype) (`LightIntensity_9_ECD54D6042218D6F0D69FEAA9BDDBD7C` _lightintensity)) (break `/Game/Environment_BPs/Lights/Struct_Cave_Light_Info` (`self.Light Info`)))
  (`LightComponent.SetIntensity` (select `/Game/Environment_BPs/Lights/Enum_Cave_Light_Types` _lighttype :`NewEnumerator0` (`self.Cave Light Point`) :`NewEnumerator2` (`self.Cave Light Spot`) :!type "LightComponent Object Reference") _lightintensity)
  (goto _label :!via `Stop`))

(event `/Game/Environment_BPs/Lights/BPI_Cave_Light.Deactivate Light Flicker Tick`
  (`KismetSystemLibrary.K2_ClearAndInvalidateTimerHandle` (`self.Flicker Tick Timer`)))

(event `/Game/Environment_BPs/Lights/BPI_Cave_Light.Activate Light Flicker Tick`
  (params (`Max Duration` :type "Float (double-precision)"))
  (set `self.Flicker Duration` (`KismetMathLibrary.RandomFloatInRange` 0.1 `Max Duration`))
  (set `self.Flicker Start Time` (`KismetSystemLibrary.GetGameTimeInSeconds`))
  (bind _returnvalue (`KismetSystemLibrary.K2_SetTimerDelegate` (delegate `/Game/Environment_BPs/Lights/BPI_Cave_Light.Cave Light Flicker`) 0.01 true))
  (set `self.Flicker Tick Timer` _returnvalue))

(event `/Game/Environment_BPs/Lights/BPI_Cave_Light.Cave Light Flicker`
  (if (>= (`KismetSystemLibrary.GetGameTimeInSeconds`) (+ (`self.Flicker Start Time`) (`self.Flicker Duration`)))
    (`KismetSystemLibrary.K2_ClearAndInvalidateTimerHandle` (`self.Flicker Tick Timer`))
    (`LightComponent.SetIntensity` (select `/Game/Environment_BPs/Lights/Enum_Cave_Light_Types` (`.LightType_18_0A74EB4641551F41F0FC41B50E7D4E5C` (break `/Game/Environment_BPs/Lights/Struct_Cave_Light_Info` (`self.Light Info`))) :`NewEnumerator0` (`self.Cave Light Point`) :`NewEnumerator2` (`self.Cave Light Spot`) :!type "LightComponent Object Reference") (* (`.LightIntensity_9_ECD54D6042218D6F0D69FEAA9BDDBD7C` (break `/Game/Environment_BPs/Lights/Struct_Cave_Light_Info` (`self.Light Info`))) (`self.Life Remaining %`)))
    (`KismetSystemLibrary.Delay` 4.0)
    (`self.Activate Flicker Check`)
    (elif (`KismetMathLibrary.RandomBoolWithWeight` 0.75)
      (if (>= (- (`KismetSystemLibrary.GetGameTimeInSeconds`) (`self.Last Flicker Time`)) (`KismetMathLibrary.RandomFloatInRange` 1.0 2.0))
        (set `self.Last Flicker Time` (`KismetSystemLibrary.GetGameTimeInSeconds`))
        (`LightComponent.SetIntensity` (select `/Game/Environment_BPs/Lights/Enum_Cave_Light_Types` (`.LightType_18_0A74EB4641551F41F0FC41B50E7D4E5C` (break `/Game/Environment_BPs/Lights/Struct_Cave_Light_Info` (`self.Light Info`))) :`NewEnumerator0` (`self.Cave Light Point`) :`NewEnumerator2` (`self.Cave Light Spot`) :!type "LightComponent Object Reference") (* (* (`.LightIntensity_9_ECD54D6042218D6F0D69FEAA9BDDBD7C` (break `/Game/Environment_BPs/Lights/Struct_Cave_Light_Info` (`self.Light Info`))) (`self.Life Remaining %`)) 0.5)))
      (else
        (`LightComponent.SetIntensity` (select `/Game/Environment_BPs/Lights/Enum_Cave_Light_Types` (`.LightType_18_0A74EB4641551F41F0FC41B50E7D4E5C` (break `/Game/Environment_BPs/Lights/Struct_Cave_Light_Info` (`self.Light Info`))) :`NewEnumerator0` (`self.Cave Light Point`) :`NewEnumerator2` (`self.Cave Light Spot`) :!type "LightComponent Object Reference") (* (`.LightIntensity_9_ECD54D6042218D6F0D69FEAA9BDDBD7C` (break `/Game/Environment_BPs/Lights/Struct_Cave_Light_Info` (`self.Light Info`))) (`self.Life Remaining %`)))))))

(event `self.ReceiveBeginPlay`
  (`self.Activate Flicker Check`))

(event `/Game/Environment_BPs/Lights/BPI_Cave_Light.Activate Flicker Check`
  (if (`.Organic?_20_2A75652140992C838A3095B935751F8D` (break `/Game/Environment_BPs/Lights/Struct_Cave_Light_Info` (`self.Light Info`)))
    (bind _returnvalue (`KismetSystemLibrary.K2_SetTimerDelegate` (delegate `Flicker Check Tick`) 0.05 true))
    (set `self.Flicker Check Timer` _returnvalue)))

(event `Flicker Check Tick`
  (if (`KismetMathLibrary.RandomBoolWithWeight` 0.05)
    (if (>= (- (`KismetSystemLibrary.GetGameTimeInSeconds`) (`self.Last Flicker Check Success`)) 3.0)
      (set `self.Last Flicker Check Success` (`KismetSystemLibrary.GetGameTimeInSeconds`))
      (`self.Activate Light Flicker Tick` (`KismetMathLibrary.RandomFloatInRange` 3.0 6.0))
      (`self.Deactivate Flicker Check`))))

(event `/Game/Environment_BPs/Lights/BPI_Cave_Light.Deactivate Flicker Check`
  (`KismetSystemLibrary.K2_ClearAndInvalidateTimerHandle` (`self.Flicker Check Timer`)))

(fn `UserConstructionScript`
  (bind (_lighttype _lightintensity _attenuationradius _lightcolour _usetemperature _temperature _organic_ _lightmesh) (break `/Game/Environment_BPs/Lights/Struct_Cave_Light_Info` (`self.Light Info`)))
  (`StaticMeshComponent.SetStaticMesh` (`self.Light Mesh`) _lightmesh)
  (switch `/Game/Environment_BPs/Lights/Enum_Cave_Light_Types` _lighttype
    (:`NewEnumerator0`
      (`LightComponent.SetIntensity` (`self.Cave Light Spot`) 0.0)
      (`LightComponent.SetIntensity` (`self.Cave Light Point`) _lightintensity)
      (`LocalLightComponent.SetAttenuationRadius` (`self.Cave Light Point`) _attenuationradius)
      (`LightComponent.SetLightColor` (`self.Cave Light Point`) _lightcolour true)
      (`LightComponent.SetUseTemperature` (`self.Cave Light Point`) _usetemperature)
      (`LightComponent.SetTemperature` (`self.Cave Light Point`) _temperature))
    (:`NewEnumerator2`
      (`LightComponent.SetIntensity` (`self.Cave Light Point`) 0.0)
      (`LightComponent.SetIntensity` (`self.Cave Light Spot`) _lightintensity)
      (`LocalLightComponent.SetAttenuationRadius` (`self.Cave Light Spot`) _attenuationradius)
      (`LightComponent.SetLightColor` (`self.Cave Light Spot`) _lightcolour true)
      (`LightComponent.SetUseTemperature` (`self.Cave Light Spot`) _usetemperature)
      (`LightComponent.SetTemperature` (`self.Cave Light Spot`) _temperature))))