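; BP_Insane_Writing is an environment actor showing scrambled writing on a widget, which decrypts once the game mode's loop count reaches a required value.
; Decrypt and encrypt events drive the widget, falling back to shaking characters when the loop is too early; decrypting also activates a linked journal addition.
; A reversible timeline fades widget opacity for highlight and dim.
; Collision overlaps only track decryption proximity; their calls to these events are disconnected.
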(event `self.ReceiveBeginPlay`
  (bind _aswbp_insane_writing (cast `/Game/Environment_BPs/Writing/WBP_Insane_Writing` (`WidgetComponent.GetWidget` (`self.Insane Writing`))))
  (bind _output_get (set `self.As WBP Insane Writing` _aswbp_insane_writing))
  (set `/Game/Environment_BPs/Writing/WBP_Insane_Writing.Intended Decryption Text` (`self.Decrypted Text`) _output_get)
  (set `/Game/Environment_BPs/Writing/WBP_Insane_Writing.Wrap Size` (`self.Wrap Sizing`) _output_get))

(event `Highlight Writing`
  (`TimelineComponent.SetPlayRate` (`self.Highlight Writing Timeline`) (/ 1.0 (`self.Highlight / Dim Writing Time`)))
  (bind (_direction _alpha) (`Timeline|Highlight Writing Timeline` :!label _label)
    (:`Update`
      (`WidgetComponent.SetTintColorAndOpacity` (`self.Insane Writing`) (`KismetMathLibrary.MakeColor` 1.0 1.0 1.0 (`KismetMathLibrary.Lerp` 0.01 1.0 _alpha))))))

(event `Decrypt Writing`
  (bind _as_wbp_insane_writing (`self.As WBP Insane Writing`))
  (bind _loop_count (message `/Game/Core/Modes/BPI_Gamemode.Get Loop Count` (`GameplayStatics.GetGameMode`)))
  (if (>= _loop_count (`self.Required loop for Decryption`))
    (`/Game/Environment_BPs/Writing/WBP_Insane_Writing.Decrypt Writing` _as_wbp_insane_writing (`self.Time for Decryption`))
    (`/Game/Player/Journal/BP_Journal_Addition_Collision.Activate Journal Addition` (`self.Associated Journal Addition`))
    (else
      (`/Game/Environment_BPs/Writing/WBP_Insane_Writing.Shake Characters Without Decrypting` _as_wbp_insane_writing))))

(event `Dim Writing`
  (goto _label :!via `Reverse`))

(event `Encrypt Writing`
  (bind _as_wbp_insane_writing (`self.As WBP Insane Writing`))
  (bind _loop_count (message `/Game/Core/Modes/BPI_Gamemode.Get Loop Count` (`GameplayStatics.GetGameMode`)))
  (if (>= _loop_count (`self.Required loop for Decryption`))
    (`/Game/Environment_BPs/Writing/WBP_Insane_Writing.Encrypt Writing` _as_wbp_insane_writing (`self.Time for Encryption`))
    (else
      (`/Game/Environment_BPs/Writing/WBP_Insane_Writing.Stop Shaking Characters Without Decrypting` _as_wbp_insane_writing))))

(event `self.Decrypt Attempt Collision.OnComponentBeginOverlap`
  (params (OverlappedComponent :type "PrimitiveComponent Object Reference") (OtherActor :type "Actor Object Reference") (OtherComp :type "PrimitiveComponent Object Reference") (OtherBodyIndex :type Integer) (bFromSweep :type Boolean) (SweepResult :type "HitResult Structure (by ref)"))
  (set `self.Player Close Enough for Decryption` true))

(event `self.Decrypt Attempt Collision.OnComponentEndOverlap`
  (params (OverlappedComponent :type "PrimitiveComponent Object Reference") (OtherActor :type "Actor Object Reference") (OtherComp :type "PrimitiveComponent Object Reference") (OtherBodyIndex :type Integer))
  (set `self.Player Close Enough for Decryption` false))

(event `self.Opacity Change Collision.OnComponentBeginOverlap`
  (params (OverlappedComponent :type "PrimitiveComponent Object Reference") (OtherActor :type "Actor Object Reference") (OtherComp :type "PrimitiveComponent Object Reference") (OtherBodyIndex :type Integer) (bFromSweep :type Boolean) (SweepResult :type "HitResult Structure (by ref)")))

(event `self.Opacity Change Collision.OnComponentEndOverlap`
  (params (OverlappedComponent :type "PrimitiveComponent Object Reference") (OtherActor :type "Actor Object Reference") (OtherComp :type "PrimitiveComponent Object Reference") (OtherBodyIndex :type Integer)))

(fn `UserConstructionScript`
  (bind _aswbp_insane_writing (cast `/Game/Environment_BPs/Writing/WBP_Insane_Writing` (`WidgetComponent.GetWidget` (`self.Insane Writing`))))
  (set `/Game/Environment_BPs/Writing/WBP_Insane_Writing.Intended Decryption Text` (`self.Decrypted Text`) _aswbp_insane_writing))