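; Trigger volume that lets the player highlight and decrypt BP_Insane_Writing actors by looking at them.
; Overlapping its collision, or already standing inside at BeginPlay, starts a looping timer that box-traces forward from the camera.
; Hit writings highlight and, via paired DoOnce gates, decrypt or encrypt depending on player proximity.
; Writings leaving view, or all tracked ones when overlap ends, dim and re-encrypt.
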(event `Reset Decryption Look At Do Once`
  (goto _label :!via `Reset`))

(event `Player Look Writing Check`
  (bind _returnvalue (`GameplayStatics.GetPlayerCameraManager` 0))
  (bind _returnvalue_2 (`PlayerCameraManager.GetCameraLocation` _returnvalue))
  (bind _returnvalue_3 (`PlayerCameraManager.GetCameraRotation` _returnvalue))
  (`KismetArrayLibrary.Array_Clear` (`self.Hit Insane Writings`))
  (bind (_outhits _returnvalue_4) (`KismetSystemLibrary.BoxTraceMultiForObjects` _returnvalue_2 (+ _returnvalue_2 (* (`KismetMathLibrary.GetForwardVector` _returnvalue_3) 999.0)) (32.0 32.0 32.0) _returnvalue_3 (`|MakeArray` "ObjectTypeQuery9" :!type "EObjectTypeQuery Enum")))
  (if _returnvalue_4
    (for _array_element _outhits
      (bind _asbp_insane_writing (cast `/Game/Environment_BPs/Writing/BP_Insane_Writing` (`.HitActor` (`GameplayStatics.BreakHitResult` _array_element))))
      (if (not (`KismetArrayLibrary.Array_Contains` (`self.Hit Insane Writings`) _asbp_insane_writing))
        (`KismetArrayLibrary.Array_Add` (`self.Hit Insane Writings`) _asbp_insane_writing))
      (if (not (`KismetArrayLibrary.Array_Contains` (`self.Writing Being Looked At`) _asbp_insane_writing))
        (`/Game/Environment_BPs/Writing/BP_Insane_Writing.Highlight Writing` _asbp_insane_writing)
        (`KismetArrayLibrary.Array_Add` (`self.Writing Being Looked At`) _asbp_insane_writing))
      (if (`/Game/Environment_BPs/Writing/BP_Insane_Writing.Player Close Enough for Decryption` _asbp_insane_writing)
        (`|ExecutionSequence`
          (:`then_0`
            (goto _label_2 :!via `Reset`))
          (:`then_1`
            (`/Engine/EditorBlueprintResources/StandardMacros.DoOnce` false :!label _label
              (:`Completed`
                (`/Game/Environment_BPs/Writing/BP_Insane_Writing.Decrypt Writing` _asbp_insane_writing)))))
        (else
          (`|ExecutionSequence`
            (:`then_0`
              (goto _label :!via `Reset`))
            (:`then_1`
              (`/Engine/EditorBlueprintResources/StandardMacros.DoOnce` false :!label _label_2
                (:`Completed`
                  (`/Game/Environment_BPs/Writing/BP_Insane_Writing.Encrypt Writing` _asbp_insane_writing))))))))
    (bind _output_get (set `self.Temp Writings Being Looked At` (`self.Writing Being Looked At`)))
    (for _array_element_2 _output_get
      (if (not (`KismetArrayLibrary.Array_Contains` (`self.Hit Insane Writings`) _array_element_2))
        (`/Game/Environment_BPs/Writing/BP_Insane_Writing.Dim Writing` _array_element_2)
        (`/Game/Environment_BPs/Writing/BP_Insane_Writing.Encrypt Writing` _array_element_2)
        (`KismetArrayLibrary.Array_RemoveItem` (`self.Writing Being Looked At`) _array_element_2)))
    (else
      (for _array_element_3 (`self.Writing Being Looked At`)
        (`/Game/Environment_BPs/Writing/BP_Insane_Writing.Dim Writing` _array_element_3)
        (`/Game/Environment_BPs/Writing/BP_Insane_Writing.Encrypt Writing` _array_element_3))
      (`KismetArrayLibrary.Array_Clear` (`self.Writing Being Looked At`))
      (`self.Reset Decryption Look At Do Once`))))

(event `self.Player Look Collision.OnComponentEndOverlap`
  (params (OverlappedComponent :type "PrimitiveComponent Object Reference") (OtherActor :type "Actor Object Reference") (OtherComp :type "PrimitiveComponent Object Reference") (OtherBodyIndex :type Integer))
  (`KismetSystemLibrary.K2_ClearAndInvalidateTimerHandle` (`self.Player Look Timer`))
  (for _array_element (`self.Writing Being Looked At`)
    (`/Game/Environment_BPs/Writing/BP_Insane_Writing.Dim Writing` _array_element)
    (`/Game/Environment_BPs/Writing/BP_Insane_Writing.Encrypt Writing` _array_element))
  (`KismetArrayLibrary.Array_Clear` (`self.Writing Being Looked At`)))

(event `self.Player Look Collision.OnComponentBeginOverlap`
  (params (OverlappedComponent :type "PrimitiveComponent Object Reference") (OtherActor :type "Actor Object Reference") (OtherComp :type "PrimitiveComponent Object Reference") (OtherBodyIndex :type Integer) (bFromSweep :type Boolean) (SweepResult :type "HitResult Structure (by ref)"))
  (bind _returnvalue (`KismetSystemLibrary.K2_SetTimerDelegate` (delegate `Player Look Writing Check`) 0.25 true :!label _label_3))
  (set `self.Player Look Timer` _returnvalue))

(event `self.ReceiveBeginPlay`
  (`KismetSystemLibrary.Delay` 1.0)
  (if (not (`KismetArrayLibrary.Array_IsEmpty` (`self.GetOverlappingActors` "/Game/Player/BP_Player.BP_Player_C")))
    (goto _label_3)))

(fn `UserConstructionScript`)