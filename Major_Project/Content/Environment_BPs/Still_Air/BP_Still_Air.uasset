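; BP_Still_Air is an environmental hazard volume of stale air that damages the player over time.
; Overlapping the collision box starts a delay timer, which then launches a looping one-second timer applying DamagePerSecond through player 0's health component.
; Ending the overlap or the player's health reaching zero clears the timers.
; The construction script and BeginPlay both scale the VFX from the box extent.
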(event `self.ReceiveBeginPlay`
  (bind (_returnvalue_x _returnvalue_y _returnvalue_z) (`KismetMathLibrary.BreakVector` (`BoxComponent.GetScaledBoxExtent` (`self.Stale Air Collision`))))
  (`SceneComponent.SetWorldScale3D` (`self.Stale Air VFX`) (`KismetMathLibrary.MakeVector` (* (/ _returnvalue_x 350.0) 0.5) (* (/ _returnvalue_y 350.0) 0.5) (/ _returnvalue_z 350.0))))

(event `Stale Air Damage Loop`
  (bind _returnvalue (`GameplayStatics.GetPlayerCharacter` 0))
  (bind _returnvalue_2 (`self.GetComponentByClass` _returnvalue "/Game/Player/BPC_Player_Health.BPC_Player_Health_C"))
  (`/Game/Player/BPC_Player_Health.Player Take Damage` _returnvalue_2 (`self.Damage Per Second`) (`self.K2_GetActorLocation` _returnvalue) (`KismetMathLibrary.RandomUnitVector`))
  (if (<= (`/Game/Player/BPC_Player_Health.Health` _returnvalue_2) 0.0)
    (`self.Stop Stale Air Damage`)))

(event `Start Stale Air Damage`
  (bind _returnvalue (`KismetSystemLibrary.K2_SetTimerDelegate` (delegate `Stale Air Damage Loop`) 1.0 true))
  (set `self.Damage Loop` _returnvalue))

(event `Stop Stale Air Damage`
  (`KismetSystemLibrary.K2_ClearAndInvalidateTimerHandle` (`self.Start Damage Timer`))
  (`KismetSystemLibrary.K2_ClearAndInvalidateTimerHandle` (`self.Damage Loop`)))

(event `self.Stale Air Collision.OnComponentBeginOverlap`
  (params (OverlappedComponent :type "PrimitiveComponent Object Reference") (OtherActor :type "Actor Object Reference") (OtherComp :type "PrimitiveComponent Object Reference") (OtherBodyIndex :type Integer) (bFromSweep :type Boolean) (SweepResult :type "HitResult Structure (by ref)"))
  (bind _returnvalue (`KismetSystemLibrary.K2_SetTimerDelegate` (delegate `Start Stale Air Damage`) (`self.Delay For Entering`)))
  (set `self.Start Damage Timer` _returnvalue))

(event `self.Stale Air Collision.OnComponentEndOverlap`
  (params (OverlappedComponent :type "PrimitiveComponent Object Reference") (OtherActor :type "Actor Object Reference") (OtherComp :type "PrimitiveComponent Object Reference") (OtherBodyIndex :type Integer))
  (`self.Stop Stale Air Damage`))

(fn `UserConstructionScript`
  (bind (_returnvalue_x _returnvalue_y _returnvalue_z) (`KismetMathLibrary.BreakVector` (`BoxComponent.GetScaledBoxExtent` (`self.Stale Air Collision`))))
  (`SceneComponent.SetWorldScale3D` (`self.Stale Air VFX`) (`KismetMathLibrary.MakeVector` (* (/ _returnvalue_x 350.0) 0.5) (* (/ _returnvalue_y 350.0) 0.5) (/ _returnvalue_z 350.0))))