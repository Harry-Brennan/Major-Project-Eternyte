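; Player inventory component that lays acquired items out on a canvas actor in the world and manages the left-hand item.
; BeginPlay spawns socket-attached held items, which are shown or hidden as the left-hand item changes.
; Opening box-traces for clear ground, swaps input mapping contexts and runs a timed camera trace to hover items for equipping.
; The use action prioritises minecarts and lock parts over the held item.
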(event `self.ReceiveBeginPlay`
  (bind _returnvalue (`|SpawnActorFromClass` "/Game/Items/BP_Inventory_Canvas.BP_Inventory_Canvas_C" (`KismetMathLibrary.MakeTransform` (0.0 0.0 0.0)) "Undefined" "MultiplyWithRoot" null null))
  (bind _output_get (set `self.Inventory Canvas` _returnvalue))
  (`Actor.SetActorHiddenInGame` _output_get true)
  (bind _asbp_player (cast `/Game/Player/BP_Player` (`self.GetOwner`)))
  (set `self.As BP Player` _asbp_player)
  (bind _returnvalue_2 (`|SpawnActorFromClass` "/Game/Items/Flashlight/BP_Flashlight.BP_Flashlight_C" (`KismetMathLibrary.MakeTransform` (0.0 0.0 0.0)) "Undefined" "MultiplyWithRoot" (`self.GetOwner`) null))
  (bind _output_get_2 (set `self.Player's FlashLight` _returnvalue_2))
  (`Actor.K2_AttachToComponent` _output_get_2 (`Actor.GetComponentByClass` (`self.GetOwner`) "/Script/Engine.SkeletalMeshComponent") "Flashlight Socket" "SnapToTarget" "SnapToTarget" "KeepWorld" true)
  (bind _returnvalue_3 (`|SpawnActorFromClass` "/Game/Items/Left_Hand_Items/Phone/BP_Phone_Held.BP_Phone_Held_C" (`KismetMathLibrary.MakeTransform` (0.0 0.0 0.0)) "Undefined" "MultiplyWithRoot" (`self.GetOwner`) "NewEnumerator1" null))
  (bind _output_get_3 (set `self.Player's Phone` _returnvalue_3))
  (`Actor.K2_AttachToComponent` _output_get_3 (`Actor.GetComponentByClass` (`self.GetOwner`) "/Script/Engine.SkeletalMeshComponent") "Phone_Socket" "SnapToTarget" "SnapToTarget" "KeepWorld" true)
  (`Actor.SetActorHiddenInGame` _output_get_3 true)
  (bind _returnvalue_4 (`|SpawnActorFromClass` "/Game/Items/Left_Hand_Items/Rope/BP_Rope_Held.BP_Rope_Held_C" (`KismetMathLibrary.MakeTransform` (0.0 0.0 0.0)) "Undefined" "MultiplyWithRoot" (`self.GetOwner`) "NewEnumerator2" null))
  (bind _output_get_4 (set `self.Player's Rope` _returnvalue_4))
  (`Actor.K2_AttachToComponent` _output_get_4 (`Actor.GetComponentByClass` (`self.GetOwner`) "/Script/Engine.SkeletalMeshComponent") "Rope_Socket" "SnapToTarget" "SnapToTarget" "KeepWorld" true)
  (`Actor.SetActorHiddenInGame` _output_get_4 true)
  (bind _returnvalue_5 (`|SpawnActorFromClass` "/Game/Items/Left_Hand_Items/Dynamite/BP_Dynamite_Held.BP_Dynamite_Held_C" (`KismetMathLibrary.MakeTransform` (0.0 0.0 0.0)) "Undefined" "MultiplyWithRoot" (`self.GetOwner`) "NewEnumerator3" null))
  (bind _output_get_5 (set `self.Player's Dynamite` _returnvalue_5))
  (`Actor.K2_AttachToComponent` _output_get_5 (`Actor.GetComponentByClass` (`self.GetOwner`) "/Script/Engine.SkeletalMeshComponent") "Dynamite_Socket" "SnapToTarget" "SnapToTarget" "KeepWorld" true)
  (`Actor.SetActorHiddenInGame` _output_get_5 true)
  (bind _returnvalue_6 (`|SpawnActorFromClass` "/Game/Items/Left_Hand_Items/EMF/BP_EMF_Reader_Held.BP_EMF_Reader_Held_C" (`KismetMathLibrary.MakeTransform` (0.0 0.0 0.0)) "Undefined" "MultiplyWithRoot" null "NewEnumerator4" null))
  (bind _output_get_6 (set `self.Player's EMF` _returnvalue_6))
  (`Actor.K2_AttachToComponent` _output_get_6 (`Actor.GetComponentByClass` (`self.GetOwner`) "/Script/Engine.SkeletalMeshComponent") "EMF_Socket" "SnapToTarget" "SnapToTarget" "KeepWorld" true)
  (`Actor.SetActorHiddenInGame` _output_get_6 true)
  (`self.Add Item to Left Hand` (`self.Left Hand Item`)))

(event `Reset Inventory`
  (bind _returnvalue (pcsubsystem `EnhancedInputLocalPlayerSubsystem` (`GameplayStatics.GetPlayerController` 0)))
  (`KismetArrayLibrary.Array_Clear` (`self.Items Acquired`))
  (`KismetSystemLibrary.K2_ClearAndInvalidateTimerHandle` (`self.Item Selection Trace Timer`))
  (set `self.Hovered Item` null)
  (set `self.Inventory Opening / Closing` true :!label _label)
  (`KismetSystemLibrary.K2_ClearAndInvalidateTimerHandle` (`self.Item Selection Trace Timer`))
  (`/Game/Items/BP_Inventory_Canvas.Hide All Items` (`self.Inventory Canvas`))
  (`KismetSystemLibrary.Delay` 1.0)
  (set `self.Inventory Open` false)
  (set `self.Inventory Opening / Closing` false)
  (`LegacyCameraShake.StartLegacyCameraShake` (`GameplayStatics.GetPlayerCameraManager` 0) "/Game/Items/BP_Inventory_Camera_Shake.BP_Inventory_Camera_Shake_C")
  (`Actor.K2_SetActorLocationAndRotation` :`self` (`self.Inventory Canvas`))
  (`Actor.SetActorHiddenInGame` (`self.Inventory Canvas`) true)
  (`/Engine/EditorBlueprintResources/StandardMacros.IsValid` _returnvalue
    (:`Is Valid`
      (`EnhancedInputSubsystemInterface.RemoveMappingContext` _returnvalue "/Game/Player/Input/IMC_Inventory_Open.IMC_Inventory_Open" (struct))
      (`EnhancedInputSubsystemInterface.AddMappingContext` _returnvalue "/Game/Player/Input/IMC_Default.IMC_Default" 0 (struct))
      (set `self.Inventory Close Cooldown` true)
      (`KismetSystemLibrary.Delay` 0.25)
      (set `self.Inventory Close Cooldown` false))))

(event `Force Close Inventory`
  (`FMODBlueprintStatics.PlayEventAtLocation` "/Game/FMOD/Events/Inventory/Close_Inventory.Close_Inventory" (`KismetMathLibrary.MakeTransform` (`Actor.K2_GetActorLocation` (`self.Inventory Canvas`))) :!label _label_2)
  (goto _label))

(event `EnhancedInput|/Game/Player/Input/Actions/Menus/IA_Inventory_Toggle`
  (params (ActionValue :type Boolean) (ElapsedSeconds :type "Float (double-precision)") (TriggeredSeconds :type "Float (double-precision)") (InputAction :type "InputAction Object Reference" :default "/Game/Player/Input/Actions/Menus/IA_Inventory_Toggle.IA_Inventory_Toggle"))
  (bind _returnvalue (`self.GetOwner`))
  (bind _returnvalue_2 (pcsubsystem `EnhancedInputLocalPlayerSubsystem` (`GameplayStatics.GetPlayerController` 0)))
  (:`Triggered`
    (if (`NavMovementComponent.IsFalling` (`Actor.GetComponentByClass` (`self.GetOwner`) "/Script/Engine.CharacterMovementComponent"))
      _
      (elif (`self.Inventory Opening / Closing`)
        _
        (elif (not (`self.Inventory Close Cooldown`))
          (`LegacyCameraShake.StartLegacyCameraShake` (`GameplayStatics.GetPlayerCameraManager` 0) "/Game/Items/BP_Inventory_Camera_Shake.BP_Inventory_Camera_Shake_C")
          (if (`self.Inventory Open`)
            (goto _label_2)
            (else
              (bind (_can_place_inventory_here_ _loc _rot) (`self.Inventory Place Line Trace`))
              (if _can_place_inventory_here_
                (set `self.Inventory Opening / Closing` true)
                (`FMODBlueprintStatics.PlayEventAtLocation` "/Game/FMOD/Events/Inventory/Open_Inventory.Open_Inventory" (`KismetMathLibrary.MakeTransform` (+ (`Actor.K2_GetActorLocation` _returnvalue) (* (`Actor.GetActorForwardVector` _returnvalue) -25.0)) (`KismetMathLibrary.MakeRotator` 0.0)))
                (set `self.Hovered Item` null)
                (set `self.Inventory Open` true)
                (`Actor.K2_SetActorLocationAndRotation` (`self.Inventory Canvas`) _loc _rot false false)
                (`/Game/Items/BP_Inventory_Canvas.Show Acquired Items` (`self.Inventory Canvas`) (`self.Items Acquired`))
                (`Actor.SetActorHiddenInGame` (`self.Inventory Canvas`) false)
                (`/Engine/EditorBlueprintResources/StandardMacros.IsValid` _returnvalue_2
                  (:`Is Valid`
                    (`EnhancedInputSubsystemInterface.RemoveMappingContext` _returnvalue_2 "/Game/Player/Input/IMC_Default.IMC_Default" (struct))
                    (`EnhancedInputSubsystemInterface.AddMappingContext` _returnvalue_2 "/Game/Player/Input/IMC_Inventory_Open.IMC_Inventory_Open" 0 (struct))
                    (bind _returnvalue_3 (`KismetSystemLibrary.K2_SetTimer` null "Inventory Item Selection Trace" 0.01 true))
                    (set `self.Item Selection Trace Timer` _returnvalue_3)
                    (`KismetSystemLibrary.Delay` 0.3)
                    (set `self.Inventory Opening / Closing` false)))
                (else
                  (`FMODBlueprintStatics.PlayEventAtLocation` "/Game/FMOD/Events/Inventory/Inventory_Unable_To_Open.Inventory_Unable_To_Open" (`KismetMathLibrary.MakeTransform` (`Actor.K2_GetActorLocation` (`self.GetOwner`)))))))))))))

(event `EnhancedInput|/Game/Player/Input/Actions/Items/IA_Pickup_Equip_Item`
  (params (ActionValue :type Boolean) (ElapsedSeconds :type "Float (double-precision)") (TriggeredSeconds :type "Float (double-precision)") (InputAction :type "InputAction Object Reference" :default "/Game/Player/Input/Actions/Items/IA_Pickup_Equip_Item.IA_Pickup_Equip_Item"))
  (bind _overlapping_item_to_pickup (`self.Overlapping Item to Pickup`))
  (:`Triggered`
    (if (`self.Inventory Open`)
      (`/Engine/EditorBlueprintResources/StandardMacros.IsValid` (`self.Hovered Item`)
        (:`Is Valid`
          (if (not (`/Game/Items/BP_Item_Within_Inventory.Equipping Item` (`self.Hovered Item`)))
            (`/Game/Items/BP_Item_Within_Inventory.Equip Item` (`self.Hovered Item`) 0.25)
            (set `self.Hovered Item` null)
            (`LegacyCameraShake.StartLegacyCameraShake` (`GameplayStatics.GetPlayerCameraManager` 0) "/Game/Items/BP_Inventory_Camera_Shake.BP_Inventory_Camera_Shake_C"))))
      (else
        (`/Engine/EditorBlueprintResources/StandardMacros.IsValid` _overlapping_item_to_pickup
          (:`Is Valid`
            (`/Game/Items/BP_Item_Pickup.Attempt Pickup` _overlapping_item_to_pickup)))))))

(event `Add Item to Left Hand`
  (params (Item :type "/Game/Items/Enum_Left_Hand_Items Enum" :default "NewEnumerator0"))
  (`FMODBlueprintStatics.PlayEventAtLocation` "/Game/FMOD/Events/Inventory/Inventory_Rummage.Inventory_Rummage" (`KismetMathLibrary.MakeTransform` (`Actor.K2_GetActorLocation` (`self.GetOwner`))))
  (bind _output_get (set `self.Left Hand Item` Item))
  (switch `/Game/Items/Enum_Left_Hand_Items` _output_get
    (:`NewEnumerator1`
      (`Actor.SetActorHiddenInGame` (`self.Player's Phone`) false))
    (:`NewEnumerator2`
      (`Actor.SetActorHiddenInGame` (`self.Player's Rope`) false))
    (:`NewEnumerator3`
      (`Actor.SetActorHiddenInGame` (`self.Player's Dynamite`) false))
    (:`NewEnumerator4`
      (`Actor.SetActorHiddenInGame` (`self.Player's EMF`) false))))

(event `Add Item to Inventory`
  (params (`Item Name` :type "/Game/Items/Enum_Left_Hand_Items Enum" :default "NewEnumerator0"))
  (if (not (`KismetArrayLibrary.Array_Contains` (`self.Items Acquired`) `Item Name`))
    (`KismetArrayLibrary.Array_Add` (`self.Items Acquired`) `Item Name`)
    (`FMODBlueprintStatics.PlayEventAtLocation` "/Game/FMOD/Events/Inventory/Inventory_Rummage.Inventory_Rummage" (`KismetMathLibrary.MakeTransform` (`Actor.K2_GetActorLocation` (`self.GetOwner`))))
    (`LegacyCameraShake.StartLegacyCameraShake` (`GameplayStatics.GetPlayerCameraManager` 0) "/Game/Items/BP_Inventory_Camera_Shake.BP_Inventory_Camera_Shake_C")))

(event `Remove Item from Left Hand`
  (bind _inventory_canvas (`self.Inventory Canvas`))
  (switch `/Game/Items/Enum_Left_Hand_Items` (`self.Left Hand Item`)
    (:`NewEnumerator1`
      (`Actor.SetActorHiddenInGame` (`self.Player's Phone`) true)
      (if (`/Game/Items/Left_Hand_Items/Phone/BP_Phone_Held.Phone Active` (`self.Player's Phone`))
        (`/Game/Items/Left_Hand_Items/Phone/BP_Phone_Held.Force Deactivate Phone` (`self.Player's Phone`))))
    (:`NewEnumerator2`
      (`Actor.SetActorHiddenInGame` (`self.Player's Rope`) true))
    (:`NewEnumerator3`
      (`Actor.SetActorHiddenInGame` (`self.Player's Dynamite`) true))
    (:`NewEnumerator4`
      (`Actor.SetActorHiddenInGame` (`self.Player's EMF`) true)))
  (`/Game/Items/BP_Inventory_Canvas.Add Item to Canvas` _inventory_canvas (`self.Left Hand Item`))
  (`FMODBlueprintStatics.PlayEventAtLocation` "/Game/FMOD/Events/Inventory/Inventory_Rummage.Inventory_Rummage" (`KismetMathLibrary.MakeTransform` (`Actor.K2_GetActorLocation` _inventory_canvas)))
  (set `self.Left Hand Item` "NewEnumerator0"))

(event `Force Use Phone`
  (`/Game/Items/Left_Hand_Items/BP_Left_Hand_Item.Use Item` (`self.Player's Phone`) :!label _label_3))

(event `EnhancedInput|/Game/Player/Input/Actions/Items/IA_Use_Left_Item`
  (params (ActionValue :type Boolean) (ElapsedSeconds :type "Float (double-precision)") (TriggeredSeconds :type "Float (double-precision)") (InputAction :type "InputAction Object Reference" :default "/Game/Player/Input/Actions/Items/IA_Use_Left_Item.IA_Use_Left_Item"))
  (bind _returnvalue (`GameplayStatics.GetPlayerCameraManager` 0))
  (bind _returnvalue_2 (`PlayerCameraManager.GetCameraLocation` _returnvalue))
  (bind _overlappingactors (`Actor.GetOverlappingActors` (`self.GetOwner`) "/Game/Environment_BPs/Lock/BP_Full_Lock.BP_Full_Lock_C"))
  (:`Triggered`
    (if (`KismetArrayLibrary.Array_IsEmpty` (`Actor.GetOverlappingActors` (`self.GetOwner`) "/Game/Environment_BPs/Minecart/BP_Minecart.BP_Minecart_C"))
      (if (`KismetArrayLibrary.Array_IsEmpty` _overlappingactors)
        (switch `/Game/Items/Enum_Left_Hand_Items` (`self.Left Hand Item`) :!label _label_4
          (:`NewEnumerator0`
            (`KismetSystemLibrary.PrintString` "NO LEFT HAND ITEM"))
          (:`NewEnumerator1`
            (`KismetSystemLibrary.PrintString` "PHONE")
            (goto _label_3))
          (:`NewEnumerator2`
            (`KismetSystemLibrary.PrintString` "ROPE")
            (`/Game/Items/Left_Hand_Items/BP_Left_Hand_Item.Use Item` (`self.Player's Rope`)))
          (:`NewEnumerator3`
            (`KismetSystemLibrary.PrintString` "DYNAMITE")
            (`/Game/Items/Left_Hand_Items/BP_Left_Hand_Item.Use Item` (`self.Player's Dynamite`)))
          (:`NewEnumerator4`
            (`KismetSystemLibrary.PrintString` "EMF")
            (`/Game/Items/Left_Hand_Items/BP_Left_Hand_Item.Use Item` (`self.Player's EMF`))))
        (else
          (bind _asbp_full_lock (cast `/Game/Environment_BPs/Lock/BP_Full_Lock` (`|GetArrayItem` _overlappingactors)))
          (bind _lock_part_being_looked_at (`/Game/Environment_BPs/Lock/BP_Full_Lock.Lock Part Being Looked At` _asbp_full_lock))
          (`/Engine/EditorBlueprintResources/StandardMacros.IsValid` _lock_part_being_looked_at
            (:`Is Valid`
              (`/Game/Environment_BPs/Lock/BP_Lock_Part.Turn Lock Part` _lock_part_being_looked_at))
            (:`Is Not Valid`
              (goto _label_4)))))
      (else
        (bind (_outhit _returnvalue_3) (`KismetSystemLibrary.BoxTraceSingleForObjects` :`Start` _returnvalue_2 :`End` (+ _returnvalue_2 (* (`KismetMathLibrary.GetForwardVector` (`PlayerCameraManager.GetCameraRotation` _returnvalue)) 250.0)) :`HalfSize` (8.0 8.0 8.0) :`ObjectTypes` (`|MakeArray` "ObjectTypeQuery14" :!type "EObjectTypeQuery Enum") :`bTraceComplex` true :`DrawDebugType` "ForDuration"))
        (if _returnvalue_3
          (bind _asbp_minecart (cast `/Game/Environment_BPs/Minecart/BP_Minecart` (`.HitActor` (`GameplayStatics.BreakHitResult` _outhit))))
          (`/Game/Environment_BPs/Minecart/BP_Minecart.Start Minecart` _asbp_minecart)
          (else
            (goto _label_4)))))))

(fn `Inventory Item Selection Trace`
  (bind _returnvalue (`GameplayStatics.GetPlayerCameraManager` 0))
  (bind _hovered_item (`self.Hovered Item`))
  (bind _returnvalue_2 (`PlayerCameraManager.GetCameraLocation` _returnvalue))
  (bind _returnvalue_3 (`PlayerCameraManager.GetCameraRotation` _returnvalue))
  (bind (_outhit _returnvalue_4) (`KismetSystemLibrary.BoxTraceSingleForObjects` :`Start` _returnvalue_2 :`End` (+ _returnvalue_2 (* (`KismetMathLibrary.GetForwardVector` _returnvalue_3) 9999.0)) :`HalfSize` (16.0 16.0 16.0) :`Orientation` _returnvalue_3 :`ObjectTypes` (`|MakeArray` "ObjectTypeQuery11" :!type "EObjectTypeQuery Enum") :`DrawDebugType` "ForOneFrame"))
  (if _returnvalue_4
    (bind (_bblockinghit _binitialoverlap _time _distance _location _impactpoint _normal _impactnormal _physmat _hitactor) (`GameplayStatics.BreakHitResult` _outhit))
    (if (not (== (`self.Hovered Item`) _hitactor))
      (`/Engine/EditorBlueprintResources/StandardMacros.IsValid` _hovered_item
        (:`Is Valid`
          (`/Game/Items/BP_Item_Within_Inventory.Unhover Mesh` _hovered_item 0.5))
        (:`Is Not Valid`
          _))
      (bind _asbp_item_within_inventory (cast `/Game/Items/BP_Item_Within_Inventory` _hitactor))
      (`/Game/Items/BP_Item_Within_Inventory.Hover Mesh` _asbp_item_within_inventory 0.5)
      (set `self.Hovered Item` _asbp_item_within_inventory))
    (else
      (`/Engine/EditorBlueprintResources/StandardMacros.IsValid` (`self.Hovered Item`)
        (:`Is Valid`
          (`/Game/Items/BP_Item_Within_Inventory.Unhover Mesh` (`self.Hovered Item`) 0.5)
          (set `self.Hovered Item` null))))))

(fn `Inventory Place Line Trace`
  (returns (`Can Place Inventory Here?` :type Boolean) (Loc :type "Vector Structure") (Rot :type "Rotator Structure"))
  (bind _returnvalue (`self.GetOwner`))
  (bind _returnvalue_2 (`self.GetOwner`))
  (bind _returnvalue_3 (`Actor.K2_GetActorLocation` _returnvalue_2))
  (bind _returnvalue_4 (`Actor.K2_GetActorLocation` _returnvalue))
  (bind _returnvalue_5 (* (`Actor.GetActorForwardVector` _returnvalue) 200.0))
  (bind (_outhit _returnvalue_6) (`KismetSystemLibrary.BoxTraceSingleForObjects` (+ _returnvalue_4 _returnvalue_5) (+ _returnvalue_4 _returnvalue_5 (* (`Actor.GetActorUpVector` _returnvalue) -225.0)) (8.0 8.0 0.0) (`Actor.K2_GetActorRotation` _returnvalue) (`|MakeArray` "ObjectTypeQuery1" "ObjectTypeQuery2" :!type "EObjectTypeQuery Enum")))
  (bind (_bblockinghit _binitialoverlap _time _distance _location _impactpoint _normal _impactnormal _physmat _hitactor _hitcomponent _hitbonename _bonename _hititem _elementindex _faceindex _tracestart _traceend) (`GameplayStatics.BreakHitResult` _outhit))
  (`KismetSystemLibrary.PrintString` (`KismetSystemLibrary.GetDisplayName` _hitcomponent))
  (bind (_outhit_2 _returnvalue_7) (`KismetSystemLibrary.BoxTraceSingleForObjects` _returnvalue_3 (+ _returnvalue_3 (* (`Actor.GetActorForwardVector` _returnvalue_2) 150.0)) (16.0 64.0 48.0) (`Actor.K2_GetActorRotation` _returnvalue_2) (`|MakeArray` "ObjectTypeQuery1" "ObjectTypeQuery2" :!type "EObjectTypeQuery Enum") false (`|MakeArray` (`self.GetOwner`)) "ForDuration"))
  (`KismetSystemLibrary.PrintString` (`KismetSystemLibrary.GetDisplayName` (`.HitComponent` (`GameplayStatics.BreakHitResult` _outhit_2))))
  (bind (_returnvalue_roll _returnvalue_pitch _returnvalue_yaw) (`KismetMathLibrary.BreakRotator` (`KismetMathLibrary.MakeRotFromZ` _normal)))
  (return (select `bool` _returnvalue_6 :`true` (not _returnvalue_7)) (+ (`KismetMathLibrary.SelectVector` _location _traceend _returnvalue_6) (0.0 0.0 5.0)) (`KismetMathLibrary.MakeRotator` _returnvalue_roll _returnvalue_pitch _returnvalue_yaw)))