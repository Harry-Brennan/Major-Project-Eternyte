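; BP_Phone is a phone item that flashes a light for one second when used.
; Both PhoneLight and LightReflectionBack start dark, and UsePhone raises their intensity together, then zeroes it after a delay.
; AttemptPhone triggers UsePhone only while Active is set and AvailableUses is above zero, but no graph here decrements that count.
; ResetPhone copies AvailableUses into TotalUses, leaving AvailableUses unchanged.
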(event `self.ReceiveBeginPlay`
  (`LightComponent.SetIntensity` (`self.Phone Light`) 0.0)
  (`LightComponent.SetIntensity` (`self.Light Reflection Back`) 0.0))

(event `Reset Phone`
  (set `self.Total Uses` (`self.Available Uses`)))

(event `Use Phone`
  (`LightComponent.SetIntensity` (`self.Phone Light`) 20.0)
  (`LightComponent.SetIntensity` (`self.Light Reflection Back`) 20.0)
  (`KismetSystemLibrary.Delay` 1.0)
  (`LightComponent.SetIntensity` (`self.Phone Light`) 0.0)
  (`LightComponent.SetIntensity` (`self.Light Reflection Back`) 0.0))

(event `Attempt Phone`
  (if (`self.Active`)
    (if (> (`self.Available Uses`) 0)
      (`self.Use Phone`))))

(fn `UserConstructionScript`)