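; Item pickup actor that adds its named item to the player's inventory component when picked up.
; Its radius overlap registers it as the overlapping pickup on the other actor's BPC_Inventory, clearing it once no pickups overlap.
; AttemptPickup box-traces from the camera and succeeds only if this item is hit, then hides it and disables collision.
; ResetItemPickup restores visibility and collision, so the actor is reused rather than destroyed.
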(event `Attempt Pickup`
  (bind _returnvalue (`GameplayStatics.GetPlayerCameraManager` 0))
  (bind _returnvalue_2 (`PlayerCameraManager.GetCameraLocation` _returnvalue))
  (bind _returnvalue_3 (`PlayerCameraManager.GetCameraRotation` _returnvalue))
  (bind (_outhit _returnvalue_4) (`KismetSystemLibrary.BoxTraceSingleForObjects` :`Start` _returnvalue_2 :`End` (+ _returnvalue_2 (* (`KismetMathLibrary.GetForwardVector` _returnvalue_3) 500.0)) :`HalfSize` (8.0 8.0 8.0) :`Orientation` _returnvalue_3 :`ObjectTypes` (`|MakeArray` "ObjectTypeQuery12" :!type "EObjectTypeQuery Enum") :`DrawDebugType` "Persistent" :`bIgnoreSelf` false))
  (if _returnvalue_4
    (if (== (`.HitActor` (`GameplayStatics.BreakHitResult` _outhit)) self)
      (`/Game/Items/BPC_Inventory.Add Item to Inventory` (`self.GetComponentByClass` (`GameplayStatics.GetPlayerCharacter` 0) "/Game/Items/BPC_Inventory.BPC_Inventory_C") (`self.Item Name`))
      (`self.SetActorHiddenInGame` true)
      (`self.SetActorEnableCollision` false))))

(event `Reset Item Pickup`
  (`self.SetActorHiddenInGame` false)
  (`self.SetActorEnableCollision` true))

(event `self.Item Pickup Radius.OnComponentBeginOverlap`
  (params (OverlappedComponent :type "PrimitiveComponent Object Reference") (OtherActor :type "Actor Object Reference") (OtherComp :type "PrimitiveComponent Object Reference") (OtherBodyIndex :type Integer) (bFromSweep :type Boolean) (SweepResult :type "HitResult Structure (by ref)"))
  (set `/Game/Items/BPC_Inventory.Overlapping Item to Pickup` self (`self.GetComponentByClass` OtherActor "/Game/Items/BPC_Inventory.BPC_Inventory_C")))

(event `self.Item Pickup Radius.OnComponentEndOverlap`
  (params (OverlappedComponent :type "PrimitiveComponent Object Reference") (OtherActor :type "Actor Object Reference") (OtherComp :type "PrimitiveComponent Object Reference") (OtherBodyIndex :type Integer))
  (if (`KismetArrayLibrary.Array_IsEmpty` (`self.GetOverlappingActors` OtherActor "BP_Item_Pickup_C"))
    (set `/Game/Items/BPC_Inventory.Overlapping Item to Pickup` null (`self.GetComponentByClass` OtherActor "/Game/Items/BPC_Inventory.BPC_Inventory_C"))))

(fn `UserConstructionScript`)