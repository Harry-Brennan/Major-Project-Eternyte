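; BP_Item_Within_Inventory is the 3D actor representing an item in the inventory, with its mesh chosen by item name on BeginPlay.
; A timeline lifts it along the canvas's up vector on hover and reverses on unhover or when shown via add.
; Equipping blocks hover changes while a second timeline raises it further, then hides it and swaps it into the left hand through the player's BPC_Inventory.
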(event `Hide Item`
  (`self.SetActorEnableCollision` false)
  (`self.SetActorHiddenInGame` true))

(event `Show Item`
  (`self.SetActorEnableCollision` true)
  (`self.SetActorHiddenInGame` false)
  (set `self.Non-Hovered Location` (`self.K2_GetActorLocation`)))

(event `self.ReceiveBeginPlay`
  (`StaticMeshComponent.SetStaticMesh` (`self.Inventory Item Mesh`) (select `/Game/Items/Enum_Left_Hand_Items` (`self.Inventory Item Name`) :`NewEnumerator1` "/Game/Items/Left_Hand_Items/Phone/PhoneMesh.PhoneMesh" :`NewEnumerator2` "/Game/Models/Items/Rope_Pickup.Rope_Pickup" :`NewEnumerator3` "/Game/Items/Left_Hand_Items/Dynamite/Dynamite.Dynamite" :`NewEnumerator4` "/Game/Items/Left_Hand_Items/EMF/SM_EMF_Inventory_Rep.SM_EMF_Inventory_Rep" :!type "StaticMesh Object Reference")))

(event `Hover Mesh`
  (params (`Hover Time` :type "Float (double-precision)" :default 1.0))
  (if (not (`self.Equipping Item`))
    (`TimelineComponent.SetPlayRate` (`self.Hovering Timeline`) (/ 1.0 `Hover Time`))
    (bind (_direction _alpha) (`Timeline|Hovering Timeline` :!label _label)
      (:`Update`
        (`self.K2_SetActorLocation` (`KismetMathLibrary.VLerp` (`self.Non-Hovered Location`) (+ (`self.Non-Hovered Location`) (* (`self.GetActorUpVector` (`self.Canvas Ref`)) 10.0)) _alpha))))))

(event `Unhover Mesh`
  (params (`Unhover Time` :type "Float (double-precision)" :default 1.0))
  (if (not (`self.Equipping Item`))
    (`TimelineComponent.SetPlayRate` (`self.Hovering Timeline`) (/ 1.0 `Unhover Time`))
    (goto _label :!via `Reverse`)))

(event `Show Item Via Add`
  (params (Time :type "Float (double-precision)"))
  (`TimelineComponent.SetPlayRate` (`self.Hovering Timeline`) (/ 1.0 Time))
  (set `self.Equipping Item` false)
  (`self.SetActorEnableCollision` true)
  (goto _label :!via `ReverseFromEnd`))

(event `Equip Item`
  (params (`Equip Move Time` :type "Float (double-precision)"))
  (bind _returnvalue (`self.GetComponentByClass` (`GameplayStatics.GetPlayerCharacter` 0) "/Game/Items/BPC_Inventory.BPC_Inventory_C"))
  (`TimelineComponent.SetPlayRate` (`self.Equip Timeline`) (/ 1.0 `Equip Move Time`))
  (set `self.Equipping Item` true)
  (`KismetSystemLibrary.PrintString` "EQUIP ITEM")
  (set `self.Loc Before Equipping` (`self.K2_GetActorLocation`))
  (bind (_direction _alpha) (`Timeline|Equip Timeline` :!via `PlayFromStart`)
    (:`Update`
      (`self.K2_SetActorLocation` (`KismetMathLibrary.VLerp` (`self.Loc Before Equipping`) (+ (`self.Non-Hovered Location`) (* (`self.GetActorUpVector` (`self.Canvas Ref`)) 25.0)) _alpha)))
    (:`Finished`
      (`self.Hide Item`)
      (set `self.Equipping Item` false)
      (`/Game/Items/BPC_Inventory.Remove Item from Left Hand` _returnvalue)
      (`/Game/Items/BPC_Inventory.Add Item to Left Hand` _returnvalue (`self.Inventory Item Name`)))))

(fn `UserConstructionScript`)