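; Held phone item that briefly lights up to show the loop clock and date, with limited battery uses.
; UseItem starts a three-second activation that spends a use, or plays a no-battery sound when none remain.
; A looping timer refreshes the 23:xx time from the GameMode's loop time; on activation at minute 60, the screen reads "I'M COMING" instead.
; ResetPhone copies AvailableUses into TotalUses, rather than refilling AvailableUses.
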(event `self.ReceiveBeginPlay`
  (`parent.ReceiveBeginPlay`)
  (`LightComponent.SetIntensity` (`self.Phone Light`) 0.0)
  (set `self.Available Uses` (`self.Total Uses`)))

(event `Reset Phone`
  (set `self.Total Uses` (`self.Available Uses`)))

(event `Use Phone`
  (`FMODBlueprintStatics.PlayEventAtLocation` "/Game/FMOD/Events/Phone/Phone_Activation.Phone_Activation" (`KismetMathLibrary.MakeTransform` (`self.K2_GetActorLocation`)))
  (bind _returnvalue (`KismetSystemLibrary.K2_SetTimerDelegate` (delegate `Update Time While Active`) 0.05 true))
  (bind _current_loop_time (message `/Game/Core/Modes/BPI_Gamemode.Get Current Loop Time` (`GameplayStatics.GetGameMode`)))
  (bind _returnvalue_2 (+ (`KismetMathLibrary.FFloor` (/ _current_loop_time 60.0)) 55))
  (bind _returnvalue_3 (== _returnvalue_2 60))
  (`TextRenderComponent.K2_SetText` (`self.Time Text`) (`KismetSystemLibrary.MakeLiteralText` (`KismetTextLibrary.Conv_StringToText` (`KismetMathLibrary.SelectString` "COMING" (`KismetStringLibrary.Concat_StrStr` "23:" (`KismetStringLibrary.Conv_IntToString` _returnvalue_2)) _returnvalue_3))))
  (`TextRenderComponent.K2_SetText` (`self.Day Text`) (`KismetSystemLibrary.MakeLiteralText` (`KismetTextLibrary.Conv_StringToText` (`KismetMathLibrary.SelectString` "I'M" "29 FEB" _returnvalue_3))))
  (set `self.Phone Active` true)
  (`SceneComponent.SetHiddenInGame` (`self.Time Text`) false false)
  (`SceneComponent.SetHiddenInGame` (`self.Day Text`) false false)
  (`LightComponent.SetIntensity` (`self.Phone Light`) 1.0)
  (`KismetSystemLibrary.Delay` 3.0)
  (`LightComponent.SetIntensity` (`self.Phone Light`) 0.0)
  (`/Engine/EditorBlueprintResources/StandardMacros.DecrementInt` (`self.Available Uses`)
    (:`  `
      (set `self.Phone Active` false)
      (`SceneComponent.SetHiddenInGame` (`self.Time Text`) true false)
      (`SceneComponent.SetHiddenInGame` (`self.Day Text`) true false)
      (`KismetSystemLibrary.K2_ClearAndInvalidateTimerHandle` _returnvalue))))

(event `Force Deactivate Phone`
  (`SceneComponent.SetHiddenInGame` (`self.Time Text`) false false)
  (`LightComponent.SetIntensity` (`self.Phone Light`) 0.0)
  (`/Engine/EditorBlueprintResources/StandardMacros.DecrementInt` (`self.Available Uses`)
    (:`  `
      (set `self.Phone Active` false))))

(event `self.Use Item`
  (if (`self.Phone Active`)
    _
    (elif (> (`self.Available Uses`) 0)
      (`self.Use Phone`)
      (else
        (`FMODBlueprintStatics.PlayEventAtLocation` "/Game/FMOD/Events/Phone/Phone_No_Battery.Phone_No_Battery" (`KismetMathLibrary.MakeTransform` (`self.K2_GetActorLocation`)))))))

(event `Update Time While Active`
  (bind _current_loop_time (message `/Game/Core/Modes/BPI_Gamemode.Get Current Loop Time` (`GameplayStatics.GetGameMode`)))
  (bind _returnvalue (+ (`KismetMathLibrary.FFloor` (/ _current_loop_time 60.0)) 55))
  (if (not (== _returnvalue 60))
    (`TextRenderComponent.K2_SetText` (`self.Time Text`) (`KismetSystemLibrary.MakeLiteralText` (`KismetTextLibrary.Conv_StringToText` (`KismetStringLibrary.Concat_StrStr` "23:" (`KismetStringLibrary.Conv_IntToString` _returnvalue)))))))

(fn `UserConstructionScript`
  (`parent.UserConstructionScript`))