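; Destructible actor the player blows up by placing dynamite on it, hidden and made non-colliding after the blast until reset.
; UseRange overlap, backed by a polling timer for the equipped left-hand item, shows a player-facing placement prompt.
; ActivatePlacedDynamite reveals the mesh, plays fuse effects, then detonates after a delay.
; The sphere-traced blast launches players and physics bodies, with knockback growing with distance, plus Niagara effects and camera shake.
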(event `self.ReceiveBeginPlay`
  (bind _aswbp_wiggly_menu_text (cast `/Game/UI/Menus/WBP_Wiggly_Menu_Text` (`WidgetComponent.GetWidget` (`self.Dynamite Prompt`))))
  (bind _output_get (set `self.Dynamite Prompt Widget` _aswbp_wiggly_menu_text))
  (set `/Game/UI/Menus/WBP_Wiggly_Menu_Text.Text` "LMB PLACE DYNAMITE" _output_get)
  (set `/Game/UI/Menus/WBP_Wiggly_Menu_Text.Size` 360.0 _output_get)
  (set `/Game/UI/Menus/WBP_Wiggly_Menu_Text.Irregular Shake Intensity?` true _output_get)
  (set `/Game/UI/Menus/WBP_Wiggly_Menu_Text.Shake Intensity` 0.05 _output_get)
  (set `/Game/UI/Menus/WBP_Wiggly_Menu_Text.Text Colour` (struct :`R` 1.0 :`G` 1.0 :`B` 1.0 :`A` 1.0) _output_get)
  (set `/Game/UI/Menus/WBP_Wiggly_Menu_Text.Shadow Colour` (struct :`R` 0.119792 :`A` 1.0) _output_get)
  (`Widget.SetRenderOpacity` (`/Game/UI/Menus/WBP_Wiggly_Menu_Text.WiggleTextWrapBox` (`self.Dynamite Prompt Widget`)) 0.0)
  (`self.Activate Dynamite Destructible`))

(event `Activate Dynamite Destructible`
  (set `self.Active` true)
  (`self.SetActorHiddenInGame` false)
  (`self.SetActorEnableCollision` true))

(event `Reset Dynamite Destructibles`
  (`self.SetActorHiddenInGame` false)
  (`self.SetActorEnableCollision` true)
  (set `self.Active` true))

(event `Disable Dynamite Destructible`
  (if (`self.Active`)
    (`self.SetActorHiddenInGame` true)
    (`self.SetActorEnableCollision` false)
    (set `self.Active` false)))

(event `Dynamite Explosion`
  (bind _returnvalue (`SceneComponent.K2_GetComponentLocation` (`self.Dynamite Placed Mesh`)))
  (`KismetArrayLibrary.Array_Clear` (`self.Explosion Affected Actors`))
  (bind (_outhits _returnvalue_2) (`KismetSystemLibrary.SphereTraceMultiForObjects` :`Start` _returnvalue :`End` _returnvalue :`Radius` (`self.Explosion Affect Radius`) :`ObjectTypes` (`|MakeArray` "ObjectTypeQuery4" "ObjectTypeQuery8" :!type "EObjectTypeQuery Enum") :`DrawDebugType` "ForDuration" :`bIgnoreSelf` false))
  (if _returnvalue_2
    (for _array_element _outhits
      (bind (_bblockinghit _binitialoverlap _time _distance _location _impactpoint _normal _impactnormal _physmat _hitactor _hitcomponent) (`GameplayStatics.BreakHitResult` _array_element))
      (if (not (`KismetArrayLibrary.Array_Contains` (`self.Explosion Affected Actors`) _hitactor))
        (`KismetArrayLibrary.Array_Add` (`self.Explosion Affected Actors`) _hitactor)
        (bind _asbp_player (cast `/Game/Player/BP_Player` _hitactor)
          (:`then`
            (bind _returnvalue_3 (- (`self.K2_GetActorLocation` _asbp_player) (`SceneComponent.K2_GetComponentLocation` (`self.Dynamite Placed Mesh`))))
            (`Character.LaunchCharacter` _asbp_player (* _returnvalue_3 (* (/ (`KismetMathLibrary.VSize` _returnvalue_3) (`self.Explosion Affect Radius`)) (`self.Explosion Max Knockback`))) false false))
          (:`CastFailed`
            (if (`SceneComponent.IsSimulatingPhysics` _hitcomponent "None")
              (`KismetSystemLibrary.PrintString` (`KismetSystemLibrary.GetDisplayName` _hitcomponent))
              (bind _returnvalue_4 (- (`self.K2_GetActorLocation` _hitactor) (`SceneComponent.K2_GetComponentLocation` (`self.Dynamite Placed Mesh`))))
              (`PrimitiveComponent.AddImpulse` _hitcomponent (* _returnvalue_4 (* (/ (`KismetMathLibrary.VSize` _returnvalue_4) (`self.Explosion Affect Radius`)) (`self.Explosion Max Knockback`))) "None" true)))))))
  (`NiagaraFunctionLibrary.SpawnSystemAtLocation` "/Game/VFX/MsvFx_Niagara_Explosion_Pack_01/Prefabs/Niagara_Explosion_03.Niagara_Explosion_03" (`SceneComponent.K2_GetComponentLocation` (`self.Niagara Location`)) (struct) (3.0 3.0 3.0) true true "AutoRelease")
  (`NiagaraFunctionLibrary.SpawnSystemAtLocation` "/Game/VFX/MsvFx_Niagara_Explosion_Pack_01/Prefabs/Niagara_Explosion_02.Niagara_Explosion_02" (`SceneComponent.K2_GetComponentLocation` (`self.Niagara Location`)) (struct) (3.0 3.0 3.0) true true "AutoRelease")
  (`NiagaraFunctionLibrary.SpawnSystemAtLocation` "/Game/VFX/MsvFx_Niagara_Explosion_Pack_01/Prefabs/Niagara_Smoke_Wind_01.Niagara_Smoke_Wind_01" (`SceneComponent.K2_GetComponentLocation` (`self.Niagara Location`)) (struct) (3.0 3.0 3.0) true true "AutoRelease")
  (`LegacyCameraShake.StartLegacyCameraShake` (`GameplayStatics.GetPlayerCameraManager` 0) "/Game/Items/BP_Inventory_Camera_Shake.BP_Inventory_Camera_Shake_C" 3.0)
  (`KismetSystemLibrary.Delay` 0.05)
  (`self.Disable Dynamite Destructible`))

(event `Activate Placed Dynamite`
  (`SceneComponent.SetHiddenInGame` (`self.Dynamite Placed Mesh`) false false)
  (`FMODBlueprintStatics.PlayEventAtLocation` "/Game/FMOD/Events/Dynamite/Dynamite_Fuse_then_Explode.Dynamite_Fuse_then_Explode" (`KismetMathLibrary.MakeTransform` (`SceneComponent.K2_GetComponentLocation` (`self.Dynamite Placed Mesh`))))
  (`LegacyCameraShake.StartLegacyCameraShake` (`GameplayStatics.GetPlayerCameraManager` 0) "/Game/Items/BP_Inventory_Camera_Shake.BP_Inventory_Camera_Shake_C")
  (`NiagaraFunctionLibrary.SpawnSystemAtLocation` "/Game/VFX/MsvFx_Niagara_Explosion_Pack_01/Prefabs/Niagara_Splash_Flame_01.Niagara_Splash_Flame_01" (`SceneComponent.K2_GetComponentLocation` (`self.Dynamite Placed Mesh`)) (struct) (1.0 1.0 1.0) true true "AutoRelease")
  (`KismetSystemLibrary.Delay` 1.75)
  (`self.Dynamite Explosion`))

(event `Player Detection Loop`
  (if (and (`|EnumEquality` (`/Game/Items/BPC_Inventory.Left Hand Item` (`self.GetComponentByClass` (`GameplayStatics.GetPlayerCharacter` 0) "/Game/Items/BPC_Inventory.BPC_Inventory_C")) "NewEnumerator3") (`KismetArrayLibrary.Array_IsNotEmpty` (`self.GetOverlappingActors` "/Game/Player/BP_Player.BP_Player_C")))
    (`/Game/UI/Menus/WBP_Wiggly_Menu_Text.Fade Animation` (`self.Dynamite Prompt Widget`) true :!label _label)
    (bind _returnvalue (`KismetSystemLibrary.K2_SetTimerDelegate` (delegate `Prompt Auto Rotation`) 0.01 true))
    (set `self.Prompt Auto Rotate Timer` _returnvalue)
    (set `self.Prompt Active` true)
    (`KismetSystemLibrary.K2_ClearAndInvalidateTimerHandle` (`self.Player Detection Loop Timer`))))

(event `self.Use Range.OnComponentBeginOverlap`
  (params (OverlappedComponent :type "PrimitiveComponent Object Reference") (OtherActor :type "Actor Object Reference") (OtherComp :type "PrimitiveComponent Object Reference") (OtherBodyIndex :type Integer) (bFromSweep :type Boolean) (SweepResult :type "HitResult Structure (by ref)"))
  (if (`|EnumEquality` (`/Game/Items/BPC_Inventory.Left Hand Item` (`self.GetComponentByClass` (`GameplayStatics.GetPlayerCharacter` 0) "/Game/Items/BPC_Inventory.BPC_Inventory_C")) "NewEnumerator3")
    (goto _label)
    (else
      (bind _returnvalue (`KismetSystemLibrary.K2_SetTimerDelegate` (delegate `Player Detection Loop`) 0.25 true))
      (set `self.Player Detection Loop Timer` _returnvalue))))

(event `self.Use Range.OnComponentEndOverlap`
  (params (OverlappedComponent :type "PrimitiveComponent Object Reference") (OtherActor :type "Actor Object Reference") (OtherComp :type "PrimitiveComponent Object Reference") (OtherBodyIndex :type Integer))
  (if (`self.Prompt Active`) :!label _label_2
    (`/Game/UI/Menus/WBP_Wiggly_Menu_Text.Fade Animation` (`self.Dynamite Prompt Widget`) false)
    (`KismetSystemLibrary.K2_ClearAndInvalidateTimerHandle` (`self.Prompt Auto Rotate Timer`))
    (set `self.Prompt Active` false)))

(event `Force Hide Prompt`
  (goto _label_2))

(event `Prompt Auto Rotation`
  (`SceneComponent.K2_SetWorldRotation` (`self.Dynamite Prompt`) (`KismetMathLibrary.FindLookAtRotation` (`SceneComponent.K2_GetComponentLocation` (`self.Dynamite Prompt`)) (`self.K2_GetActorLocation` (stale `self.Use Range.OnComponentBeginOverlap` OtherActor))) false false))

(fn `UserConstructionScript`
  (bind _aswbp_wiggly_menu_text (cast `/Game/UI/Menus/WBP_Wiggly_Menu_Text` (`WidgetComponent.GetWidget` (`self.Dynamite Prompt`))))
  (bind _output_get (set `self.Dynamite Prompt Widget` _aswbp_wiggly_menu_text))
  (set `/Game/UI/Menus/WBP_Wiggly_Menu_Text.Text` "LMB PLACE DYNAMITE" _output_get)
  (set `/Game/UI/Menus/WBP_Wiggly_Menu_Text.Size` 512.0 _output_get)
  (set `/Game/UI/Menus/WBP_Wiggly_Menu_Text.Irregular Shake Intensity?` false _output_get)
  (set `/Game/UI/Menus/WBP_Wiggly_Menu_Text.Shake Intensity` 0.05 _output_get)
  (set `/Game/UI/Menus/WBP_Wiggly_Menu_Text.Text Colour` (struct :`R` 1.0 :`G` 1.0 :`B` 1.0 :`A` 1.0) _output_get)
  (set `/Game/UI/Menus/WBP_Wiggly_Menu_Text.Shadow Colour` (struct :`R` 0.119792 :`A` 1.0) _output_get))