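; BP_Dynamite_Held is the left-hand dynamite item that the player spends on destructible objects.
; On UseItem, it searches its owner's overlaps for the first active BP_Dynamite_Destructible, activates that object's placed dynamite and hides its prompt.
; It then updates the owner's BPC_Inventory, changing the left-hand slot and removing the acquired item, and hides the player's dynamite actor after a short delay.
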(event `self.Use Item`
  (bind _overlapped_dynamite_destructible (`self.Overlapped Dynamite Destructible`))
  (bind _returnvalue (`self.GetComponentByClass` (`self.GetOwner`) "/Game/Items/BPC_Inventory.BPC_Inventory_C"))
  (bind _overlappingactors (`self.GetOverlappingActors` (`self.GetOwner`) "/Game/Items/Left_Hand_Items/Dynamite/BP_Dynamite_Destructible.BP_Dynamite_Destructible_C"))
  (if (not (`KismetArrayLibrary.Array_IsEmpty` _overlappingactors))
    (for _array_element _overlappingactors
      (bind _asbp_dynamite_destructible (cast `/Game/Items/Left_Hand_Items/Dynamite/BP_Dynamite_Destructible` _array_element))
      (if (`/Game/Items/Left_Hand_Items/Dynamite/BP_Dynamite_Destructible.Active` _asbp_dynamite_destructible)
        (set `self.Overlapped Dynamite Destructible` _asbp_dynamite_destructible)
        (break)))
    (`/Engine/EditorBlueprintResources/StandardMacros.IsValid` _overlapped_dynamite_destructible
      (:`Is Valid`
        (`/Game/Items/Left_Hand_Items/Dynamite/BP_Dynamite_Destructible.Activate Placed Dynamite` _overlapped_dynamite_destructible)
        (`/Game/Items/Left_Hand_Items/Dynamite/BP_Dynamite_Destructible.Force Hide Prompt` (`self.Overlapped Dynamite Destructible`))
        (set `/Game/Items/BPC_Inventory.Left Hand Item` "NewEnumerator0" _returnvalue)
        (`KismetArrayLibrary.Array_RemoveItem` (`/Game/Items/BPC_Inventory.Items Acquired` _returnvalue) "NewEnumerator3")
        (`KismetSystemLibrary.Delay` 1.0)
        (`self.SetActorHiddenInGame` (`/Game/Items/BPC_Inventory.Player's Dynamite` _returnvalue) true)))))

(fn `UserConstructionScript`
  (`parent.UserConstructionScript`))