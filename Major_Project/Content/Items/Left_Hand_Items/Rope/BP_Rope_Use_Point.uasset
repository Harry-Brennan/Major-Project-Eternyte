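; Rope use point that marks where the player can abseil, showing a wiggly "LMB ABSAIL" world prompt.
; Entering StartArea fades the prompt in if the required left-hand item is held, otherwise a looping timer polls inventory and overlap.
; A fast timer turns the prompt toward the overlapping actor until exit or a forced hide.
; It also exposes an Active toggle and sizes the cable from the route spline's length.
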(event `self.ReceiveBeginPlay`
  (bind _aswbp_wiggly_menu_text (cast `/Game/UI/Menus/WBP_Wiggly_Menu_Text` (`WidgetComponent.GetWidget` (`self.Use Rope Prompt`))))
  (bind _output_get (set `self.As WBP Wiggly Menu Text` _aswbp_wiggly_menu_text))
  (set `/Game/UI/Menus/WBP_Wiggly_Menu_Text.Text` "LMB ABSAIL" _output_get)
  (set `/Game/UI/Menus/WBP_Wiggly_Menu_Text.Size` 360.0 _output_get)
  (set `/Game/UI/Menus/WBP_Wiggly_Menu_Text.Irregular Shake Intensity?` true _output_get)
  (set `/Game/UI/Menus/WBP_Wiggly_Menu_Text.Shake Intensity` 0.05 _output_get)
  (set `/Game/UI/Menus/WBP_Wiggly_Menu_Text.Text Colour` (struct :`R` 1.0 :`G` 1.0 :`B` 1.0 :`A` 1.0) _output_get)
  (set `/Game/UI/Menus/WBP_Wiggly_Menu_Text.Shadow Colour` (struct :`R` 0.119792 :`A` 1.0) _output_get)
  (`Widget.SetRenderOpacity` (`/Game/UI/Menus/WBP_Wiggly_Menu_Text.WiggleTextWrapBox` (`self.As WBP Wiggly Menu Text`)) 0.0)
  (`self.Activate Rope Use Point`)
  (set `CableComponent.CableLength` (/ (`SplineComponent.GetSplineLength` (`self.Absail Route`)) 4.0) (`self.Absailing Rope`)))

(event `Activate Rope Use Point`
  (set `self.Active` true))

(event `Deactivate Rope Use Point`
  (set `self.Active` false))

(event `Player Detection Loop`
  (if (and (`|EnumEquality` (`/Game/Items/BPC_Inventory.Left Hand Item` (`self.GetComponentByClass` (`GameplayStatics.GetPlayerCharacter` 0) "/Game/Items/BPC_Inventory.BPC_Inventory_C")) "NewEnumerator2") (`KismetArrayLibrary.Array_IsNotEmpty` (`self.GetOverlappingActors` "/Game/Player/BP_Player.BP_Player_C")))
    (`/Game/UI/Menus/WBP_Wiggly_Menu_Text.Fade Animation` (`self.As WBP Wiggly Menu Text`) true :!label _label)
    (bind _returnvalue (`KismetSystemLibrary.K2_SetTimerDelegate` (delegate `Prompt Auto Rotation`) 0.01 true))
    (set `self.Prompt Active` true)
    (`KismetSystemLibrary.K2_ClearAndInvalidateTimerHandle` (stale `self.Start Area.OnComponentBeginOverlap` _returnvalue))))

(event `self.Start Area.OnComponentBeginOverlap`
  (params (OverlappedComponent :type "PrimitiveComponent Object Reference") (OtherActor :type "Actor Object Reference") (OtherComp :type "PrimitiveComponent Object Reference") (OtherBodyIndex :type Integer) (bFromSweep :type Boolean) (SweepResult :type "HitResult Structure (by ref)"))
  (if (`|EnumEquality` (`/Game/Items/BPC_Inventory.Left Hand Item` (`self.GetComponentByClass` (`GameplayStatics.GetPlayerCharacter` 0) "/Game/Items/BPC_Inventory.BPC_Inventory_C")) "NewEnumerator2")
    (goto _label)
    (else
      (bind _returnvalue (`KismetSystemLibrary.K2_SetTimerDelegate` (delegate `Player Detection Loop`) 0.25 true)))))

(event `self.Start Area.OnComponentEndOverlap`
  (params (OverlappedComponent :type "PrimitiveComponent Object Reference") (OtherActor :type "Actor Object Reference") (OtherComp :type "PrimitiveComponent Object Reference") (OtherBodyIndex :type Integer))
  (if (`self.Prompt Active`) :!label _label_2
    (`/Game/UI/Menus/WBP_Wiggly_Menu_Text.Fade Animation` (`self.As WBP Wiggly Menu Text`) false)
    (`KismetSystemLibrary.K2_ClearAndInvalidateTimerHandle` (stale `Player Detection Loop` _returnvalue))
    (set `self.Prompt Active` false)))

(event `Prompt Auto Rotation`
  (`SceneComponent.K2_SetWorldRotation` (`self.Use Rope Prompt`) (`KismetMathLibrary.FindLookAtRotation` (`SceneComponent.K2_GetComponentLocation` (`self.Use Rope Prompt`)) (`self.K2_GetActorLocation` (stale `self.Start Area.OnComponentBeginOverlap` OtherActor))) false false))

(event `Force Hide Prompt`
  (goto _label_2))

(fn `UserConstructionScript`
  (bind _aswbp_wiggly_menu_text (cast `/Game/UI/Menus/WBP_Wiggly_Menu_Text` (`WidgetComponent.GetWidget` (`self.Use Rope Prompt`))))
  (bind _output_get (set `self.As WBP Wiggly Menu Text` _aswbp_wiggly_menu_text))
  (set `/Game/UI/Menus/WBP_Wiggly_Menu_Text.Text` "LMB ABSAIL" _output_get)
  (set `/Game/UI/Menus/WBP_Wiggly_Menu_Text.Size` 360.0 _output_get)
  (set `/Game/UI/Menus/WBP_Wiggly_Menu_Text.Irregular Shake Intensity?` true _output_get)
  (set `/Game/UI/Menus/WBP_Wiggly_Menu_Text.Shake Intensity` 0.05 _output_get)
  (set `/Game/UI/Menus/WBP_Wiggly_Menu_Text.Text Colour` (struct :`R` 1.0 :`G` 1.0 :`B` 1.0 :`A` 1.0) _output_get)
  (set `/Game/UI/Menus/WBP_Wiggly_Menu_Text.Shadow Colour` (struct :`R` 0.119792 :`A` 1.0) _output_get))