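; Player component that runs rope abseiling, swapping input mappings and using Flying movement until the descent ends in Falling.
; Starting attaches the rope point's cable to the player; a looping timer measures progress along its route spline, adjusts cable length and ends at spline's end.
; Input moves the player on world Z and X axes and stores clamped look angles.
; A second timer scales looping rope audio with speed, alongside random movement sounds.
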(event `self.ReceiveBeginPlay`
  (bind _asbp_player (cast `/Game/Player/BP_Player` (`self.GetOwner`)))
  (set `self.As BP Player` _asbp_player))

(event `Start Absail`
  (params (`Active Rope Use Point` :type "/Game/Items/Left_Hand_Items/Rope/BP_Rope_Use_Point Object Reference"))
  (bind _absailing_rope (`self.Absailing Rope`))
  (bind _returnvalue (`Actor.GetComponentByClass` (`self.GetOwner`) "/Script/Engine.CharacterMovementComponent"))
  (bind _returnvalue_2 (pcsubsystem `EnhancedInputLocalPlayerSubsystem` (`GameplayStatics.GetPlayerController` 0)))
  (set `self.Active Rope Use Point` `Active Rope Use Point`)
  (set `self.Current Distance Along Absail` 0.0)
  (set `self.Absailing Rope` (`Actor.GetComponentByClass` (`self.Active Rope Use Point`) "/Script/CableComponent.CableComponent"))
  (`/Engine/EditorBlueprintResources/StandardMacros.IsValid` _returnvalue_2
    (:`Is Valid`
      (`EnhancedInputSubsystemInterface.RemoveMappingContext` _returnvalue_2 "/Game/Player/Input/IMC_Default.IMC_Default" (struct))
      (`EnhancedInputSubsystemInterface.AddMappingContext` _returnvalue_2 "/Game/Player/Input/IMC_Absailing.IMC_Absailing" 0 (struct))
      (`CharacterMovementComponent.SetMovementMode` (`Actor.GetComponentByClass` (`self.GetOwner`) "/Script/Engine.CharacterMovementComponent") "MOVE_Flying" 0)
      (set `CharacterMovementComponent.MaxFlySpeed` (`self.Absail Speed`) _returnvalue)
      (set `CharacterMovementComponent.BrakingDecelerationFlying` (`self.Absail Stopping Speed`) _returnvalue)
      (set `Pawn.bUseControllerRotationYaw` false (`self.As BP Player`))
      (`KismetSystemLibrary.Delay` 0.35)
      (`LegacyCameraShake.StartLegacyCameraShake` (`GameplayStatics.GetPlayerCameraManager` 0) "/Game/Items/BP_Inventory_Camera_Shake.BP_Inventory_Camera_Shake_C")
      (bind _returnvalue_3 (`KismetSystemLibrary.K2_SetTimerDelegate` (delegate `Check Absail Distance`) 0.01 true))
      (set `self.Check Distance Timer` _returnvalue_3)
      (set `CableComponent.bAttachEnd` true _absailing_rope)
      (`CableComponent.SetAttachEndTo` _absailing_rope (`self.GetOwner`) "Mesh" "Absail_Rope_Socket")
      (set `CableComponent.EndLocation` (0.0 0.0 0.0) (`self.Absailing Rope`))
      (`SceneComponent.SetHiddenInGame` (`self.Absailing Rope`) false false)
      (set `self.Absailing` true)
      (bind _returnvalue_4 (`FMODBlueprintStatics.PlayEventAttached` "/Game/FMOD/Events/Absailing/Absail_Constant_Movement.Absail_Constant_Movement" (`Actor.GetComponentByClass` (`self.GetOwner`) "/Script/Engine.SkeletalMeshComponent") "Absail_Rope_Socket" (0.0 0.0 0.0) "SnapToTarget"))
      (bind _output_get (set `self.Continuous Movement Audio` _returnvalue_4))
      (`FMODAudioComponent.SetVolume` _output_get 0.0)
      (bind _returnvalue_5 (`KismetSystemLibrary.K2_SetTimerDelegate` (delegate `Finterp Continous Vol`) 0.01 true)))))

(event `End Absail`
  (bind _returnvalue (`Actor.GetComponentByClass` (`self.As BP Player`) "/Game/Items/BPC_Inventory.BPC_Inventory_C"))
  (bind _returnvalue_2 (pcsubsystem `EnhancedInputLocalPlayerSubsystem` (`GameplayStatics.GetPlayerController` 0)))
  (set `self.Absailing` false)
  (set `self.Active Rope Use Point` null)
  (`/Engine/EditorBlueprintResources/StandardMacros.IsValid` _returnvalue_2
    (:`Is Valid`
      (`EnhancedInputSubsystemInterface.RemoveMappingContext` _returnvalue_2 "/Game/Player/Input/IMC_Absailing.IMC_Absailing" (struct))
      (`EnhancedInputSubsystemInterface.AddMappingContext` _returnvalue_2 "/Game/Player/Input/IMC_Default.IMC_Default" 0 (struct))
      (`CharacterMovementComponent.SetMovementMode` (`Actor.GetComponentByClass` (`self.GetOwner`) "/Script/Engine.CharacterMovementComponent") "MOVE_Falling" 0)
      (`KismetSystemLibrary.K2_ClearAndInvalidateTimerHandle` (`self.Check Distance Timer`))
      (set `/Game/Items/BPC_Inventory.Right Hand Item` "NewEnumerator1" (`Actor.GetComponentByClass` (`self.GetOwner`) "/Game/Items/BPC_Inventory.BPC_Inventory_C"))
      (set `/Game/Items/BPC_Inventory.Right Hand Item` "NewEnumerator1" _returnvalue)
      (`Actor.SetActorHiddenInGame` (`/Game/Items/BPC_Inventory.Player's FlashLight` _returnvalue) false)
      (set `Pawn.bUseControllerRotationYaw` true (`self.As BP Player`))
      (set `CableComponent.bAttachEnd` false (`self.Absailing Rope`))
      (`LegacyCameraShake.StartLegacyCameraShake` (`GameplayStatics.GetPlayerCameraManager` 0) "/Game/Items/BP_Inventory_Camera_Shake.BP_Inventory_Camera_Shake_C")
      (`FMODBlueprintStatics.PlayEventAtLocation` "/Game/FMOD/Events/Absailing/Absail_Start_Stop.Absail_Start_Stop" (`KismetMathLibrary.MakeTransform` (`Actor.K2_GetActorLocation` (`self.GetOwner`))))
      (`FMODAudioComponent.Stop` (`self.Continuous Movement Audio`))
      (`KismetSystemLibrary.K2_ClearAndInvalidateTimerHandle` (stale `Start Absail` _returnvalue_5)))))

(event `Finterp Continous Vol`
  (bind _returnvalue (`KismetMathLibrary.FInterpTo` (`self.Continuous Vol`) (`KismetMathLibrary.MapRangeClamped` (`KismetMathLibrary.VSize` (`Actor.GetVelocity` (`self.GetOwner`))) 0.0 450.0 0.0 1.0) (`GameplayStatics.GetWorldDeltaSeconds`) (/ 1.0 0.4)))
  (`FMODAudioComponent.SetVolume` (`self.Continuous Movement Audio`) _returnvalue)
  (set `self.Continuous Vol` _returnvalue))

(event `EnhancedInput|/Game/Player/Input/Actions/IA_Absail_Movement`
  (params (ActionValue :type "Vector2D Structure") (ElapsedSeconds :type "Float (double-precision)") (TriggeredSeconds :type "Float (double-precision)") (InputAction :type "InputAction Object Reference" :default "/Game/Player/Input/Actions/IA_Absail_Movement.IA_Absail_Movement"))
  (:`Triggered`
    (`/Engine/EditorBlueprintResources/StandardMacros.IsValid` (`self.Active Rope Use Point`)
      (:`Is Valid`
        (`Pawn.AddMovementInput` (`self.As BP Player`) (0.0 0.0 1.0) ActionValue_Y false)
        (`Pawn.AddMovementInput` (`self.As BP Player`) (1.0 0.0 0.0) ActionValue_X false)
        (if (`KismetMathLibrary.RandomBoolWithWeight` 0.01)
          (`FMODBlueprintStatics.PlayEventAtLocation` "/Game/FMOD/Events/Absailing/Absail_Periodic_Movement.Absail_Periodic_Movement" (`KismetMathLibrary.MakeTransform` (+ (`SceneComponent.GetSocketLocation` (`Actor.GetComponentByClass` (`self.GetOwner`) "/Script/Engine.SkeletalMeshComponent") "Absail_Rope_Socket") (`KismetMathLibrary.MakeVector` 0.0 0.0 (`KismetMathLibrary.RandomFloatInRange` 5.0 25.0))))))))))

(event `Check Absail Distance`
  (if (>= (`self.Current Distance Along Absail`) (`SplineComponent.GetSplineLength` (`/Game/Items/Left_Hand_Items/Rope/BP_Rope_Use_Point.Absail Route` (`self.Active Rope Use Point`))))
    (`self.End Absail`)
    (else
      (bind _output_get (set `self.Current Distance Along Absail` (`SplineComponent.GetDistanceAlongSplineAtLocation` (`/Game/Items/Left_Hand_Items/Rope/BP_Rope_Use_Point.Absail Route` (`self.Active Rope Use Point`)) (`Actor.K2_GetActorLocation` (`self.GetOwner`)) "World")))
      (set `CableComponent.CableLength` (`KismetMathLibrary.FClamp` (- _output_get -200.0) 0.0 (`SplineComponent.GetSplineLength` (`/Game/Items/Left_Hand_Items/Rope/BP_Rope_Use_Point.Absail Route` (`self.Active Rope Use Point`)))) (`self.Absailing Rope`)))))

(event `EnhancedInput|/Game/Player/Input/Actions/IA_Absail_Look`
  (params (ActionValue :type "Vector2D Structure") (ElapsedSeconds :type "Float (double-precision)") (TriggeredSeconds :type "Float (double-precision)") (InputAction :type "InputAction Object Reference" :default "/Game/Player/Input/Actions/IA_Absail_Look.IA_Absail_Look"))
  (:`Triggered`
    (set `self.Look Vertical` (`KismetMathLibrary.FClamp` (+ (`self.Look Vertical`) ActionValue_Y) -60.0 50.0))
    (set `self.Look Horizontal` (`KismetMathLibrary.FClamp` (+ (`self.Look Horizontal`) ActionValue_X) -75.0 75.0))))