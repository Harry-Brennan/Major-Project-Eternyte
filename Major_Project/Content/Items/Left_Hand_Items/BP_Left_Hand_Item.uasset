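; BP_Left_Hand_Item is a single item Blueprint that represents whatever left-hand item is set by its ItemName enum: none, phone, rope or dynamite.
; A Select on ItemName sets the ItemBaseMesh static mesh, both in the Construction Script and again on BeginPlay.
; UseItem is a placeholder that only prints the item's name, with no per-item behavior.
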(event `self.ReceiveBeginPlay`
  (`StaticMeshComponent.SetStaticMesh` (`self.Item Base Mesh`) (select `/Game/Items/Enum_Left_Hand_Items` (`self.Item Name`) :`NewEnumerator1` "/Game/Items/Left_Hand_Items/Phone/PhoneMesh.PhoneMesh" :`NewEnumerator2` "/Game/Models/Items/Rope_Held.Rope_Held" :`NewEnumerator3` "/Game/Items/Left_Hand_Items/Dynamite/Dynamite.Dynamite" :!type "StaticMesh Object Reference")))

(event `Use Item`
  (`KismetSystemLibrary.PrintString` (`KismetStringLibrary.Concat_StrStr` "USE ITEM: " (`|GetEnumeratorNameAsString` (`self.Item Name`)))))

(fn `UserConstructionScript`
  (`StaticMeshComponent.SetStaticMesh` (`self.Item Base Mesh`) (select `/Game/Items/Enum_Left_Hand_Items` (`self.Item Name`) :`NewEnumerator1` "/Game/Items/Left_Hand_Items/Phone/PhoneMesh.PhoneMesh" :`NewEnumerator2` "/Game/Models/Items/Rope_Held.Rope_Held" :`NewEnumerator3` "/Game/Items/Left_Hand_Items/Dynamite/Dynamite.Dynamite" :!type "StaticMesh Object Reference")))