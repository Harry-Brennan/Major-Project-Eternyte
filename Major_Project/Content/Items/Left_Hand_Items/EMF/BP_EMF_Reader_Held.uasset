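; Held EMF reader item that toggles on use, showing nearby sources' strength through a jittering needle, beeps and static audio.
; Sources register readings in an actor-keyed map; looping timers take the highest to drive needle and beeps, while the reader randomly adds its own low-level noise.
; Battery drains while active, forcing shutoff when empty, and recharges after a delay.
; The battery mesh scales with charge and blinks when recharging stops.
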(event `Activate Recharging EMF`
  (bind _returnvalue (`KismetSystemLibrary.K2_SetTimerDelegate` (delegate `Recharging EMF Loop`) 0.01 true))
  (set `self.Recharging Loop Timer` _returnvalue)
  (set `self.Charge At Start Recharge` (`self.Current Charge`)))

(event `Recharging EMF Loop`
  (bind _output_get (set `self.Current Charge` (`KismetMathLibrary.FInterpTo_Constant` (`self.Current Charge`) 1.0 (`GameplayStatics.GetWorldDeltaSeconds`) (/ 1.0 (/ (`self.Full Recharge Time`) (- 1.0 (`self.Charge At Start Recharge`)))))))
  (`SceneComponent.SetRelativeScale3D` (`self.EMF Battery Bottom`) (`KismetMathLibrary.MakeVector` 1.0 _output_get 1.0))
  (if (== _output_get 1.0)
    (`self.Deactivate Recharging EMF`)))

(event `Calculate Highest EMF Reading`
  (bind _values (`BlueprintMapLibrary.Map_Values` (`self.Actor - Active EMF Readings`)))
  (set `self.Current Highest EMF` 0)
  (for _array_element _values
    (if (> _array_element (`self.Current Highest EMF`))
      (set `self.Current Highest EMF` _array_element)))
  (if (== (`self.Highest EMF Reading`) (`self.Current Highest EMF`))
    (if (`KismetMathLibrary.RandomBoolWithWeight` (select `int` (`self.Current Highest EMF`) :`0` 0.0 :`1` 0.05 :`2` 0.15 :`3` 0.25 :`4` 0.3 :!type "Float (single-precision)"))
      (`FMODBlueprintStatics.PlayEventAtLocation` "/Game/FMOD/Events/EMF/EMF_Beep.EMF_Beep" (`KismetMathLibrary.MakeTransform` (`self.K2_GetActorLocation`))))
    (else
      (`FMODBlueprintStatics.PlayEventAtLocation` "/Game/FMOD/Events/EMF/EMF_Beep.EMF_Beep" (`KismetMathLibrary.MakeTransform` (`self.K2_GetActorLocation`)))
      (set `self.Highest EMF Reading` (`self.Current Highest EMF`)))))

(event `Deactivate Recharging EMF`
  (`KismetSystemLibrary.K2_ClearAndInvalidateTimerHandle` (`self.Recharging Loop Timer`))
  (set `self.Recharging` false)
  (`PrimitiveComponent.SetMaterial` (`self.EMF Battery Bottom`) 0 null)
  (`KismetSystemLibrary.Delay` 0.05)
  (`PrimitiveComponent.SetMaterial` (`self.EMF Battery Bottom`) 0 "/Game/Items/Left_Hand_Items/EMF/M_EMF_Battery.M_EMF_Battery")
  (`KismetSystemLibrary.Delay` 0.05)
  (`PrimitiveComponent.SetMaterial` (`self.EMF Battery Bottom`) 0 null)
  (`KismetSystemLibrary.Delay` 0.05)
  (`PrimitiveComponent.SetMaterial` (`self.EMF Battery Bottom`) 0 "/Game/Items/Left_Hand_Items/EMF/M_EMF_Battery.M_EMF_Battery"))

(event `Update EMF Reading`
  (bind (_returnvalue_roll _returnvalue_pitch _returnvalue_yaw) (`KismetMathLibrary.BreakRotator` (select `int` (`self.Highest EMF Reading`) :`0` (struct :`Yaw` -250.0) :`1` (struct :`Yaw` -210.0) :`2` (struct :`Yaw` -170.0) :`3` (struct :`Yaw` -130.0) :`4` (struct :`Yaw` -90.0) :!type "Rotator Structure")))
  (set `self.Target EMF Reading Hand Rot` (`KismetMathLibrary.MakeRotator` 0.0 0.0 (`KismetMathLibrary.SelectFloat` (+ _returnvalue_yaw (`KismetMathLibrary.RandomFloatInRange` -30.0 30.0)) _returnvalue_yaw (`self.EMF Active`))))
  (`SceneComponent.K2_SetRelativeRotation` (`self.EMF Hand`) (`KismetMathLibrary.RInterpTo` (`SceneComponent.RelativeRotation` (`self.EMF Hand`)) (`self.Target EMF Reading Hand Rot`) (`GameplayStatics.GetWorldDeltaSeconds`) (/ 1.0 0.25)) false false)
  (if (`self.EMF Active`)
    (if (`KismetMathLibrary.RandomBoolWithWeight` 0.05)
      (`self.Toggle EMF Source` self true (`KismetMathLibrary.RandomInteger` 2)))))

(event `Toggle EMF Source`
  (params (`Source Actor` :type "Actor Object Reference") (Add :type Boolean) (Reading :type Integer))
  (bind _actor___active_emf_readings (`self.Actor - Active EMF Readings`))
  (if Add
    (`BlueprintMapLibrary.Map_Add` _actor___active_emf_readings `Source Actor` Reading)
    (else
      (`BlueprintMapLibrary.Map_Remove` _actor___active_emf_readings `Source Actor`))))

(event `self.Use Item`
  (bind _actor___active_emf_readings (`self.Actor - Active EMF Readings`))
  (bind _emf_static (`self.EMF Static`))
  (set `self.EMF Active` (not (`self.EMF Active`)))
  (`/Engine/EditorBlueprintResources/StandardMacros.IsValid` _emf_static :!label _label
    (:`Is Valid`
      (`FMODAudioComponent.Stop` _emf_static))
    (:`Is Not Valid`
      _))
  (`FMODBlueprintStatics.PlayEventAtLocation` "/Game/FMOD/Events/EMF/EMF_Click.EMF_Click" (`KismetMathLibrary.MakeTransform` (`self.K2_GetActorLocation`)))
  (if (`self.EMF Active`)
    (`self.Deactivate Recharging EMF`)
    (`KismetSystemLibrary.Delay` 0.2)
    (bind _returnvalue (`FMODBlueprintStatics.PlayEventAttached` "/Game/FMOD/Events/EMF/EMF_Static.EMF_Static" (`self.Item Base Mesh`) "None" (0.0 0.0 0.0) "SnapToTarget"))
    (set `self.EMF Static` _returnvalue)
    (bind _returnvalue_2 (`KismetSystemLibrary.K2_SetTimerDelegate` (delegate `Update EMF Reading`) 0.01 true))
    (bind _returnvalue_3 (`KismetSystemLibrary.K2_SetTimerDelegate` (delegate `Calculate Highest EMF Reading`) 0.05 true))
    (bind _returnvalue_4 (`KismetSystemLibrary.K2_SetTimerDelegate` (delegate `EMF Deplete Charge Loop`) 0.01 true))
    (set `self.Charge At Start Use` (`self.Current Charge`))
    (else
      (bind _keys (`BlueprintMapLibrary.Map_Keys` _actor___active_emf_readings))
      (for _array_element _keys
        (`BlueprintMapLibrary.Map_Add` _actor___active_emf_readings _array_element))
      (`KismetSystemLibrary.Delay` 0.5)
      (if (not (`self.EMF Active`))
        (`KismetSystemLibrary.K2_ClearAndInvalidateTimerHandle` _returnvalue_2)
        (`KismetSystemLibrary.K2_ClearAndInvalidateTimerHandle` _returnvalue_3)
        (`KismetSystemLibrary.K2_ClearAndInvalidateTimerHandle` _returnvalue_4)
        (`KismetSystemLibrary.Delay` (`self.Recharge Delay`))
        (if (not (`self.EMF Active`))
          (`self.Activate Recharging EMF`))))))

(event `Force Deactivate EMF`
  (set `self.EMF Active` false)
  (goto _label))

(event `EMF Deplete Charge Loop`
  (bind _output_get (set `self.Current Charge` (`KismetMathLibrary.FInterpTo_Constant` (`self.Current Charge`) 0.0 (`GameplayStatics.GetWorldDeltaSeconds`) (/ 1.0 (/ (`self.Full Charge Use Time`) (/ 1.0 (`self.Charge At Start Use`)))))))
  (`SceneComponent.SetRelativeScale3D` (`self.EMF Battery Bottom`) (`KismetMathLibrary.MakeVector` 1.0 _output_get 1.0))
  (if (`KismetMathLibrary.NearlyEqual_FloatFloat` _output_get 0.0 1e-05)
    (`KismetSystemLibrary.K2_ClearAndInvalidateTimerHandle` (stale `self.Use Item` _returnvalue_4))
    (`self.Force Deactivate EMF`)))

(fn `UserConstructionScript`
  (`parent.UserConstructionScript`))