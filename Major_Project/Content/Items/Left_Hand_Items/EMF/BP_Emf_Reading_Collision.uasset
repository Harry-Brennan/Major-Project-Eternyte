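; BP_Emf_Reading_Collision is an EMF source volume that feeds a reading to a player's EMF item.
; While Active, overlapping an actor with an inventory component registers this actor as a source on that player's EMF, but only if its reading beats the current highest.
; Ending the overlap while Active removes the source, without the validity or reading checks made on entry.
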(event `self.Player Detection.OnComponentBeginOverlap`
  (params (OverlappedComponent :type "PrimitiveComponent Object Reference") (OtherActor :type "Actor Object Reference") (OtherComp :type "PrimitiveComponent Object Reference") (OtherBodyIndex :type Integer) (bFromSweep :type Boolean) (SweepResult :type "HitResult Structure (by ref)"))
  (bind _returnvalue (`self.GetComponentByClass` OtherActor "/Game/Items/BPC_Inventory.BPC_Inventory_C"))
  (bind _player_s_emf (`/Game/Items/BPC_Inventory.Player's EMF` _returnvalue))
  (if (`self.Active?`)
    (`/Engine/EditorBlueprintResources/StandardMacros.IsValid` _returnvalue
      (:`Is Valid`
        (if (< (`/Game/Items/Left_Hand_Items/EMF/BP_EMF_Reader_Held.Highest EMF Reading` _player_s_emf) (`self.EMF Reading`))
          (`/Game/Items/Left_Hand_Items/EMF/BP_EMF_Reader_Held.Toggle EMF Source` _player_s_emf self true (`self.EMF Reading`)))))))

(event `self.Player Detection.OnComponentEndOverlap`
  (params (OverlappedComponent :type "PrimitiveComponent Object Reference") (OtherActor :type "Actor Object Reference") (OtherComp :type "PrimitiveComponent Object Reference") (OtherBodyIndex :type Integer))
  (if (`self.Active?`)
    (`/Game/Items/Left_Hand_Items/EMF/BP_EMF_Reader_Held.Toggle EMF Source` (`/Game/Items/BPC_Inventory.Player's EMF` (`self.GetComponentByClass` OtherActor "/Game/Items/BPC_Inventory.BPC_Inventory_C")) self false (`self.EMF Reading`))))

(fn `UserConstructionScript`)