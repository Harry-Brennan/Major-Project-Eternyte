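; BP_Loop_Action_Handler triggers world changes for loop actions, moving stale air or setting off landslides in named areas of the game.
; Its LoopAction event switches on a LoopActionType enum and calls the matching stale air or landslide reference, with all landslides sharing one hard-coded argument.
; Each incoming action type is also printed as a debug string.
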(event `Loop Action`
  (params (`Loop Action Type` :type "/Game/Core/Loop/Enum_Loop_Actions Enum" :default "NewEnumerator0"))
  (`KismetSystemLibrary.PrintString` (`|GetEnumeratorNameAsString` `Loop Action Type`))
  (switch `/Game/Core/Loop/Enum_Loop_Actions` `Loop Action Type`
    (:`NewEnumerator0`
      (`/Game/Environment_BPs/Stale_Air/BP_Moving_Stale_Air.Activate Stale Air Movement` (`self.Abseiling 2 Stale Air`)))
    (:`NewEnumerator4`
      (`/Game/Environment_BPs/Stale_Air/BP_Moving_Stale_Air.Activate Stale Air Movement` (`self.Quantum Crossroads Stale Air`)))
    (:`NewEnumerator1`
      (`/Game/Environment_BPs/Landslide/BP_Landslide.Activate Landslide` (`self.Upper Fog Twin Landslide`) 0.25))
    (:`NewEnumerator2`
      (`/Game/Environment_BPs/Landslide/BP_Landslide.Activate Landslide` (`self.Gravity Inverter Landslide`) 0.25))
    (:`NewEnumerator3`
      (`/Game/Environment_BPs/Landslide/BP_Landslide.Activate Landslide` (`self.Minecart Connector Landslide`) 0.25))))

(fn `UserConstructionScript`)