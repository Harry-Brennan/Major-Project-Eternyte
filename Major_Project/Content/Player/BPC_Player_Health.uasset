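; Player health component for BP_Player, handling damage, partial regeneration, death and reset.
; Damage triggers camera shake, blood effects and audio, then after a retriggerable delay regenerates health up to half.
; Looping timers ease walk speed and a blood-mask post-process material on the camera toward health-based values.
; Death ragdolls the mesh, notifies the game mode to restart the loop and spawns a temporary dead-body actor.
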(event Custom|Reset%20Player%20Health
  (bind _as_bp_player (Variables|Default|GetAs%20BP%20Player))
  (bind _mesh (Variables|/Script/Engine.Character|GetMesh _as_bp_player))
  (Variables|Default|SetHealth 1.0)
  (Variables|Default|SetAlive true)
  (Class|SkeletalMeshComponent|SetAllBodiesSimulatePhysics _mesh false)
  (Transformation|AttachComponentToComponent _mesh (Variables|/Script/Engine.Actor|GetRootComponent (Components|GetOwner)) "None" "SnapToTarget" "SnapToTarget" "KeepWorld" true)
  (Transformation|SetRelativeLocationAndRotation _mesh "0.000000,0.000000,-89.000000" "0.000000,-90.000000,0.000000" false false)
  (Variables|/Script/Engine.CharacterMovementComponent|SetMaxWalkSpeed (Actor|GetComponentbyClass (Variables|Default|GetAs%20BP%20Player) "/Script/Engine.CharacterMovementComponent") 3.5e+02))

(event Custom|Player%20Take%20Damage
  (params (Take%20Damage :type Float%20%28double-precision%29) (Location%20of%20Damage :type Vector) (Normal%20of%20Damage :type Vector))
  (bind _as_bp_player (Variables|Default|GetAs%20BP%20Player))
  (if (Variables|Default|GetAlive)
    (if (not (== Take%20Damage 0.0))
      (bind _output_get (Variables|Default|SetHealth (- (Variables|Default|GetHealth) Take%20Damage)))
      (Class|LegacyCameraShake|StartLegacyCameraShake (Game|GetPlayerCameraManager 0) "/Game/Player/BP_Take_Damage_CS.BP_Take_Damage_CS_C" (Math|Float|MapRangeClamped Take%20Damage 0.0 1.0 1.0 3.0) "CameraLocal" "0, 0, 0")
      (CallFunction|DeactivateHealthRegen)
      (Default|BloodEffect (Actor|GetComponentbyClass (Components|GetOwner) "/Game/VFX/Blood/Blood_Splatter/BPS/BPC_Blood_Effect.BPC_Blood_Effect_C") Location%20of%20Damage Normal%20of%20Damage (Components|GetOwner) Take%20Damage)
      (if (<= _output_get 0.0)
        (CallFunction|PlayerDeath)
        (else
          (Class|FMODBlueprintStatics|PlayEventatLocation "/Game/FMOD/Events/Player/Player_Take_Damage.Player_Take_Damage" (Math|Transform|MakeTransform (Transformation|GetActorLocation (Components|GetOwner)) "0, 0, 0" "1.000000,1.000000,1.000000"))))
      (if (Math|Boolean|NANDBoolean (Utilities|Time|IsValidTimerHandle (Variables|/Game/Player/BP_Player.BP_Player_C|GetCrouching%20Lerp%20Speed%20Timer _as_bp_player)) (Utilities|Time|IsValidTimerHandle (Variables|/Game/Player/BP_Player.BP_Player_C|GetLerp%20Sprint%20Speed%20Timer _as_bp_player)))
        (bind _returnvalue (Utilities|Time|SetTimerbyEvent (delegate Custom|Lerp%20Movement%20Speed%20For%20Health) 0.01 true))
        (Variables|Default|SetLerp%20Movement%20Speed%20Timer _returnvalue))
      (Utilities|FlowControl|RetriggerableDelay (Variables|Default|GetHealth%20Regen%20Delay))
      (if (Variables|Default|GetAlive)
        (CallFunction|ActivateHealthRegen)))))

(event Custom|Player%20Death
  (bind _returnvalue (Components|GetOwner))
  (bind _returnvalue_2 (Actor|GetComponentbyClass _returnvalue "/Script/Engine.SkeletalMeshComponent"))
  (Class|FMODBlueprintStatics|PlayEventatLocation "/Game/FMOD/Events/Player/Player_Death.Player_Death" (Math|Transform|MakeTransform (Transformation|GetActorLocation (Components|GetOwner)) "0, 0, 0" "1.000000,1.000000,1.000000"))
  (Variables|Default|SetAlive true)
  (Class|SkeletalMeshComponent|SetAllBodiesSimulatePhysics (Variables|/Script/Engine.Character|GetMesh (Variables|Default|GetAs%20BP%20Player)) true)
  (Class|BPIGamemode|RestartLoop(Message) (Game|GetGameMode))
  (Utilities|FlowControl|Delay 3.0)
  (bind _returnvalue_3 (Game|SpawnActorfromClass "/Game/Player/BP_Player_Dead_Body.BP_Player_Dead_Body_C" (Math|Transform|MakeTransform (Transformation|GetWorldLocation _returnvalue_2) (Transformation|GetWorldRotation _returnvalue_2) "1.000000,1.000000,1.000000") "Undefined" "MultiplyWithRoot" 0 _returnvalue_2 0))
  (Actor|SetLifeSpan _returnvalue_3 305.0))

(event Custom|Activate%20Health%20Regen
  (if (< (Variables|Default|GetHealth) 0.5)
    (bind _returnvalue (Utilities|Time|SetTimerbyEvent (delegate Custom|Health%20Regen%20Loop) 0.01 true))
    (Variables|Default|SetRegen%20Timer _returnvalue)))

(event Custom|Deactivate%20Health%20Regen
  (Utilities|Time|ClearandInvalidateTimerbyHandle (Variables|Default|GetRegen%20Timer)))

(event Custom|Health%20Regen%20Loop
  (bind _output_get (Variables|Default|SetHealth (+ (Variables|Default|GetHealth) 0.025)))
  (if (>= _output_get 0.5)
    (CallFunction|DeactivateHealthRegen)))

(event Custom|Interp%20Blood%20Mask
  (bind _returnvalue (Rendering|Material|GetScalarParameterValue (Variables|Default|GetBlood%20Damage%20Mask) "Radial Colour Amount" :!class /Script/Engine.MaterialInstanceDynamic))
  (Rendering|Material|SetScalarParameterValue (Variables|Default|GetBlood%20Damage%20Mask) "Radial Colour Amount" (Math|Interpolation|FInterptoConstant _returnvalue (Math|Float|MapRangeClamped (Variables|Default|GetHealth) 0.0 1.0 0.2 0.8) (Utilities|Time|GetWorldDeltaSeconds) 0.4) :!class /Script/Engine.MaterialInstanceDynamic)
  (bind _returnvalue_2 (Rendering|Material|GetScalarParameterValue (Variables|Default|GetBlood%20Damage%20Mask) "Blur Amount" :!class /Script/Engine.MaterialInstanceDynamic))
  (Rendering|Material|SetScalarParameterValue (Variables|Default|GetBlood%20Damage%20Mask) "Blur Amount" (Math|Interpolation|FInterptoConstant _returnvalue_2 (Math|Float|MapRangeClamped (Variables|Default|GetHealth) 0.0 1.0 0.4 0.0) (Utilities|Time|GetWorldDeltaSeconds) 0.4) :!class /Script/Engine.MaterialInstanceDynamic)
  (bind _returnvalue_3 (Rendering|Material|GetScalarParameterValue (Variables|Default|GetBlood%20Damage%20Mask) "Blur Effectiveness" :!class /Script/Engine.MaterialInstanceDynamic))
  (Rendering|Material|SetScalarParameterValue (Variables|Default|GetBlood%20Damage%20Mask) "Blur Effectiveness" (Math|Interpolation|FInterptoConstant _returnvalue_3 (Math|Float|MapRangeClamped (Variables|Default|GetHealth) 0.0 1.0 1.0 0.0) (Utilities|Time|GetWorldDeltaSeconds) 0.4) :!class /Script/Engine.MaterialInstanceDynamic))

(event Custom|Lerp%20Movement%20Speed%20For%20Health
  (bind _output_get (Variables|/Script/Engine.CharacterMovementComponent|SetMaxWalkSpeed (Actor|GetComponentbyClass (Variables|Default|GetAs%20BP%20Player) "/Script/Engine.CharacterMovementComponent") (Math|Interpolation|FInterptoConstant (Variables|/Script/Engine.CharacterMovementComponent|GetMaxWalkSpeed (Actor|GetComponentbyClass (Variables|Default|GetAs%20BP%20Player) "/Script/Engine.CharacterMovementComponent")) (Math|Float|Clamp(Float) (* 3.5e+02 (Math|Float|MapRangeClamped (Variables|Default|GetHealth) 0.0 0.75 0.0 1.0)) 175.0 3.5e+02) (Utilities|Time|GetWorldDeltaSeconds) 5e+01))))

(event EventBeginPlay
  (bind _asbp_player (Utilities|Casting|CastToBP_Player (Components|GetOwner)))
  (bind _output_get (Variables|Default|SetAs%20BP%20Player _asbp_player))
  (bind _returnvalue (Rendering|Material|CreateDynamicMaterialInstance "/Game/VFX/Blood/M_Blood_Damage_Mask.M_Blood_Damage_Mask" "None" "None" :!class /Script/Engine.KismetMaterialLibrary))
  (bind _output_get_2 (Variables|Default|SetBlood%20Damage%20Mask _returnvalue))
  (bind _structout (Utilities|Struct|SetmembersinPostProcessSettings (Variables|/Script/Engine.CameraComponent|GetPostProcessSettings (Actor|GetComponentbyClass _output_get "/Script/Engine.CameraComponent")) (Utilities|Struct|MakeWeightedBlendables (Utilities|Array|MakeArray (Utilities|Struct|MakeWeightedBlendable 1.0 _output_get_2)))))
  (Variables|/Script/Engine.CameraComponent|SetPostProcessSettings (Actor|GetComponentbyClass _output_get "/Script/Engine.CameraComponent") _structout)
  (Rendering|Material|SetScalarParameterValue (Variables|Default|GetBlood%20Damage%20Mask) "Radial Colour Amount" 1.0 :!class /Script/Engine.MaterialInstanceDynamic)
  (bind _returnvalue_2 (Utilities|Time|SetTimerbyEvent (delegate Custom|Interp%20Blood%20Mask) 0.01 true))
  (Variables|Default|SetInterp%20Blood%20Mask%20Timer _returnvalue_2))

(event Input|KeyboardEvents|DebugKeyX
  (params (Key :type Key%20Structure :default "None") (ActionValue :type Input%20Action%20Value%20Structure))
  (:Pressed
    (CallFunction|PlayerTakeDamage 0.1 (Transformation|GetActorLocation (Components|GetOwner)) (Math|Random|RandomUnitVector))))