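; BPC_Journal is a player component that stores the journal notes the player has acquired and handles opening the journal.
; Events add a note to the acquired list or clear it.
; The toggle input action asks the game mode to toggle the journal, but only while the owner's character movement is not falling.
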(event `Add Journal Note`
  (params (`Journal Note` :type "/Game/Player/Journal/Enum_Journal_Note_Names Enum" :default "NewEnumerator0"))
  (`KismetArrayLibrary.Array_Add` (`self.Acquired Journal Notes`) `Journal Note`))

(event `Reset Journal Notes`
  (`KismetArrayLibrary.Array_Clear` (`self.Acquired Journal Notes`)))

(event `EnhancedInput|/Game/Player/Input/Actions/Menus/IA_Toggle_Journal`
  (params (ActionValue :type Boolean) (ElapsedSeconds :type "Float (double-precision)") (TriggeredSeconds :type "Float (double-precision)") (InputAction :type "InputAction Object Reference" :default "/Game/Player/Input/Actions/Menus/IA_Toggle_Journal.IA_Toggle_Journal"))
  (:`Triggered`
    (if (not (`NavMovementComponent.IsFalling` (`Actor.GetComponentByClass` (`self.GetOwner`) "/Script/Engine.CharacterMovementComponent")))
      (message `/Game/Core/Modes/BPI_Gamemode.Toggle Journal GM` (`GameplayStatics.GetGameMode`)))))