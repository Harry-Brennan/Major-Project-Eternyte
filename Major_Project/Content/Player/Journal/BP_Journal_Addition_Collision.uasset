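; BP_Journal_Addition_Collision is a collision actor that adds a configured note to the player's journal once the game has reached a required loop count.
; On activation it checks the GameMode's loop count, then adds the note through the player's BPC_Journal component if not already acquired.
; It disables its own collision after adding the note, and a reset event turns collision back on.
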(event `Activate Journal Addition`
  (bind _returnvalue (`self.GetComponentByClass` (`GameplayStatics.GetPlayerCharacter` 0) "/Game/Player/Journal/BPC_Journal.BPC_Journal_C"))
  (bind _loop_count (message `/Game/Core/Modes/BPI_Gamemode.Get Loop Count` (`GameplayStatics.GetGameMode`)))
  (if (>= _loop_count (`self.Loop Count Required`))
    (if (not (`KismetArrayLibrary.Array_Contains` (`/Game/Player/Journal/BPC_Journal.Acquired Journal Notes` _returnvalue) (`self.Journal Note To Add`)))
      (`/Game/Player/Journal/BPC_Journal.Add Journal Note` _returnvalue (`self.Journal Note To Add`))
      (`self.SetActorEnableCollision` false))))

(event `Reset Journal Addition Collision`
  (`self.SetActorEnableCollision` true))

(fn `UserConstructionScript`)