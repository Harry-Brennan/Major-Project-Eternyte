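; Anim notify for Dweller footsteps that plays a step sound and spawns a dust poof.
; An RFoot flag picks the foot socket for the poof and trace, while the sound's socket names are None.
; Camera shake fades with the player's distance from the mesh.
; An object trace along the owner's up axis at the foot picks the Niagara poof colour, with debug drawing left on.
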(fn `Received_Notify`
  (params (MeshComp :type "SkeletalMeshComponent Object Reference") (Animation :type "AnimSequenceBase Object Reference") (EventReference :type "AnimNotifyEventReference Structure (by ref)"))
  (returns (ReturnValue :type Boolean))
  (bind _returnvalue (`Actor.GetActorUpVector` (`ActorComponent.GetOwner` MeshComp)))
  (bind _returnvalue_2 (`SceneComponent.GetSocketLocation` MeshComp (`KismetMathLibrary.SelectName` "RightFoot" "LeftFoot" (`self.R Foot?`))))
  (`FMODBlueprintStatics.PlayEventAtLocation` "/Game/FMOD/Events/Dweller/Step.Step" (`KismetMathLibrary.MakeTransform` (`SceneComponent.GetSocketLocation` MeshComp (`KismetMathLibrary.SelectName` "None" "None" (`self.R Foot?`)))))
  (`LegacyCameraShake.StartLegacyCameraShake` (`GameplayStatics.GetPlayerCameraManager` 0) "/Game/Creatures/Main_Creature/BP_Dweller_Step_Camera_Shake.BP_Dweller_Step_Camera_Shake_C" (`KismetMathLibrary.MapRangeClamped` (`KismetMathLibrary.Vector_Distance` (`SceneComponent.K2_GetComponentLocation` MeshComp) (`Actor.K2_GetActorLocation` (`GameplayStatics.GetPlayerCharacter` 0))) 0.0 3500.0 1.0 0.0))
  (bind (_outhit _returnvalue_3) (`KismetSystemLibrary.LineTraceSingleForObjects` :`Start` (+ _returnvalue_2 (* _returnvalue -250.0)) :`End` (+ _returnvalue_2 (* _returnvalue 25.0)) :`ObjectTypes` (`|MakeArray` "ObjectTypeQuery7" :!type "EObjectTypeQuery Enum") :`bTraceComplex` true :`DrawDebugType` "ForDuration" :`bIgnoreSelf` false))
  (bind _returnvalue_4 (`NiagaraFunctionLibrary.SpawnSystemAtLocation` "/Game/VFX/Characters/NS_Character_Foot_Poof.NS_Character_Foot_Poof" _returnvalue_2))
  (`NiagaraComponent.SetVariableLinearColor` _returnvalue_4 "Poof_Colour" (`KismetMathLibrary.SelectColor` (`KismetMathLibrary.MakeColor` 1.0) (`KismetMathLibrary.MakeColor` 0.19 0.06) _returnvalue_3))
  (return false))