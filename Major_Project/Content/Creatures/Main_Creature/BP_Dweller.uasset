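; Main monster character: idles, stalks, chases and attacks the player, exposing state getters alongside AIC_Dweller perception.
; Timers drive wander teleports, chase limits and sprint breathers.
; While stalking, camera-angle and trace checks build aggression when watched, ending in a roar and chase, or trigger fleeing and teleporting when sight breaks.
; Forced loop chase periodically relocates it near the player; attacks slow time, launch and damage the player.
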(event `self.ReceiveBeginPlay`
  (bind _asaic_dweller (cast `/Game/Creatures/Main_Creature/AI/AIC_Dweller` (`self.GetController`)))
  (set `self.As AIC Dweller` _asaic_dweller)
  (bind _asbp_player (cast `/Game/Player/BP_Player` (`GameplayStatics.GetPlayerCharacter` 0)))
  (set `self.Player Ref` _asbp_player))

(event `Dweller Sprint Breath`
  (set `CharacterMovementComponent.MaxWalkSpeed` 250.0 (`self.CharacterMovement`))
  (`KismetSystemLibrary.PrintString` "Dweller Out of Breath")
  (`FMODBlueprintStatics.PlayEventAtLocation` "/Game/FMOD/Events/Dweller/Dweller_Breath.Dweller_Breath" (`KismetMathLibrary.MakeTransform` (`self.K2_GetActorLocation`)))
  (`NiagaraFunctionLibrary.SpawnSystemAtLocation` "/Game/VFX/Characters/Breath/NS_Player_Breath.NS_Player_Breath" (`SceneComponent.GetSocketLocation` (`self.Mesh`) "Head") (struct) (1.0 1.0 1.0) true true "AutoRelease")
  (`KismetSystemLibrary.Delay` (`KismetMathLibrary.RandomFloatInRange` (`self.Min Breath Time`) (`self.Max Breath Time`)))
  (`KismetSystemLibrary.PrintString` "Dweller Out of Breath Finish")
  (set `CharacterMovementComponent.MaxWalkSpeed` 1000.0 (`self.CharacterMovement`))
  (bind _returnvalue (`KismetSystemLibrary.K2_SetTimerDelegate` (delegate `Dweller Sprint Breath`) (`KismetMathLibrary.RandomFloatInRange` (`self.Min Sprint Time`) (`self.Max Sprint Time`)) :!label _label))
  (set `self.Dweller Sprint Breath Timer` _returnvalue)
  (bind _returnvalue_2 (`KismetSystemLibrary.K2_SetTimerDelegate` (delegate `Chase Max Time`) (`KismetMathLibrary.RandomFloatInRange` 15.0 20.0)))
  (set `self.Chase Max Time Timer` _returnvalue_2)
  (`self.Reset Attack Do Once`)
  (message `/Game/Core/Modes/BPI_Gamemode.Activate Chase Lights` (`GameplayStatics.GetGameMode`)))

(event `Chase Max Time`
  (if (`|EnumEquality` (`self.Dweller State`) "NewEnumerator2")
    (`/Game/Creatures/Main_Creature/BPI_Dweller.Update to Stalking`)))

(event `/Game/Creatures/Main_Creature/BPI_Dweller.Update to Chasing`
  (bind _charactermovement (`self.CharacterMovement`))
  (set `self.Stalking Run Away` false)
  (set `self.Dweller State` "NewEnumerator2")
  (set `CharacterMovementComponent.MaxWalkSpeed` 1000.0 _charactermovement)
  (set `CharacterMovementComponent.MaxAcceleration` 1500.0 _charactermovement)
  (goto _label))

(event `/Game/Creatures/Main_Creature/BPI_Dweller.Update to Idling`
  (bind _charactermovement (`self.CharacterMovement`))
  (set `self.Stalking Run Away` false)
  (set `self.Dweller State` "NewEnumerator0")
  (set `CharacterMovementComponent.MaxWalkSpeed` 250.0 _charactermovement :!label _label_2)
  (set `CharacterMovementComponent.MaxAcceleration` 250.0 _charactermovement)
  (`KismetSystemLibrary.K2_ClearAndInvalidateTimerHandle` (`self.Dweller Sprint Breath Timer`))
  (`FMODAudioComponent.Play` (`self.Muttering / Whispering Sound`))
  (`FMODAudioComponent.Stop` (`self.Staring Sound`))
  (message `/Game/Core/Modes/BPI_Gamemode.Deactivate Chase Lights` (`GameplayStatics.GetGameMode`))
  (`FMODAudioComponent.Stop` (`self.Scream FMOD`)))

(event `/Game/Creatures/Main_Creature/BPI_Dweller.Update to Moving to New Area`
  (set `self.Dweller State` "NewEnumerator3")
  (goto _label_2))

(event `/Game/Creatures/Main_Creature/BPI_Dweller.Update Active`
  (params (`Active?` :type Boolean))
  (set `self.Active` `Active?`))

(event `/Game/Creatures/Main_Creature/BPI_Dweller.Update Area to Wander To`
  (params (`New Wander Area` :type "/Game/Creatures/Main_Creature/BP_Wandering_Area Object Reference"))
  (set `self.Move to Area` `New Wander Area`))

(event `/Game/Creatures/Main_Creature/BPI_Dweller.Start Wandering Timer`
  (`KismetSystemLibrary.K2_ClearAndInvalidateTimerHandle` (`self.Wandering Timer`))
  (set `self.Wandering Start Time` (`KismetSystemLibrary.GetGameTimeInSeconds`))
  (set `self.Wandering Max Time` (`KismetMathLibrary.RandomFloatInRange` 25.0 60.0))
  (set `self.Current Area` (`self.Move to Area`))
  (`/Game/Creatures/Main_Creature/BPI_Dweller.Update to Idling`)
  (bind _returnvalue (`KismetSystemLibrary.K2_SetTimerDelegate` (delegate `Wandering Timer Loop`) 0.5 true))
  (set `self.Wandering Timer` _returnvalue))

(event `Wandering Timer Loop`
  (bind _returnvalue (`self.K2_GetActorLocation`))
  (bind _possible_new_wandering_areas (`self.Possible New Wandering Areas`))
  (bind _returnvalue_2 (`self.K2_GetActorLocation` (`self.Move to Area`)))
  (bind _returnvalue_3 (+ (`NavigationSystemV1.K2_GetRandomReachablePointInRadius` _returnvalue_2 2000.0 null null) (0.0 0.0 50.0)))
  (if (>= (`KismetSystemLibrary.GetGameTimeInSeconds`) (+ (`self.Wandering Start Time`) (`self.Wandering Max Time`)))
    (if (`|EnumEquality` (`self.Dweller State`) "NewEnumerator0")
      (if (>= (`self.GetDistanceTo` (`GameplayStatics.GetPlayerCharacter` 0)) 2500.0)
        (bind _outactors (`GameplayStatics.GetAllActorsOfClass` "/Game/Creatures/Main_Creature/BP_Wandering_Area.BP_Wandering_Area_C"))
        (bind _output_get (set `self.Possible New Wandering Areas` _outactors))
        (`KismetArrayLibrary.Array_RemoveItem` _output_get (`self.Current Area`))
        (bind _asbp_wandering_area (cast `/Game/Creatures/Main_Creature/BP_Wandering_Area` (select `bool` (`KismetMathLibrary.RandomBoolWithWeight` 0.5) :`false` (`KismetArrayLibrary.Array_Random` _possible_new_wandering_areas) :`true` (`.ReturnValue` (`GameplayStatics.FindNearestActor` (`self.K2_GetActorLocation` (`GameplayStatics.GetPlayerCharacter` 0)) _possible_new_wandering_areas)) :!type "Actor Object Reference")))
        (`/Game/Creatures/Main_Creature/BPI_Dweller.Update Area to Wander To` _asbp_wandering_area)
        (set `self.Dweller State` "NewEnumerator3")
        (`KismetSystemLibrary.K2_ClearAndInvalidateTimerHandle` (`self.Wandering Timer`))
        (`FMODBlueprintStatics.PlayEventAtLocation` "/Game/FMOD/Events/Dweller/Teleport_New_Area.Teleport_New_Area" (`KismetMathLibrary.MakeTransform` _returnvalue_2))
        (if (<= (`KismetMathLibrary.Vector_Distance` _returnvalue_3 (`self.K2_GetActorLocation` (`GameplayStatics.GetPlayerCharacter` 0))) 1500.0) :!label _label_3
          (`KismetSystemLibrary.DelayUntilNextTick`)
          (goto _label_3)
          (else
            (`self.K2_SetActorLocation` _returnvalue_3)
            (`FMODBlueprintStatics.PlayEventAtLocation` "/Game/FMOD/Events/Dweller/Teleport_New_Area.Teleport_New_Area" (`KismetMathLibrary.MakeTransform` _returnvalue))
            (`|SpawnActorFromClass` "/Game/VFX/Blood/Bloodsplosion/BPs/BP_BloodSplosion.BP_BloodSplosion_C" (`KismetMathLibrary.MakeTransform` _returnvalue) "Undefined" "MultiplyWithRoot" null 150 null)))
        (else
          (set `self.Wandering Start Time` (`KismetSystemLibrary.GetGameTimeInSeconds`))))
      (else
        (`KismetSystemLibrary.K2_ClearAndInvalidateTimerHandle` (`self.Wandering Timer`))))))

(event `/Game/Creatures/Main_Creature/BPI_Dweller.Stop Wandering Timer Loop`
  (`KismetSystemLibrary.K2_ClearAndInvalidateTimerHandle` (`self.Wandering Timer`)))

(event `/Game/Creatures/Main_Creature/BPI_Dweller.Stare At Player`
  (`Controller.SetControlRotation` (`self.GetController`) (`KismetMathLibrary.FindLookAtRotation` (`self.K2_GetActorLocation`) (`self.K2_GetActorLocation` (`GameplayStatics.GetPlayerCharacter` 0)))))

(event `/Game/Creatures/Main_Creature/BPI_Dweller.Decrease Aggression Rating`
  (params (`Amount to Decrease By` :type "Float (double-precision)"))
  (bind _returnvalue (- (`self.Aggression Rating`) `Amount to Decrease By`))
  (if (<= _returnvalue 0.0)
    (`KismetSystemLibrary.K2_ClearAndInvalidateTimerHandle` (`self.Decrease Aggression Timer`))
    (else
      (set `self.Aggression Rating` _returnvalue))))

(event `/Game/Creatures/Main_Creature/BPI_Dweller.Increase Aggression Rating`
  (params (`Agression to Increase` :type "Float (double-precision)"))
  (bind _output_get (set `self.Aggression Rating` (+ (`self.Aggression Rating`) `Agression to Increase`)))
  (if (`self.Force Loop Chase Active`)
    (`KismetSystemLibrary.K2_ClearAndInvalidateTimerHandle` (`self.Staring Aggression Timer`))
    (`KismetSystemLibrary.K2_ClearAndInvalidateTimerHandle` (`self.Stalking Max Time Timer`))
    (elif (>= _output_get 1.0)
      (`KismetSystemLibrary.K2_ClearAndInvalidateTimerHandle` (`self.Staring Aggression Timer`))
      (set `self.Roaring` true)
      (`LegacyCameraShake.StartLegacyCameraShake` (`GameplayStatics.GetPlayerCameraManager` 0) "/Game/Creatures/Main_Creature/BP_Roar_Camera_Shake.BP_Roar_Camera_Shake_C")
      (bind _returnvalue (`FMODBlueprintStatics.PlayEventAttached` "/Game/FMOD/Events/Dweller/Scream.Scream" (`self.Mesh`) "Head" (0.0 0.0 0.0) "KeepRelativeOffset"))
      (set `self.Scream FMOD` _returnvalue)
      (`KismetSystemLibrary.K2_ClearAndInvalidateTimerHandle` (`self.Stalking Max Time Timer`)))))

(event `Roar End`
  (set `self.Roaring` false)
  (`/Game/Creatures/Main_Creature/BPI_Dweller.Update to Chasing`))

(event `/Game/Creatures/Main_Creature/BPI_Dweller.Reset Aggression Rating`
  (set `self.Aggression Rating` 0.0))

(event `/Game/Creatures/Main_Creature/BPI_Dweller.Update to Stalking`
  (if (`|EnumEquality` (`self.Dweller State`) "NewEnumerator1")
    _
    (elif (not (`self.Stalking Run Away`))
      (bind _returnvalue (`KismetSystemLibrary.K2_SetTimer` null "Stalking Max Time" (`KismetMathLibrary.RandomFloatInRange` 15.0 20.0)))
      (set `self.Stalking Max Time Timer` _returnvalue)
      (`FMODAudioComponent.Play` (`self.Staring Sound`))
      (`FMODAudioComponent.Stop` (`self.Muttering / Whispering Sound`))
      (`KismetSystemLibrary.K2_ClearAndInvalidateTimerHandle` (`self.Dweller Sprint Breath Timer`))
      (set `self.Rotation before Staring` (`self.K2_GetActorRotation`))
      (`|ExecutionSequence`
        (:`then_0`
          (bind (_direction _alpha) (`Timeline|Rotate to Face Player` :!via `PlayFromStart`)
            (:`Update`
              (`self.K2_SetActorRotation` (`KismetMathLibrary.RLerp` (`self.Rotation before Staring`) (`KismetMathLibrary.FindLookAtRotation` (`self.K2_GetActorLocation`) (`self.K2_GetActorLocation` (`GameplayStatics.GetPlayerCharacter` 0))) _alpha true)))))
        (:`then_1`
          (set `self.Dweller State` "NewEnumerator1")
          (bind _returnvalue_2 (`KismetSystemLibrary.K2_SetTimerDelegate` (delegate `Stalking Player Look At Check`) 0.01 true))
          (set `self.Stalking Player Look At Timer` _returnvalue_2))))))

(event `Decrease Aggression Rating Loop`
  (`/Game/Creatures/Main_Creature/BPI_Dweller.Decrease Aggression Rating` (/ 0.1 2.0)))

(event `Staring Aggression Increase`
  (`/Game/Creatures/Main_Creature/BPI_Dweller.Increase Aggression Rating` (/ 0.1 2.0)))

(event `Stalking Player Look At Check`
  (bind _player_ref (`self.Player Ref`))
  (bind _player_camera (`/Game/Player/BP_Player.Player Camera` (`self.Player Ref`)))
  (if (`KismetMathLibrary.InRange_FloatFloat` (`KismetMathLibrary.DegAcos` (`KismetMathLibrary.Dot_VectorVector` (`KismetMathLibrary.GetDirectionUnitVector` (`SceneComponent.K2_GetComponentLocation` _player_camera) (`self.K2_GetActorLocation`)) (`SceneComponent.GetForwardVector` _player_camera))) 0.0 (* (`PlayerCameraManager.GetFOVAngle` (`GameplayStatics.GetPlayerCameraManager` 0)) 0.5))
    (bind (_outhit _returnvalue) (`KismetSystemLibrary.LineTraceSingle` (`self.K2_GetActorLocation`) (+ (`SceneComponent.K2_GetComponentLocation` (`/Game/Player/BP_Player.Player Camera` _player_ref)) (* (`KismetMathLibrary.GetForwardVector` (`KismetMathLibrary.FindLookAtRotation` (`self.K2_GetActorLocation`) (`self.K2_GetActorLocation` _player_ref))) 25.0)) "TraceTypeQuery1" false (`|MakeArray` (`self.Player Ref`) :!type "Actor Object Reference") "ForOneFrame" false))
    (if _returnvalue
      (if (`self.Being Looked At`) :!label _label_4
        (if (`|EnumEquality` (`self.Dweller State`) "NewEnumerator1")
          (`KismetSystemLibrary.K2_ClearAndInvalidateTimerHandle` (`self.Stalking Max Time Timer`))
          (set `self.Being Looked At` false)
          (`/Game/Creatures/Main_Creature/BPI_Dweller.Stop Stalking Player Look At Check` :!label _label_5)
          (`self.Dweller Run From Player Sight`)
          (`KismetSystemLibrary.K2_ClearAndInvalidateTimerHandle` (`self.Staring Aggression Timer`))
          (`KismetSystemLibrary.K2_ClearAndInvalidateTimerHandle` (`self.Stalking Player Look At Timer`))
          (`KismetSystemLibrary.Delay` 1.0)
          (if (not (`self.Being Looked At`))
            (bind _returnvalue_2 (`KismetSystemLibrary.K2_SetTimerDelegate` (delegate `Decrease Aggression Rating Loop`) 0.1 true))
            (set `self.Decrease Aggression Timer` _returnvalue_2))
          (else
            (`KismetSystemLibrary.K2_ClearAndInvalidateTimerHandle` (`self.Stalking Player Look At Timer`)))))
      (elif (`self.Being Looked At`)
        (if (`|EnumEquality` (`self.Dweller State`) "NewEnumerator2")
          (`KismetSystemLibrary.K2_ClearAndInvalidateTimerHandle` (`self.Stalking Player Look At Timer`))
          (`KismetSystemLibrary.K2_ClearAndInvalidateTimerHandle` (`self.Decrease Aggression Timer`)))
        (else
          (set `self.Being Looked At` true)
          (`KismetSystemLibrary.K2_ClearAndInvalidateTimerHandle` (`self.Decrease Aggression Timer`))
          (if (not (`KismetSystemLibrary.K2_IsValidTimerHandle` (`self.Staring Aggression Timer`)))
            (bind _returnvalue_3 (`KismetSystemLibrary.K2_SetTimerDelegate` (delegate `Staring Aggression Increase`) 0.1 true))
            (set `self.Staring Aggression Timer` _returnvalue_3)))))
    (else
      (goto _label_4))))

(event `Stalking Max Time`
  (goto _label_5))

(event `/Game/Creatures/Main_Creature/BPI_Dweller.Stop Stalking Player Look At Check`
  (`KismetSystemLibrary.K2_ClearAndInvalidateTimerHandle` (`self.Stalking Player Look At Timer`)))

(event `Dweller Run From Player Sight`
  (bind _charactermovement (`self.CharacterMovement`))
  (`KismetSystemLibrary.PrintString` "DWELLER RUN FROM PLAYER SIGHT")
  (set `CharacterMovementComponent.MaxAcceleration` 1250.0 _charactermovement)
  (set `CharacterMovementComponent.MaxWalkSpeed` (* (`CharacterMovementComponent.MaxWalkSpeed` _charactermovement) 10.0) _charactermovement)
  (set `self.Stalking Run Away` true)
  (`KismetSystemLibrary.Delay` 3.0)
  (if (`self.Stalking Run Away`)
    (`/Game/Creatures/Main_Creature/BPI_Dweller.End / Stop Stalk Run Away`)))

(event `/Game/Creatures/Main_Creature/BPI_Dweller.End / Stop Stalk Run Away`
  (bind _charactermovement (`self.CharacterMovement`))
  (`KismetSystemLibrary.PrintString` "END STALK RUN AWAY")
  (set `CharacterMovementComponent.MaxAcceleration` 250.0 _charactermovement)
  (set `CharacterMovementComponent.MaxWalkSpeed` (/ (`CharacterMovementComponent.MaxWalkSpeed` _charactermovement) 10.0) _charactermovement)
  (set `self.Stalking Run Away` false)
  (`self.Teleport to Random Non-Player Area`))

(event `/Game/Creatures/Main_Creature/BPI_Dweller.Teleport to Random Non-Player Area`
  (`KismetSystemLibrary.PrintString` "TELEPORT TO RANDOM NON-PLAYER AREA")
  (bind _asbp_wandering_area (cast `/Game/Creatures/Main_Creature/BP_Wandering_Area` (`.ReturnValue` (`GameplayStatics.FindNearestActor` (`self.K2_GetActorLocation`) (`self.Possible New Wandering Areas`)))))
  (`KismetArrayLibrary.Array_RemoveItem` (`self.Possible New Wandering Areas`) _asbp_wandering_area)
  (`/Game/Creatures/Main_Creature/BPI_Dweller.Update Area to Wander To` null)
  (bind _output_get (set `self.Flee Area to Move to` (`KismetArrayLibrary.Array_Random` (`self.Possible New Wandering Areas`))))
  (bind _returnvalue (+ (`NavigationSystemV1.K2_GetRandomReachablePointInRadius` (`SceneComponent.K2_GetComponentLocation` (`/Game/Creatures/Main_Creature/BP_Wandering_Area.Area Centre` _output_get)) 350.0 null null) (0.0 0.0 50.0)))
  (`self.K2_SetActorLocation` _returnvalue)
  (`/Game/Creatures/Main_Creature/BPI_Dweller.Update Area to Wander To` _output_get)
  (set `self.Dweller State` "NewEnumerator3")
  (`FMODBlueprintStatics.PlayEventAtLocation` "/Game/FMOD/Events/Dweller/Teleport_New_Area.Teleport_New_Area" (`KismetMathLibrary.MakeTransform` _returnvalue)))

(event `/Game/Creatures/Main_Creature/BPI_Dweller.Force Loop Chase`
  (params (`First Loop?` :type Boolean))
  (bind _returnvalue (`self.K2_GetActorLocation` (`GameplayStatics.GetPlayerCharacter` 0)))
  (set `self.Active` false)
  (if `First Loop?`
    (bind _outactors (`GameplayStatics.GetAllActorsOfClassWithTag` "/Script/Engine.StaticMeshActor" "Dweller_First_Loop_Chase_Start"))
    (`self.K2_SetActorTransform` (`self.GetTransform` (`|GetArrayItem` _outactors)))
    (else
      (bind _randomlocation (`NavigationSystemV1.K2_GetRandomLocationInNavigableRadius` _returnvalue 5250.0 null null :!label _label_6))
      (if (<= (`KismetMathLibrary.Vector_Distance` _randomlocation _returnvalue) 5000.0)
        (goto _label_6)
        (else
          (`self.K2_SetActorTransform` (`KismetMathLibrary.MakeTransform` (+ _randomlocation (`KismetMathLibrary.MakeVector` 0.0 0.0 (`CapsuleComponent.GetScaledCapsuleHalfHeight` (`self.CapsuleComponent`)))) (`KismetMathLibrary.FindLookAtRotation` _randomlocation _returnvalue)))))))
  (set `self.Roaring` true)
  (`LegacyCameraShake.StartLegacyCameraShake` (`GameplayStatics.GetPlayerCameraManager` 0) "/Game/Creatures/Main_Creature/BP_Roar_Camera_Shake.BP_Roar_Camera_Shake_C")
  (bind _returnvalue_2 (`FMODBlueprintStatics.PlayEventAttached` "/Game/FMOD/Events/Dweller/Scream.Scream" (`self.Mesh`) "Head" (0.0 0.0 0.0) "KeepRelativeOffset"))
  (set `self.Scream FMOD` _returnvalue_2)
  (`KismetSystemLibrary.Delay` 1.0)
  (set `self.Force Loop Chase Active` true)
  (`self.Reset Attack Do Once`)
  (message `/Game/Core/Modes/BPI_Gamemode.Activate Chase Lights` (`GameplayStatics.GetGameMode`))
  (bind _returnvalue_3 (`KismetSystemLibrary.K2_SetTimerDelegate` (delegate `Force Chase Relocation Loop`) 15.0 true))
  (set `self.Force Chase Relocation Timer` _returnvalue_3))

(event `self.Attack Radius.OnComponentBeginOverlap`
  (params (OverlappedComponent :type "PrimitiveComponent Object Reference") (OtherActor :type "Actor Object Reference") (OtherComp :type "PrimitiveComponent Object Reference") (OtherBodyIndex :type Integer) (bFromSweep :type Boolean) (SweepResult :type "HitResult Structure (by ref)"))
  (`/Engine/EditorBlueprintResources/StandardMacros.DoOnce` false :!label _label_7
    (:`Completed`
      (`self.Attack`))))

(event `Force Chase Relocation Loop`
  (bind _returnvalue (`self.K2_GetActorLocation` (`GameplayStatics.GetPlayerCharacter` 0)))
  (if (`self.Force Loop Chase Active`)
    (bind _randomlocation (`NavigationSystemV1.K2_GetRandomLocationInNavigableRadius` _returnvalue 5250.0 null null :!label _label_8))
    (if (<= (`KismetMathLibrary.Vector_Distance` _randomlocation _returnvalue) 5000.0)
      (goto _label_8)
      (else
        (`self.K2_SetActorTransform` (`KismetMathLibrary.MakeTransform` (+ _randomlocation (`KismetMathLibrary.MakeVector` 0.0 0.0 (`CapsuleComponent.GetScaledCapsuleHalfHeight` (`self.CapsuleComponent`)))) (`KismetMathLibrary.FindLookAtRotation` _randomlocation _returnvalue)))))
    (else
      (`KismetSystemLibrary.K2_ClearAndInvalidateTimerHandle` (`self.Force Chase Relocation Timer`)))))

(event `Reset Attack Do Once`
  (goto _label_7 :!via `Reset`))

(event `Attack`
  (bind _returnvalue (`GameplayStatics.GetPlayerCharacter` 0))
  (bind _returnvalue_2 (`self.K2_GetActorLocation`))
  (bind _returnvalue_3 (`GameplayStatics.GetPlayerController` 0))
  (bind _returnvalue_4 (`GameplayStatics.GetGameMode`))
  (bind _returnvalue_5 (`GameplayStatics.GetGameMode`))
  (bind _scream_fmod (`self.Scream FMOD`))
  (bind _returnvalue_6 (`self.K2_GetActorLocation` (`GameplayStatics.GetPlayerCharacter` 0)))
  (bind _returnvalue_7 (`self.GetComponentByClass` (`GameplayStatics.GetPlayerCharacter` 0) "/Game/Items/BPC_Inventory.BPC_Inventory_C"))
  (bind _returnvalue_8 (`self.GetComponentByClass` (`GameplayStatics.GetPlayerCharacter` 0) "/Game/Items/Left_Hand_Items/Rope/BPC_Abseil.BPC_Abseil_C"))
  (set `self.Attacking` true)
  (`KismetSystemLibrary.K2_ClearAndInvalidateTimerHandle` (`self.Chase Max Time Timer`))
  (`KismetSystemLibrary.Delay` 0.2)
  (`/Engine/EditorBlueprintResources/StandardMacros.IsValid` _scream_fmod
    (:`Is Valid`
      (`FMODAudioComponent.Stop` _scream_fmod))
    (:`Is Not Valid`
      _))
  (`FMODBlueprintStatics.PlayEventAttached` "/Game/FMOD/Events/Dweller/Attack.Attack" (`self.Mesh`) "Head" (0.0 0.0 0.0) "KeepRelativeOffset")
  (`Controller.SetControlRotation` _returnvalue_3 (`KismetMathLibrary.FindLookAtRotation` _returnvalue_6 _returnvalue_2))
  (`EnhancedInputSubsystemInterface.RemoveMappingContext` (pcsubsystem `EnhancedInputLocalPlayerSubsystem` _returnvalue_3) "/Game/Player/Input/IMC_Default.IMC_Default" (struct))
  (if (`/Game/Items/BPC_Inventory.Inventory Open` _returnvalue_7)
    (`/Game/Items/BPC_Inventory.Force Close Inventory` _returnvalue_7)
    (else
      (bind _journal_open (message `/Game/Core/Modes/BPI_Gamemode.Is Journal Open` _returnvalue_5))
      (if _journal_open
        (message `/Game/Core/Modes/BPI_Gamemode.Force Close Journal` _returnvalue_5)
        (else
          (bind _pause_menu_open (message `/Game/Core/Modes/BPI_Gamemode.Is Pause Menu Open` _returnvalue_4))
          (if _pause_menu_open
            (message `/Game/Core/Modes/BPI_Gamemode.Force Close Pause Menu` _returnvalue_4)
            (elif (`/Game/Items/Left_Hand_Items/Rope/BPC_Abseil.Abseiling` _returnvalue_8)
              (`/Game/Items/Left_Hand_Items/Rope/BPC_Abseil.End Abseil` _returnvalue_8)))))))
  (set `Actor.CustomTimeDilation` 0.1 (`GameplayStatics.GetPlayerController` 0))
  (`self.LaunchCharacter` _returnvalue (+ (* (`KismetMathLibrary.GetForwardVector` (`KismetMathLibrary.FindLookAtRotation` (`self.K2_GetActorLocation` (`GameplayStatics.GetPlayerCharacter` 0)) (`self.K2_GetActorLocation`))) -1500.0) (0.0 0.0 750.0)) true true)
  (`KismetSystemLibrary.Delay` 0.15)
  (`/Game/Player/BPC_Player_Health.Player Take Damage` (`self.GetComponentByClass` _returnvalue "/Game/Player/BPC_Player_Health.BPC_Player_Health_C") 5.0 (`self.K2_GetActorLocation` (`GameplayStatics.GetPlayerCharacter` 0)) (- _returnvalue_6 _returnvalue_2))
  (`self.End attack`))

(event `/Game/Creatures/Main_Creature/BPI_Dweller.End attack`
  (`KismetSystemLibrary.PrintString` "END ATTACK")
  (set `self.Attacking` false)
  (set `Actor.CustomTimeDilation` 1.0 (`GameplayStatics.GetPlayerController` 0)))

(fn `Get Active`
  (returns (Active :type Boolean))
  (return (`self.Active`)))

(fn `Get Area Moving To`
  (returns (`Area Moving To Ref` :type "/Game/Creatures/Main_Creature/BP_Wandering_Area Object Reference"))
  (return (`self.Move to Area`)))

(fn `Get Area To Wander To`
  (returns (`Area To Wander To` :type "/Game/Creatures/Main_Creature/BP_Wandering_Area Object Reference"))
  (return (`self.Move to Area`)))

(fn `Get Can See Player`
  (returns (`Can See Player` :type Boolean))
  (return (`/Game/Creatures/Main_Creature/AI/AIC_Dweller.Seeing Player` (`self.As AIC Dweller`))))

(fn `Get Can Sense Player`
  (returns (`Can Sense Player` :type Boolean))
  (return (`/Game/Creatures/Main_Creature/AI/AIC_Dweller.Sensing Player` (`self.As AIC Dweller`))))

(fn `Get Current State`
  (returns (`Current State` :type "/Game/Creatures/Main_Creature/Enum_Dweller_State Enum"))
  (return (`self.Dweller State`)))

(fn `Get Current Wandering Area`
  (returns (`Wandering Area` :type "/Game/Creatures/Main_Creature/BP_Wandering_Area Object Reference"))
  (return (`self.Current Area`)))

(fn `Get Player Looking At Dweller`
  (returns (`Player Looking At Dweller` :type Boolean))
  (return (`self.Being Looked At`)))

(fn `Get Should Stalk Move`
  (returns (`Should Stalk Move` :type Boolean))
  (return (or (not (`self.Being Looked At`)) (`self.Stalking Run Away`))))

(fn `Get Stalk Run Away`
  (returns (`Stalk Run Away` :type Boolean))
  (return (`self.Stalking Run Away`)))

(fn `Get Wandering Timer`
  (returns (`Wandering Timer` :type "TimerHandle Structure"))
  (return (`self.Wandering Timer`)))

(fn `Is Attacking`
  (returns (Attacking :type Boolean))
  (return false))

(fn `Is Force Loop Chase Active`
  (returns (`Force Loop Chase` :type Boolean))
  (return (`self.Force Loop Chase Active`)))

(fn `UserConstructionScript`)