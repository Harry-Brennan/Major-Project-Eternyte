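; Cave eye creature Blueprint whose moving eye mesh follows the player by shifting between preset local positions.
; On BeginPlay, a slow looping timer picks the preset, transformed by the main eye mesh, that lies closest to the player character.
; A fast looping timer interpolates the moving mesh's relative location toward that target, avoiding Tick.
; A deactivate event clears both timers.
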(event `Update Eye Position`
  (`SceneComponent.K2_SetRelativeLocation` (`self.Moving Eye SM`) (`KismetMathLibrary.VInterpTo` (`SceneComponent.RelativeLocation` (`self.Moving Eye SM`)) (`self.Look At Position`) (`GameplayStatics.GetWorldDeltaSeconds`) (/ 1.0 1.0)) false false))

(event `self.ReceiveBeginPlay`
  (`self.Activate Player Tracking`))

(event `Activate Player Tracking`
  (bind _returnvalue (`KismetSystemLibrary.K2_SetTimerDelegate` (delegate `Player Tracking Calc`) 0.25 true))
  (set `self.Tracking Timer` _returnvalue)
  (bind _returnvalue_2 (`KismetSystemLibrary.K2_SetTimerDelegate` (delegate `Update Eye Position`) 0.01 true))
  (set `self.Update Eye Position Timer` _returnvalue_2))

(event `Player Tracking Calc`
  (bind _vector (`self.Find Closest Possible Tracking Position`))
  (set `self.Look At Position` _vector))

(event `Deactivate Player Tracking`
  (`KismetSystemLibrary.K2_ClearAndInvalidateTimerHandle` (`self.Tracking Timer`))
  (`KismetSystemLibrary.K2_ClearAndInvalidateTimerHandle` (`self.Update Eye Position Timer`)))

(fn `Find Closest Possible Tracking Position`
  (returns (Vector :type "Vector Structure"))
  (locals (`Closest Index` :type Integer) (`Closest Distance` :type "Float (double-precision)" :default 99999.0))
  (if (> (`KismetArrayLibrary.Array_Length` (`self.Possible Eye Positions (local)`)) 1)
    (for (_array_element _array_index) (`self.Possible Eye Positions (local)`)
      (bind _returnvalue (`KismetMathLibrary.Vector_Distance` (`KismetMathLibrary.TransformLocation` (`SceneComponent.K2_GetComponentToWorld` (`self.Main Eye SM`)) _array_element) (`self.K2_GetActorLocation` (`GameplayStatics.GetPlayerCharacter` 0))))
      (if (< _returnvalue (`local.Closest Distance`))
        (set `local.Closest Distance` _returnvalue)
        (set `local.Closest Index` _array_index)))
    (return (`|GetArrayItem` (`self.Possible Eye Positions (local)`) (`local.Closest Index`)))
    (else
      (return (`|GetArrayItem` (`self.Possible Eye Positions (local)`) (`local.Closest Index`))))))

(fn `UserConstructionScript`)