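; Blood explosion actor that bursts on spawn with sound and a Niagara effect sized by BloodAmount, healing nearby actors before destroying itself after a short delay.
; A debug-drawn sphere trace heals each unique interface-implementing hit actor except the owner, scaled by BloodAmount and horizontal distance falloff.
; Niagara exports particle data back to the actor, which spawns fading, randomly sized blood decals facing against particle velocity and plays a splatter sound.
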(event `self.ReceiveBeginPlay`
  (bind _returnvalue (`self.K2_GetActorLocation`))
  (bind _hit_players (`self.Hit Players`))
  (bind _returnvalue_2 (`KismetMathLibrary.Conv_IntToDouble` (* (`self.Blood_Amount`) 3)))
  (`NiagaraComponent.SetVariableInt` (`self.BloodSplosion`) "user.Blood_Amount" (`self.Blood_Amount`))
  (`NiagaraComponent.SetVariableObject` (`self.BloodSplosion`) "user.BP_Blood" self)
  (`GameplayStatics.PlaySoundAtLocation` "/Game/VFX/Bloodsplosion/Audio/BloodSplosion_SC.BloodSplosion_SC" (`self.K2_GetActorLocation`) (struct) 1.0 1.0 0.0 null null null null)
  (`|ExecutionSequence`
    (:`then_0`
      (`KismetArrayLibrary.Array_Clear` (`self.Hit Players`))
      (bind (_outhits _returnvalue_3) (`KismetSystemLibrary.SphereTraceMultiForObjects` :`Start` _returnvalue :`End` _returnvalue :`Radius` _returnvalue_2 :`ObjectTypes` (`|MakeArray` "ObjectTypeQuery8" :!type "EObjectTypeQuery Enum") :`DrawDebugType` "ForDuration"))
      (if _returnvalue_3
        (for _array_element _outhits
          (bind (_bblockinghit _binitialoverlap _time _distance _location _impactpoint _normal _impactnormal _physmat _hitactor) (`GameplayStatics.BreakHitResult` _array_element))
          (if (not (`KismetArrayLibrary.Array_Contains` _hit_players _hitactor))
            (`KismetArrayLibrary.Array_Add` _hit_players _hitactor)
            (if (and (`KismetSystemLibrary.DoesImplementInterface` _hitactor) (!= (`self.GetOwner`) _hitactor))
              (bind (_returnvalue_x _returnvalue_y _returnvalue_z) (`KismetMathLibrary.BreakVector` (`self.K2_GetActorLocation` _hitactor)))
              (`self.Heal` (`self.GetComponentByClass` _hitactor null) (`KismetMathLibrary.Conv_IntToDouble` (`KismetMathLibrary.FFloor` (* (/ (`self.Blood_Amount`) 3) (- 1.0 (/ (- (`KismetMathLibrary.VSize` (- (`KismetMathLibrary.MakeVector` (.x (`self.K2_GetActorLocation`)) (.y (`self.K2_GetActorLocation`)) _returnvalue_z) (`KismetMathLibrary.MakeVector` _returnvalue_x _returnvalue_y _returnvalue_z))) 75.0) _returnvalue_2)))))))))))
    (:`then_1`
      (`KismetSystemLibrary.Delay` 2.2)
      (`self.K2_DestroyActor`))))

(event `self.ReceiveParticleData`
  (params (Data :type "Array of BasicParticleData Structure (by ref)") (NiagaraSystem :type "NiagaraSystem Object Reference") (SimulationPositionOffset :type "Vector Structure (by ref)"))
  (bind _blood_amount (`self.Blood_Amount`))
  (for _array_element Data
    (bind (_position _size _velocity) (break `BasicParticleData` _array_element))
    (bind _returnvalue (`GameplayStatics.SpawnDecalAtLocation` "/Game/VFX/Blood_Splatter/Materials/MI_Blood_Decal_Advanced.MI_Blood_Decal_Advanced" (128.0 256.0 256.0) _position (`KismetMathLibrary.Conv_VectorToRotator` (* _velocity -1.0))))
    (`DecalComponent.SetFadeOut` _returnvalue 3.0 5.0 true)
    (bind _returnvalue_2 (`DecalComponent.CreateDynamicMaterialInstance` _returnvalue))
    (`MaterialInstanceDynamic.SetScalarParameterValue` _returnvalue_2 "Radius" (`KismetMathLibrary.FClamp` (`KismetMathLibrary.Lerp` (* _blood_amount 0.1) (`KismetMathLibrary.Conv_IntToDouble` _blood_amount) (`KismetMathLibrary.RandomFloatInRange` 0.0 1.0)) 1.0 300.0)))
  (`GameplayStatics.PlaySoundAtLocation` "/Game/VFX/Blood_Splatter/Audio/Blood_Audio/Blood_Splatter_SC.Blood_Splatter_SC" _position (struct) 1.0 1.0 0.0 null null null null))

(fn `UserConstructionScript`)