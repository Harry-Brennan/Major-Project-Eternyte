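; Blood drop effect actor that turns Niagara particle data into fading blood decals with a splatter sound.
; On BeginPlay it passes itself to the Niagara system as a user object to receive exported particle data.
; Each particle spawns a decal oriented against its velocity, with a randomized radius set through a dynamic material instance.
; After each batch's loop, one sound plays using the loop element's position.
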(event `self.ReceiveBeginPlay`
  (`NiagaraComponent.SetVariableObject` (`self.NS_Blood_Effect`) "user.BP_Blood" self))

(event `self.ReceiveParticleData`
  (params (Data :type "Array of BasicParticleData Structure (by ref)") (NiagaraSystem :type "NiagaraSystem Object Reference") (SimulationPositionOffset :type "Vector Structure (by ref)"))
  (bind _decalsize (`self.DecalSize`))
  (for _array_element Data
    (bind (_position _size _velocity) (break `BasicParticleData` _array_element))
    (bind _returnvalue (`GameplayStatics.SpawnDecalAtLocation` "/Game/VFX/Blood_Splatter/Materials/MI_Blood_Decal_Advanced.MI_Blood_Decal_Advanced" (128.0 256.0 256.0) _position (`KismetMathLibrary.Conv_VectorToRotator` (* _velocity -1.0))))
    (`DecalComponent.SetFadeOut` _returnvalue 3.0 5.0 true)
    (bind _returnvalue_2 (`DecalComponent.CreateDynamicMaterialInstance` _returnvalue))
    (`MaterialInstanceDynamic.SetScalarParameterValue` _returnvalue_2 "Radius" (`KismetMathLibrary.FClamp` (`KismetMathLibrary.Lerp` (* _decalsize 0.1) _decalsize (`KismetMathLibrary.RandomFloatInRange` 0.0 1.0)) 1.0 300.0)))
  (`GameplayStatics.PlaySoundAtLocation` "/Game/VFX/Blood_Splatter/Audio/Blood_Audio/Blood_Splatter_SC.Blood_Splatter_SC" _position (struct) 1.0 1.0 0.0 null null null null))

(fn `UserConstructionScript`)