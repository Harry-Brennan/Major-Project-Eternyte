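; Animation notify that spawns the Niagara foot poof effect on a character's mesh at a named socket.
; A complex line trace along the owner's up axis through the socket checks one object type, with debug drawing left on.
; The hit result tints the attached effect's Poof_Colour red on a hit, dark brown otherwise.
; Spawning only happens when Attached is set, with no unattached fallback.
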(fn `Received_Notify`
  (params (MeshComp :type "SkeletalMeshComponent Object Reference") (Animation :type "AnimSequenceBase Object Reference") (EventReference :type "AnimNotifyEventReference Structure (by ref)"))
  (returns (ReturnValue :type Boolean))
  (bind _returnvalue (`Actor.GetActorUpVector` (`ActorComponent.GetOwner` MeshComp)))
  (bind _returnvalue_2 (`SceneComponent.GetSocketLocation` MeshComp (`self.SocketName`)))
  (bind (_outhit _returnvalue_3) (`KismetSystemLibrary.LineTraceSingleForObjects` :`Start` (+ _returnvalue_2 (* _returnvalue -250.0)) :`End` (+ _returnvalue_2 (* _returnvalue 25.0)) :`ObjectTypes` (`|MakeArray` "ObjectTypeQuery7" :!type "EObjectTypeQuery Enum") :`bTraceComplex` true :`DrawDebugType` "ForDuration" :`bIgnoreSelf` false))
  (if (`self.Attached`)
    (bind _returnvalue_4 (`NiagaraFunctionLibrary.SpawnSystemAttached` "/Game/VFX/Characters/NS_Character_Foot_Poof.NS_Character_Foot_Poof" MeshComp (`self.SocketName`) (0.0 0.0 0.0) (struct) "KeepRelativeOffset" true))
    (`NiagaraComponent.SetVariableLinearColor` _returnvalue_4 "Poof_Colour" (`KismetMathLibrary.SelectColor` (`KismetMathLibrary.MakeColor` 1.0) (`KismetMathLibrary.MakeColor` 0.19 0.06 0.0) _returnvalue_3))
    (else
      (return false))))